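; BP_StopEria is a stop-area trigger that ends a BP_Sample actor's run when flagged.
; Box overlap sets HitObj and Remove for any actor and stores the BP_Sample it casts to, while end overlap clears only HitObj.
; Tick consumes the Set flag, which nothing here raises, then marks the stored actor as End.
; It also drops the first ALLTarget entry if Remove is still pending.
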(event `self.ReceiveTick`
  (params (DeltaSeconds :type "Float (single-precision)"))
  (bind _myactor (`self.MyActor`))
  (if (`self.Set`)
    (set `self.Set` false)
    (if (`KismetSystemLibrary.IsValid` _myactor)
      (set `/Game/MyContents/BluePrints/BP_Sample.End` true _myactor)
      (if (`self.Remove`)
        (`KismetArrayLibrary.Array_Remove` (`/Game/MyContents/BluePrints/BP_Sample.ALLTarget` _myactor))
        (set `self.Remove` false)))))

(event `self.Box.OnComponentBeginOverlap`
  (params (OverlappedComponent :type "PrimitiveComponent Object Reference") (OtherActor :type "Actor Object Reference") (OtherComp :type "PrimitiveComponent Object Reference") (OtherBodyIndex :type Integer) (bFromSweep :type Boolean) (SweepResult :type "HitResult Structure (by ref)"))
  (set `self.HitObj` true)
  (set `self.Remove` true)
  (bind _asbp_sample (cast `/Game/MyContents/BluePrints/BP_Sample` OtherActor))
  (set `self.MyActor` _asbp_sample))

(event `self.Box.OnComponentEndOverlap`
  (params (OverlappedComponent :type "PrimitiveComponent Object Reference") (OtherActor :type "Actor Object Reference") (OtherComp :type "PrimitiveComponent Object Reference") (OtherBodyIndex :type Integer))
  (set `self.HitObj` false))

(fn `UserConstructionScript`)