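; BP_ChoiceObject is a picking-arm machine that takes goods from nine red, white and blue spawn slots and hands them to BP_Clane, bound for the oven table.
; Slot overlaps track occupancy and per-color counts for progress displays.
; Tick picks a random occupied slot and, outside Map_Edit, plays its runtime-bound Level Sequence when BP_Oven state allows.
; Arm and conveyor overlaps retarget goods, reversing the sequence for returns.
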(event `self.ReceiveBeginPlay`
  (`parent.ReceiveBeginPlay`)
  (`|ExecutionSequence`
    (:`then_0`
      (`PrimitiveComponent.SetSimulatePhysics` (`self.5`) false)
      (`self.Init` "NewEnumerator6" (`|MakeArray` (`self.5`) (`self.5idou`) (`self.5moveclane`) (`self.5oshidashi`))) ; 親の変数の初期化
      ;[1 1 1] アニメーションの初期化
      (bind _output_get (set `self.Binding` (`self.MakeBinding`)))
      (bind _keys (`BlueprintMapLibrary.Map_Keys` _output_get))
      (for _array_element _keys
        (bind (_outactor _returnvalue) (`LevelSequencePlayer.CreateLevelSequencePlayer` _array_element))
        (`LevelSequenceActor.SetBinding` _outactor (`BlueprintMapLibrary.Map_Find` (`self.Binding`) _array_element) (`|MakeArray` self :!type "Actor Object Reference") false)
        (`MovieSceneSequencePlayer.SetPlayRate` _returnvalue (`self.Speed`))
        (`BlueprintMapLibrary.Map_Add` (`self.PickingLevelSequence`) _array_element _returnvalue)
        (set `self.StartOrRevers` true)
        (set `self.PlaySequence` true))
      (`self.InputCollitionName`))
    (:`then_1`
      (`self.InitProgress` (`self.RedCount`) (`self.MaxRedCount`) (`self.RedString`) 0 "Hidden")
      (`self.InitProgress` (`self.BlueCount`) (`self.MaxBlueCount`) (`self.BlueString`) 0 "Hidden")
      (`self.InitProgress` (`self.WhiteCount`) (`self.MaxWhiteCount`) (`self.WhiteString`) 0 "Hidden"))))

(event `self.ReceiveTick`
  (params (DeltaSeconds :type "Float (single-precision)"))
  (`parent.ReceiveTick` DeltaSeconds)
  (`|ExecutionSequence`
    (:`then_0`
      (if (not (`KismetSystemLibrary.IsValid` (`self.BP_PramamGoods`)))
        ;[1 1 1] 通常の開始時の時ランダムにスポーン位置にあるオブジェクトに向けてアニメーションを開始するためのキーを入力
        (if (== (`self.PlayString`) "")
          (bind _keys (`BlueprintMapLibrary.Map_Keys` (`self.spawnallay`)))
          (bind _output_get (set `self.PlayString` (`KismetArrayLibrary.Array_Random` _keys)))
          (if (not (`BlueprintMapLibrary.Map_Find` (`self.spawnallay`) _output_get))
            (set `self.PlayString` ""))
          (else
            (set `self.StartOrRevers` true)))))
    (:`then_1`
      (bind _returnvalue (`GameplayStatics.GetCurrentLevelName` true))
      (if (!= _returnvalue "Map_Edit")
        ;[1 1 1] アニメーションを開始（再生中は再生させない）
        (bind _keys_2 (`BlueprintMapLibrary.Map_Keys` (`self.BPE_Picking Or LevelSequence_0`)))
        (for _array_element _keys_2
          (bind _value (`BlueprintMapLibrary.Map_Find` (`self.PickingLevelSequence`) (`BlueprintMapLibrary.Map_Find` (`self.BPE_Picking Or LevelSequence_0`) _array_element)))
          (if (`KismetSystemLibrary.IsValid` _value)
            (add `MovieSceneSequencePlayer.OnFinished` _value (delegate `FinisheAnim`))
            (bind _outactors (`GameplayStatics.GetAllActorsOfClass` "/Game/MyContents/BluePrints/MachineObject/BP_Oven.BP_Oven_C"))
            (for _array_element_2 _outactors
              (if (and (`self.PlaySequence`) (`KismetSystemLibrary.IsValid` (`self.NowAnimation`)) (`|EnumEquality` (`/Game/MyContents/BluePrints/MachineObject/BP_Oven.BPE_SuperToaki` _array_element_2) "NewEnumerator4"))
                (if (`self.StartOrRevers`)
                  (if (not (`self.HitHakobuLocation`))
                    (`MovieSceneSequencePlayer.Play` (`self.NowAnimation`))
                    (set `self.PlaySequence` false :!label _label))
                  (elif (`self.HitHakobuLocation`)
                    (`MovieSceneSequencePlayer.PlayReverse` (`self.NowAnimation`))
                    (goto _label)))))))))
    (:`then_2`
      (if (`self.HitHakobuLocation`)
        (bind _outactors_2 (`GameplayStatics.GetAllActorsOfClass` "/Game/MyContents/BluePrints/MachineObject/BP_Oven.BP_Oven_C"))
        (for _array_element_3 _outactors_2
          (if (`|EnumEquality` (`/Game/MyContents/BluePrints/MachineObject/BP_Oven.BPE_SuperToaki` _array_element_3) "NewEnumerator1")
            (set `self.HitHakobuLocation` false)))))
    (:`then_3`
      (`self.UpDataProgress` (`self.RedString`) (`self.MaxRedCount`) (`self.RedCount`))
      (`self.UpDataProgress` (`self.BlueString`) (`self.MaxBlueCount`) (`self.BlueCount`))
      (`self.UpDataProgress` (`self.WhiteString`) (`self.MaxWhiteCount`) (`self.WhiteCount`)))))

(event `FinisheAnim`
  ;[1 1 1] アニメーションを開始（再生中は再生させない）
  (set `self.PlaySequence` true)
  (set `self.PlayString` ""))

(event `self.ArmCollition.OnComponentBeginOverlap`
  (params (OverlappedComponent :type "PrimitiveComponent Object Reference") (OtherActor :type "Actor Object Reference") (OtherComp :type "PrimitiveComponent Object Reference") (OtherBodyIndex :type Integer) (bFromSweep :type Boolean) (SweepResult :type "HitResult Structure (by ref)"))
  (bind _noseru (`self.noseru`))
  ;[1 1 1] 加工品がアームにあたった処理、加工品がベルトコンベアの手前にあたった処理、加工品がベルトコンベアの奥にあたった処理
  (bind _asbp_parent_goods (cast `/Game/MyContents/BluePrints/ProcessedProducts/BP_ParentGoods` OtherActor))
  (if (`KismetSystemLibrary.IsValid` (`self.BP_PramamGoods`))
    (if (`/Game/MyContents/BluePrints/ProcessedProducts/BP_ParentGoods.Return` (`self.BP_PramamGoods`))
      (set `/Game/MyContents/BluePrints/ProcessedProducts/BP_ParentGoods.Target` _noseru (`self.BP_PramamGoods`))
      (set `/Game/MyContents/BluePrints/ProcessedProducts/BP_ParentGoods.ReversTarget` null (`self.BP_PramamGoods`))
      (set `/Game/MyContents/BluePrints/ProcessedProducts/BP_ParentGoods.NextTarget` null (`self.BP_PramamGoods`)))
    (else
      (bind _output_get (set `self.BP_PramamGoods` _asbp_parent_goods))
      (set `/Game/MyContents/BluePrints/ProcessedProducts/BP_ParentGoods.Target` _noseru _output_get))))

(event `self.HakobuLocation.OnComponentBeginOverlap`
  (params (OverlappedComponent :type "PrimitiveComponent Object Reference") (OtherActor :type "Actor Object Reference") (OtherComp :type "PrimitiveComponent Object Reference") (OtherBodyIndex :type Integer) (bFromSweep :type Boolean) (SweepResult :type "HitResult Structure (by ref)"))
  ;[1 1 1] 加工品がアームにあたった処理、加工品がベルトコンベアの手前にあたった処理、加工品がベルトコンベアの奥にあたった処理
  (cast `/Game/MyContents/BluePrints/ProcessedProducts/BP_ParentGoods` OtherActor)
  (if (`/Game/MyContents/BluePrints/ProcessedProducts/BP_ParentGoods.Return` (`self.BP_PramamGoods`))
    (set `self.StartOrRevers` false)
    (else
      (set `self.HitHakobuLocation` true)
      (set `/Game/MyContents/BluePrints/ProcessedProducts/BP_ParentGoods.Target` (`self.HakobuLocation`) (`self.BP_PramamGoods`))
      (set `/Game/MyContents/BluePrints/ProcessedProducts/BP_ParentGoods.NextTarget` (`self.HakobuLocation1`) (`self.BP_PramamGoods`)))))

(event `self.HakobuLocation1.OnComponentBeginOverlap`
  (params (OverlappedComponent :type "PrimitiveComponent Object Reference") (OtherActor :type "Actor Object Reference") (OtherComp :type "PrimitiveComponent Object Reference") (OtherBodyIndex :type Integer) (bFromSweep :type Boolean) (SweepResult :type "HitResult Structure (by ref)"))
  ;[1 1 1] 加工品がアームにあたった処理、加工品がベルトコンベアの手前にあたった処理、加工品がベルトコンベアの奥にあたった処理
  (cast `/Game/MyContents/BluePrints/ProcessedProducts/BP_ParentGoods` OtherActor)
  (`/Engine/EditorBlueprintResources/StandardMacros.DoOnce` false :!label _label_2
    (:`Completed`
      (bind _outactors (`GameplayStatics.GetAllActorsOfClass` "/Game/MyContents/BluePrints/MachineObject/BP_Oven.BP_Oven_C"))
      (for _array_element _outactors
        (set `/Game/MyContents/BluePrints/ProcessedProducts/BP_ParentGoods.NextEria` (`/Game/MyContents/BluePrints/MachineObject/BP_Oven.tablebox` _array_element) (`self.BP_PramamGoods`)))
      (bind _outactors_2 (`GameplayStatics.GetAllActorsOfClass` "/Game/MyContents/BluePrints/MachineObject/BP_Clane.BP_Clane_C"))
      (for _array_element_2 _outactors_2
        (`/Game/MyContents/BluePrints/MachineObject/BP_Clane.AddTargetArray` _array_element_2 (`self.BP_PramamGoods`)))
      (set `self.BP_PramamGoods` null))))

(event `self.HakobuLocation1.OnComponentEndOverlap`
  (params (OverlappedComponent :type "PrimitiveComponent Object Reference") (OtherActor :type "Actor Object Reference") (OtherComp :type "PrimitiveComponent Object Reference") (OtherBodyIndex :type Integer))
  (goto _label_2 :!via `Reset`))

(event `self.SpawnLocationWhite1.OnComponentBeginOverlap`
  (params (OverlappedComponent :type "PrimitiveComponent Object Reference") (OtherActor :type "Actor Object Reference") (OtherComp :type "PrimitiveComponent Object Reference") (OtherBodyIndex :type Integer) (bFromSweep :type Boolean) (SweepResult :type "HitResult Structure (by ref)"))
  (bind _asbp_parent_goods (cast `/Game/MyContents/BluePrints/ProcessedProducts/BP_ParentGoods` OtherActor))
  (`self.HitGoodsObject` (`/Game/MyContents/BluePrints/ProcessedProducts/BP_ParentGoods.Goods` _asbp_parent_goods) OtherComp (`self.SpawnLocationWhite1`))
  (`|ExecutionSequence`
    (:`then_0`
      (`/Engine/EditorBlueprintResources/StandardMacros.DoOnce` false :!label _label
        (:`Completed`
          (`/Engine/EditorBlueprintResources/StandardMacros.IncrementFloat` (`self.WhiteCount`)))))
    (:`then_1`
      (goto _label_2 :!via `Reset`))))

(event `self.SpawnLocationWhite1.OnComponentEndOverlap`
  (params (OverlappedComponent :type "PrimitiveComponent Object Reference") (OtherActor :type "Actor Object Reference") (OtherComp :type "PrimitiveComponent Object Reference") (OtherBodyIndex :type Integer))
  (cast `/Game/MyContents/BluePrints/ProcessedProducts/BP_ParentGoods` OtherActor)
  (`self.Hit End Goods Object` (`self.SpawnLocationWhite1`) OtherComp)
  (`|ExecutionSequence`
    (:`then_0`
      (`/Engine/EditorBlueprintResources/StandardMacros.DoOnce` false :!label _label_2
        (:`Completed`
          (`/Engine/EditorBlueprintResources/StandardMacros.DecrementFloat` (`self.WhiteCount`)))))
    (:`then_1`
      (goto _label :!via `Reset`))))

(event `self.SpawnLocationWhite2.OnComponentBeginOverlap`
  (params (OverlappedComponent :type "PrimitiveComponent Object Reference") (OtherActor :type "Actor Object Reference") (OtherComp :type "PrimitiveComponent Object Reference") (OtherBodyIndex :type Integer) (bFromSweep :type Boolean) (SweepResult :type "HitResult Structure (by ref)"))
  (bind _asbp_parent_goods (cast `/Game/MyContents/BluePrints/ProcessedProducts/BP_ParentGoods` OtherActor))
  (`self.HitGoodsObject` (`/Game/MyContents/BluePrints/ProcessedProducts/BP_ParentGoods.Goods` _asbp_parent_goods) OtherComp (`self.SpawnLocationWhite2`))
  (`|ExecutionSequence`
    (:`then_0`
      (`/Engine/EditorBlueprintResources/StandardMacros.DoOnce` false :!label _label_3
        (:`Completed`
          (`/Engine/EditorBlueprintResources/StandardMacros.IncrementFloat` (`self.WhiteCount`)))))
    (:`then_1`
      (goto _label_4 :!via `Reset`))))

(event `self.SpawnLocationWhite2.OnComponentEndOverlap`
  (params (OverlappedComponent :type "PrimitiveComponent Object Reference") (OtherActor :type "Actor Object Reference") (OtherComp :type "PrimitiveComponent Object Reference") (OtherBodyIndex :type Integer))
  (cast `/Game/MyContents/BluePrints/ProcessedProducts/BP_ParentGoods` OtherActor)
  (`self.Hit End Goods Object` (`self.SpawnLocationWhite2`) OtherComp)
  (`|ExecutionSequence`
    (:`then_0`
      (`/Engine/EditorBlueprintResources/StandardMacros.DoOnce` false :!label _label_4
        (:`Completed`
          (`/Engine/EditorBlueprintResources/StandardMacros.DecrementFloat` (`self.WhiteCount`)))))
    (:`then_1`
      (goto _label_3 :!via `Reset`))))

(event `self.SpawnLocationWhite3.OnComponentBeginOverlap`
  (params (OverlappedComponent :type "PrimitiveComponent Object Reference") (OtherActor :type "Actor Object Reference") (OtherComp :type "PrimitiveComponent Object Reference") (OtherBodyIndex :type Integer) (bFromSweep :type Boolean) (SweepResult :type "HitResult Structure (by ref)"))
  (bind _asbp_parent_goods (cast `/Game/MyContents/BluePrints/ProcessedProducts/BP_ParentGoods` OtherActor))
  (`self.HitGoodsObject` (`/Game/MyContents/BluePrints/ProcessedProducts/BP_ParentGoods.Goods` _asbp_parent_goods) OtherComp (`self.SpawnLocationWhite3`))
  (`|ExecutionSequence`
    (:`then_0`
      (`/Engine/EditorBlueprintResources/StandardMacros.DoOnce` false :!label _label_5
        (:`Completed`
          (`/Engine/EditorBlueprintResources/StandardMacros.IncrementFloat` (`self.WhiteCount`)))))
    (:`then_1`
      (goto _label_6 :!via `Reset`))))

(event `self.SpawnLocationWhite3.OnComponentEndOverlap`
  (params (OverlappedComponent :type "PrimitiveComponent Object Reference") (OtherActor :type "Actor Object Reference") (OtherComp :type "PrimitiveComponent Object Reference") (OtherBodyIndex :type Integer))
  (cast `/Game/MyContents/BluePrints/ProcessedProducts/BP_ParentGoods` OtherActor)
  (`self.Hit End Goods Object` (`self.SpawnLocationWhite3`) OtherComp)
  (`|ExecutionSequence`
    (:`then_0`
      (`/Engine/EditorBlueprintResources/StandardMacros.DoOnce` false :!label _label_6
        (:`Completed`
          (`/Engine/EditorBlueprintResources/StandardMacros.DecrementFloat` (`self.WhiteCount`)))))
    (:`then_1`
      (goto _label_5 :!via `Reset`))))

(event `self.SpawnLocationBlue1.OnComponentBeginOverlap`
  (params (OverlappedComponent :type "PrimitiveComponent Object Reference") (OtherActor :type "Actor Object Reference") (OtherComp :type "PrimitiveComponent Object Reference") (OtherBodyIndex :type Integer) (bFromSweep :type Boolean) (SweepResult :type "HitResult Structure (by ref)"))
  (bind _asbp_parent_goods (cast `/Game/MyContents/BluePrints/ProcessedProducts/BP_ParentGoods` OtherActor))
  (`self.HitGoodsObject` (`/Game/MyContents/BluePrints/ProcessedProducts/BP_ParentGoods.Goods` _asbp_parent_goods) OtherComp (`self.SpawnLocationBlue1`))
  (`|ExecutionSequence`
    (:`then_0`
      (`/Engine/EditorBlueprintResources/StandardMacros.DoOnce` false :!label _label
        (:`Completed`
          (`/Engine/EditorBlueprintResources/StandardMacros.IncrementFloat` (`self.BlueCount`)))))
    (:`then_1`
      (goto _label_2 :!via `Reset`))))

(event `self.SpawnLocationBlue1.OnComponentEndOverlap`
  (params (OverlappedComponent :type "PrimitiveComponent Object Reference") (OtherActor :type "Actor Object Reference") (OtherComp :type "PrimitiveComponent Object Reference") (OtherBodyIndex :type Integer))
  (cast `/Game/MyContents/BluePrints/ProcessedProducts/BP_ParentGoods` OtherActor)
  (`self.Hit End Goods Object` (`self.SpawnLocationBlue1`) OtherComp)
  (`|ExecutionSequence`
    (:`then_0`
      (`/Engine/EditorBlueprintResources/StandardMacros.DoOnce` false :!label _label_2
        (:`Completed`
          (`/Engine/EditorBlueprintResources/StandardMacros.DecrementFloat` (`self.BlueCount`)))))
    (:`then_1`
      (goto _label :!via `Reset`))))

(event `self.SpawnLocationBlue2.OnComponentBeginOverlap`
  (params (OverlappedComponent :type "PrimitiveComponent Object Reference") (OtherActor :type "Actor Object Reference") (OtherComp :type "PrimitiveComponent Object Reference") (OtherBodyIndex :type Integer) (bFromSweep :type Boolean) (SweepResult :type "HitResult Structure (by ref)"))
  (bind _asbp_parent_goods (cast `/Game/MyContents/BluePrints/ProcessedProducts/BP_ParentGoods` OtherActor))
  (`self.HitGoodsObject` (`/Game/MyContents/BluePrints/ProcessedProducts/BP_ParentGoods.Goods` _asbp_parent_goods) OtherComp (`self.SpawnLocationBlue2`))
  (`|ExecutionSequence`
    (:`then_0`
      (`/Engine/EditorBlueprintResources/StandardMacros.DoOnce` false :!label _label_3
        (:`Completed`
          (`/Engine/EditorBlueprintResources/StandardMacros.IncrementFloat` (`self.BlueCount`)))))
    (:`then_1`
      (goto _label_4 :!via `Reset`))))

(event `self.SpawnLocationBlue2.OnComponentEndOverlap`
  (params (OverlappedComponent :type "PrimitiveComponent Object Reference") (OtherActor :type "Actor Object Reference") (OtherComp :type "PrimitiveComponent Object Reference") (OtherBodyIndex :type Integer))
  (cast `/Game/MyContents/BluePrints/ProcessedProducts/BP_ParentGoods` OtherActor)
  (`self.Hit End Goods Object` (`self.SpawnLocationBlue2`) OtherComp)
  (`|ExecutionSequence`
    (:`then_0`
      (`/Engine/EditorBlueprintResources/StandardMacros.DoOnce` false :!label _label_4
        (:`Completed`
          (`/Engine/EditorBlueprintResources/StandardMacros.DecrementFloat` (`self.BlueCount`)))))
    (:`then_1`
      (goto _label_3 :!via `Reset`))))

(event `self.SpawnLocationBlue3.OnComponentBeginOverlap`
  (params (OverlappedComponent :type "PrimitiveComponent Object Reference") (OtherActor :type "Actor Object Reference") (OtherComp :type "PrimitiveComponent Object Reference") (OtherBodyIndex :type Integer) (bFromSweep :type Boolean) (SweepResult :type "HitResult Structure (by ref)"))
  (bind _asbp_parent_goods (cast `/Game/MyContents/BluePrints/ProcessedProducts/BP_ParentGoods` OtherActor))
  (`self.HitGoodsObject` (`/Game/MyContents/BluePrints/ProcessedProducts/BP_ParentGoods.Goods` _asbp_parent_goods) OtherComp (`self.SpawnLocationBlue3`))
  (`|ExecutionSequence`
    (:`then_0`
      (`/Engine/EditorBlueprintResources/StandardMacros.DoOnce` false :!label _label_5
        (:`Completed`
          (`/Engine/EditorBlueprintResources/StandardMacros.IncrementFloat` (`self.BlueCount`)))))
    (:`then_1`
      (goto _label_6 :!via `Reset`))))

(event `self.SpawnLocationBlue3.OnComponentEndOverlap`
  (params (OverlappedComponent :type "PrimitiveComponent Object Reference") (OtherActor :type "Actor Object Reference") (OtherComp :type "PrimitiveComponent Object Reference") (OtherBodyIndex :type Integer))
  (cast `/Game/MyContents/BluePrints/ProcessedProducts/BP_ParentGoods` OtherActor)
  (`self.Hit End Goods Object` (`self.SpawnLocationBlue3`) OtherComp)
  (`|ExecutionSequence`
    (:`then_0`
      (`/Engine/EditorBlueprintResources/StandardMacros.DoOnce` false :!label _label_6
        (:`Completed`
          (`/Engine/EditorBlueprintResources/StandardMacros.DecrementFloat` (`self.BlueCount`)))))
    (:`then_1`
      (goto _label_5 :!via `Reset`))))

(event `self.SpawnLocationRed1.OnComponentBeginOverlap`
  (params (OverlappedComponent :type "PrimitiveComponent Object Reference") (OtherActor :type "Actor Object Reference") (OtherComp :type "PrimitiveComponent Object Reference") (OtherBodyIndex :type Integer) (bFromSweep :type Boolean) (SweepResult :type "HitResult Structure (by ref)"))
  (bind _asbp_parent_goods (cast `/Game/MyContents/BluePrints/ProcessedProducts/BP_ParentGoods` OtherActor))
  (`self.HitGoodsObject` (`/Game/MyContents/BluePrints/ProcessedProducts/BP_ParentGoods.Goods` _asbp_parent_goods) OtherComp (`self.SpawnLocationRed1`))
  (`|ExecutionSequence`
    (:`then_0`
      (`/Engine/EditorBlueprintResources/StandardMacros.DoOnce` false :!label _label
        (:`Completed`
          (`/Engine/EditorBlueprintResources/StandardMacros.IncrementFloat` (`self.RedCount`)))))
    (:`then_1`
      (goto _label_2 :!via `Reset`))))

(event `self.SpawnLocationRed1.OnComponentEndOverlap`
  (params (OverlappedComponent :type "PrimitiveComponent Object Reference") (OtherActor :type "Actor Object Reference") (OtherComp :type "PrimitiveComponent Object Reference") (OtherBodyIndex :type Integer))
  (cast `/Game/MyContents/BluePrints/ProcessedProducts/BP_ParentGoods` OtherActor)
  (`self.Hit End Goods Object` (`self.SpawnLocationRed1`) OtherComp)
  (`|ExecutionSequence`
    (:`then_0`
      (`/Engine/EditorBlueprintResources/StandardMacros.DoOnce` false :!label _label_2
        (:`Completed`
          (`/Engine/EditorBlueprintResources/StandardMacros.DecrementFloat` (`self.RedCount`)))))
    (:`then_1`
      (goto _label :!via `Reset`))))

(event `self.SpawnLocationRed2.OnComponentBeginOverlap`
  (params (OverlappedComponent :type "PrimitiveComponent Object Reference") (OtherActor :type "Actor Object Reference") (OtherComp :type "PrimitiveComponent Object Reference") (OtherBodyIndex :type Integer) (bFromSweep :type Boolean) (SweepResult :type "HitResult Structure (by ref)"))
  (bind _asbp_parent_goods (cast `/Game/MyContents/BluePrints/ProcessedProducts/BP_ParentGoods` OtherActor))
  (`self.HitGoodsObject` (`/Game/MyContents/BluePrints/ProcessedProducts/BP_ParentGoods.Goods` _asbp_parent_goods) OtherComp (`self.SpawnLocationRed2`))
  (`|ExecutionSequence`
    (:`then_0`
      (`/Engine/EditorBlueprintResources/StandardMacros.DoOnce` false :!label _label_3
        (:`Completed`
          (`/Engine/EditorBlueprintResources/StandardMacros.IncrementFloat` (`self.RedCount`)))))
    (:`then_1`
      (goto _label_4 :!via `Reset`))))

(event `self.SpawnLocationRed2.OnComponentEndOverlap`
  (params (OverlappedComponent :type "PrimitiveComponent Object Reference") (OtherActor :type "Actor Object Reference") (OtherComp :type "PrimitiveComponent Object Reference") (OtherBodyIndex :type Integer))
  (cast `/Game/MyContents/BluePrints/ProcessedProducts/BP_ParentGoods` OtherActor)
  (`self.Hit End Goods Object` (`self.SpawnLocationRed2`) OtherComp)
  (`|ExecutionSequence`
    (:`then_0`
      (`/Engine/EditorBlueprintResources/StandardMacros.DoOnce` false :!label _label_4
        (:`Completed`
          (`/Engine/EditorBlueprintResources/StandardMacros.DecrementFloat` (`self.RedCount`)))))
    (:`then_1`
      (goto _label_3 :!via `Reset`))))

(event `self.SpawnLocationRed3.OnComponentBeginOverlap`
  (params (OverlappedComponent :type "PrimitiveComponent Object Reference") (OtherActor :type "Actor Object Reference") (OtherComp :type "PrimitiveComponent Object Reference") (OtherBodyIndex :type Integer) (bFromSweep :type Boolean) (SweepResult :type "HitResult Structure (by ref)"))
  (bind _asbp_parent_goods (cast `/Game/MyContents/BluePrints/ProcessedProducts/BP_ParentGoods` OtherActor))
  (`self.HitGoodsObject` (`/Game/MyContents/BluePrints/ProcessedProducts/BP_ParentGoods.Goods` _asbp_parent_goods) OtherComp (`self.SpawnLocationRed3`))
  (`|ExecutionSequence`
    (:`then_0`
      (`/Engine/EditorBlueprintResources/StandardMacros.DoOnce` false :!label _label_5
        (:`Completed`
          (`/Engine/EditorBlueprintResources/StandardMacros.IncrementFloat` (`self.RedCount`)))))
    (:`then_1`
      (goto _label_6 :!via `Reset`))))

(event `self.SpawnLocationRed3.OnComponentEndOverlap`
  (params (OverlappedComponent :type "PrimitiveComponent Object Reference") (OtherActor :type "Actor Object Reference") (OtherComp :type "PrimitiveComponent Object Reference") (OtherBodyIndex :type Integer))
  (cast `/Game/MyContents/BluePrints/ProcessedProducts/BP_ParentGoods` OtherActor)
  (`self.Hit End Goods Object` (`self.SpawnLocationRed3`) OtherComp)
  (`|ExecutionSequence`
    (:`then_0`
      (`/Engine/EditorBlueprintResources/StandardMacros.DoOnce` false :!label _label_6
        (:`Completed`
          (`/Engine/EditorBlueprintResources/StandardMacros.DecrementFloat` (`self.RedCount`)))))
    (:`then_1`
      (goto _label_5 :!via `Reset`))))

(fn `GoodsTargetLocation`
  (params (Target :type "PrimitiveComponent Object Reference") (`Delta Location X` :type "Float (double-precision)"))
  (returns (HitLocation :type Boolean))
  (bind _returnvalue_x (`KismetMathLibrary.BreakVector` (`SceneComponent.K2_GetComponentLocation` Target)))
  (bind _returnvalue_x_2 (`KismetMathLibrary.BreakVector` (`SceneComponent.K2_GetComponentLocation` (`/Game/MyContents/BluePrints/ProcessedProducts/BP_ParentGoods.Goods` (`self.BP_PramamGoods`)))))
  (bind _returnvalue (`KismetMathLibrary.NearlyEqual_FloatFloat` _returnvalue_x_2 _returnvalue_x (`KismetMathLibrary.Abs` (* `Delta Location X` 2.0))))
  (if _returnvalue
    (`SceneComponent.K2_SetWorldLocationAndRotation` :`self` (`/Game/MyContents/BluePrints/ProcessedProducts/BP_ParentGoods.Goods` (`self.BP_PramamGoods`)) :`NewLocation` (`SceneComponent.K2_GetComponentLocation` Target))
    (else
      (`SceneComponent.K2_AddWorldOffset` (`/Game/MyContents/BluePrints/ProcessedProducts/BP_ParentGoods.Goods` (`self.BP_PramamGoods`)) (`KismetMathLibrary.MakeVector` `Delta Location X`) false false)))
  (return _returnvalue))

(fn `Hit End Goods Object`
  (params (SpawnLocation :type "Object Object Reference") (OtherComp :type "PrimitiveComponent Object Reference"))
  (`BlueprintMapLibrary.Map_Add` (`self.spawnallay`) (`KismetSystemLibrary.GetObjectName` SpawnLocation))
  (`PrimitiveComponent.SetSimulatePhysics` OtherComp false))

(fn `HitColorSpown`
  (params (BP_ParamGoods :type "/Game/MyContents/BluePrints/ProcessedProducts/BP_ParentGoods Object Reference") (SpawnLocation :type "PrimitiveComponent Object Reference"))
  (`PrimitiveComponent.SetSimulatePhysics` (`/Game/MyContents/BluePrints/ProcessedProducts/BP_ParentGoods.Goods` BP_ParamGoods) false)
  (`BlueprintMapLibrary.Map_Add` (`self.spawnallay`) (`KismetSystemLibrary.GetObjectName` SpawnLocation) true)
  (if (`KismetSystemLibrary.IsValid` (`self.BP_PramamGoods`))
    (if (`/Game/MyContents/BluePrints/ProcessedProducts/BP_ParentGoods.Return` (`self.BP_PramamGoods`))
      (`SceneComponent.K2_SetWorldLocationAndRotation` :`self` (`/Game/MyContents/BluePrints/ProcessedProducts/BP_ParentGoods.Goods` (`self.BP_PramamGoods`)) :`NewLocation` (`SceneComponent.K2_GetComponentLocation` SpawnLocation))
      (set `/Game/MyContents/BluePrints/ProcessedProducts/BP_ParentGoods.Target` null (`self.BP_PramamGoods`))
      (set `/Game/MyContents/BluePrints/ProcessedProducts/BP_ParentGoods.Return` false (`self.BP_PramamGoods`))
      (set `self.BP_PramamGoods` null)
      (set `self.HitHakobuLocation` false)
      (set `self.PlayString` ""))))

(fn `HitGoodsObject`
  (params (Goods :type "SceneComponent Object Reference") (OtherComp :type "PrimitiveComponent Object Reference") (SpawnLocation :type "BoxComponent Object Reference"))
  (bind _returnvalue (`SceneComponent.K2_GetComponentLocation` SpawnLocation))
  (bind _returnvalue_2 (`KismetSystemLibrary.GetObjectName` SpawnLocation))
  (if (`self.StartOrRevers`)
    (`PrimitiveComponent.SetSimulatePhysics` OtherComp false)
    (if (not (`KismetSystemLibrary.IsValid` (`self.Other Comp`)))
      (`BlueprintMapLibrary.Map_Add` (`self.spawnallay`) _returnvalue_2 true)
      (`SceneComponent.K2_SetWorldLocationAndRotation` :`self` Goods :`NewLocation` _returnvalue))
    (else
      (`BlueprintMapLibrary.Map_Add` (`self.spawnallay`) _returnvalue_2 true)
      (`SceneComponent.K2_SetWorldLocationAndRotation` :`self` (`/Game/MyContents/BluePrints/ProcessedProducts/BP_ParentGoods.Goods` (`self.BP_PramamGoods`)) :`NewLocation` _returnvalue)
      (set `self.BP_PramamGoods` null))))

(fn `InputCollitionName`
  (bind _spawnlocationwhite1 (`self.SpawnLocationWhite1`))
  (bind _spawnlocationwhite2 (`self.SpawnLocationWhite2`))
  (bind _spawnlocationwhite3 (`self.SpawnLocationWhite3`))
  (bind _spawnlocationred1 (`self.SpawnLocationRed1`))
  (bind _spawnlocationred2 (`self.SpawnLocationRed2`))
  (bind _spawnlocationred3 (`self.SpawnLocationRed3`))
  (bind _spawnlocationblue3 (`self.SpawnLocationBlue3`))
  (bind _spawnlocationblue1 (`self.SpawnLocationBlue1`))
  (bind _spawnlocationblue2 (`self.SpawnLocationBlue2`))
  (bind _returnvalue (`KismetSystemLibrary.GetObjectName` _spawnlocationblue3))
  (bind _returnvalue_2 (`KismetSystemLibrary.GetObjectName` _spawnlocationblue1))
  (bind _returnvalue_3 (`KismetSystemLibrary.GetObjectName` _spawnlocationblue2))
  (bind _returnvalue_4 (`KismetSystemLibrary.GetObjectName` _spawnlocationwhite1))
  (bind _returnvalue_5 (`KismetSystemLibrary.GetObjectName` _spawnlocationwhite2))
  (bind _returnvalue_6 (`KismetSystemLibrary.GetObjectName` _spawnlocationwhite3))
  (bind _returnvalue_7 (`KismetSystemLibrary.GetObjectName` _spawnlocationred1))
  (bind _returnvalue_8 (`KismetSystemLibrary.GetObjectName` _spawnlocationred2))
  (bind _returnvalue_9 (`KismetSystemLibrary.GetObjectName` _spawnlocationred3))
  (`BlueprintMapLibrary.Map_Add` (`self.spawnallay`) _returnvalue_4)
  (`BlueprintMapLibrary.Map_Add` (`self.Spawn Location`) _returnvalue_4 _spawnlocationwhite1)
  (`BlueprintMapLibrary.Map_Add` (`self.BPE_Picking Or LevelSequence_0`) _returnvalue_4 "/Game/MyContents/LevelSequences/Picking/NPicking_White1.NPicking_White1")
  (`BlueprintMapLibrary.Map_Add` (`self.spawnallay`) _returnvalue_5)
  (`BlueprintMapLibrary.Map_Add` (`self.Spawn Location`) _returnvalue_5 _spawnlocationwhite2)
  (`BlueprintMapLibrary.Map_Add` (`self.BPE_Picking Or LevelSequence_0`) _returnvalue_5 "/Game/MyContents/LevelSequences/Picking/NPicking_White2.NPicking_White2")
  (`BlueprintMapLibrary.Map_Add` (`self.spawnallay`) _returnvalue_6)
  (`BlueprintMapLibrary.Map_Add` (`self.Spawn Location`) _returnvalue_6 _spawnlocationwhite3)
  (`BlueprintMapLibrary.Map_Add` (`self.BPE_Picking Or LevelSequence_0`) _returnvalue_6 "/Game/MyContents/LevelSequences/Picking/NPicking_White3.NPicking_White3")
  (`BlueprintMapLibrary.Map_Add` (`self.spawnallay`) _returnvalue_7)
  (`BlueprintMapLibrary.Map_Add` (`self.Spawn Location`) _returnvalue_7 _spawnlocationred1)
  (`BlueprintMapLibrary.Map_Add` (`self.BPE_Picking Or LevelSequence_0`) _returnvalue_7 "/Game/MyContents/LevelSequences/Picking/NPicking_Red1.NPicking_Red1")
  (`BlueprintMapLibrary.Map_Add` (`self.spawnallay`) _returnvalue_8)
  (`BlueprintMapLibrary.Map_Add` (`self.Spawn Location`) _returnvalue_8 _spawnlocationred2)
  (`BlueprintMapLibrary.Map_Add` (`self.BPE_Picking Or LevelSequence_0`) _returnvalue_8 "/Game/MyContents/LevelSequences/Picking/NPicking_Red2.NPicking_Red2")
  (`BlueprintMapLibrary.Map_Add` (`self.spawnallay`) _returnvalue_9)
  (`BlueprintMapLibrary.Map_Add` (`self.Spawn Location`) _returnvalue_9 _spawnlocationred3)
  (`BlueprintMapLibrary.Map_Add` (`self.BPE_Picking Or LevelSequence_0`) _returnvalue_9 "/Game/MyContents/LevelSequences/Picking/NPicking_Red3.NPicking_Red3")
  (`BlueprintMapLibrary.Map_Add` (`self.spawnallay`) _returnvalue_2)
  (`BlueprintMapLibrary.Map_Add` (`self.Spawn Location`) _returnvalue_2 _spawnlocationblue1)
  (`BlueprintMapLibrary.Map_Add` (`self.BPE_Picking Or LevelSequence_0`) _returnvalue_2 "/Game/MyContents/LevelSequences/Picking/NPicking_Blue1.NPicking_Blue1")
  (`BlueprintMapLibrary.Map_Add` (`self.spawnallay`) _returnvalue_3)
  (`BlueprintMapLibrary.Map_Add` (`self.Spawn Location`) _returnvalue_3 _spawnlocationblue2)
  (`BlueprintMapLibrary.Map_Add` (`self.BPE_Picking Or LevelSequence_0`) _returnvalue_3 "/Game/MyContents/LevelSequences/Picking/NPicking_Blue2.NPicking_Blue2")
  (`BlueprintMapLibrary.Map_Add` (`self.spawnallay`) _returnvalue)
  (`BlueprintMapLibrary.Map_Add` (`self.Spawn Location`) _returnvalue _spawnlocationblue3)
  (`BlueprintMapLibrary.Map_Add` (`self.BPE_Picking Or LevelSequence_0`) _returnvalue "/Game/MyContents/LevelSequences/Picking/NPicking_Blue3.NPicking_Blue3"))

(fn `UserConstructionScript`)