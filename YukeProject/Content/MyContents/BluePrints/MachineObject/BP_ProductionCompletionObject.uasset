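; BP_ProductionCompletionObject is the finish point of a production line that counts completed goods and shows progress.
; Overlapping BP_ParentGoods are targeted to the trigger and counted, while an overlapping BP_Clane is told to advance via NextEria.
; Tick destroys the stored goods after two seconds and re-arms both DoOnce gates.
; It also refreshes progress every frame, taking the goal from BPW_Sokudosettei widgets or falling back to MaxClearCount.
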(event `self.ReceiveBeginPlay`
  ;[1 1 1] 初期設定
  (`parent.ReceiveBeginPlay`)
  (`PrimitiveComponent.SetSimulatePhysics` (`self.2`) false)
  (`self.Init` "NewEnumerator5" (`|MakeArray` (`self.2`))) ; 親の変数の初期化
  (set `self.ClearCount` 0)
  (`self.InitProgress` (`KismetMathLibrary.Conv_IntToDouble` (`self.ClearCount`)) (`KismetMathLibrary.Conv_IntToDouble` (`self.MaxClearCount`)) (`self.ClearString`) 0 "Hidden"))

(event `self.ReceiveTick`
  (params (DeltaSeconds :type "Float (single-precision)"))
  (bind _unchi (`self.unchi`))
  ;[1 1 1] 完成したオブジェクトが存在するとき2秒後に消す
  (`parent.ReceiveTick` DeltaSeconds)
  (`|ExecutionSequence`
    (:`then_0`
      (if (`KismetSystemLibrary.IsValid` _unchi)
        (`KismetSystemLibrary.Delay` 2.0)
        (`self.K2_DestroyActor` _unchi)
        (`|ExecutionSequence`
          (:`then_0`
            (goto _label :!via `Reset`))
          (:`then_1`
            (goto _label_2 :!via `Reset`)))))
    (:`then_1`
      (bind _foundwidgets (`WidgetBlueprintLibrary.GetAllWidgetsOfClass` "/Game/MyContents/BluePrints/Widget/SpeedSetting/BPW_Sokudosettei.BPW_Sokudosettei_C"))
      (if (`KismetSystemLibrary.IsValid` (`|GetArrayItem` _foundwidgets))
        (for _array_element _foundwidgets
          (`self.UpDataProgress` (`self.ClearString`) (`/Game/MyContents/BluePrints/Widget/SpeedSetting/BPW_SokudosetteiItem.Data` (`/Game/MyContents/BluePrints/Widget/SpeedSetting/BPW_Sokudosettei.MaxMokuhyousuu` _array_element)) (`KismetMathLibrary.Conv_IntToDouble` (`self.ClearCount`))))
        (else
          (`self.UpDataProgress` (`self.ClearString`) (`KismetMathLibrary.Conv_IntToDouble` (`self.MaxClearCount`)) (`KismetMathLibrary.Conv_IntToDouble` (`self.ClearCount`))))))))

(event `self.nanikoreT.OnComponentBeginOverlap`
  (params (OverlappedComponent :type "PrimitiveComponent Object Reference") (OtherActor :type "Actor Object Reference") (OtherComp :type "PrimitiveComponent Object Reference") (OtherBodyIndex :type Integer) (bFromSweep :type Boolean) (SweepResult :type "HitResult Structure (by ref)"))
  ;[1 1 1] 加工品の完了した到着地点
  (`|ExecutionSequence`
    (:`then_0`
      (bind _asbp_parent_goods (cast `/Game/MyContents/BluePrints/ProcessedProducts/BP_ParentGoods` OtherActor))
      (set `/Game/MyContents/BluePrints/ProcessedProducts/BP_ParentGoods.Target` (`self.nanikoreT`) _asbp_parent_goods)
      (set `self.unchi` _asbp_parent_goods)
      (`/Engine/EditorBlueprintResources/StandardMacros.DoOnce` false :!label _label
        (:`Completed`
          (`/Engine/EditorBlueprintResources/StandardMacros.IncrementInt` (`self.ClearCount`)))))
    (:`then_1`
      (bind _asbp_clane (cast `/Game/MyContents/BluePrints/MachineObject/BP_Clane` OtherActor))
      (`/Engine/EditorBlueprintResources/StandardMacros.DoOnce` false :!label _label_2
        (:`Completed`
          (`/Game/MyContents/BluePrints/MachineObject/BP_Clane.NextEria` _asbp_clane))))))

(fn `UserConstructionScript`)