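; Parent Blueprint for processed goods that a crane carries between targets, with a removable base (Dodai).
; Each Tick it either pins Goods to Target or steps it toward NextTarget per axis at ObjSpeed, snapping on arrival, then switching to ReversTarget and setting Return.
; Stepping pauses when global time dilation drops below 0.9.
; Box overlap stores the BP_Clane, or on overlapping BP_Oven calls its NextEria and releases it.
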(event `self.ReceiveBeginPlay`
  (`PrimitiveComponent.SetCollisionEnabled` (`self.Goods`) "QueryAndPhysics")
  (set `self.ObjSpeed` 20.0))

(event `DodaiDestroy`
  (bind _dodai (`self.Dodai`))
  ;[1 1 1] 土台の削除
  (if (`KismetSystemLibrary.IsValid` _dodai)
    (`ActorComponent.K2_DestroyComponent` _dodai)))

(event `self.ReceiveTick`
  (params (DeltaSeconds :type "Float (single-precision)"))
  (bind _returnvalue (`GameplayStatics.GetGlobalTimeDilation`))
  (bind _returnvalue_2 (`GameplayStatics.GetGlobalTimeDilation`))
  (bind _returnvalue_3 (`GameplayStatics.GetGlobalTimeDilation`))
  (bind _returnvalue_4 (`GameplayStatics.GetGlobalTimeDilation`))
  (bind _returnvalue_5 (`GameplayStatics.GetGlobalTimeDilation`))
  (bind _returnvalue_6 (`GameplayStatics.GetGlobalTimeDilation`))
  (bind _goods (`self.Goods`))
  (bind _objspeed (`self.ObjSpeed`))
  (bind _nexttarget (`self.NextTarget`))
  (bind _returnvalue_7 (`SceneComponent.K2_GetComponentLocation` _nexttarget))
  (bind (_returnvalue_x _returnvalue_y _returnvalue_z) (`KismetMathLibrary.BreakVector` (`SceneComponent.K2_GetComponentLocation` _nexttarget)))
  (bind (_returnvalue_x_2 _returnvalue_y_2 _returnvalue_z_2) (`KismetMathLibrary.BreakVector` (`SceneComponent.K2_GetComponentLocation` (`self.Goods`))))
  (bind (_returnvalue_x_3 _returnvalue_y_3 _returnvalue_z_3) (`KismetMathLibrary.BreakVector` (`SceneComponent.K2_GetComponentLocation` _nexttarget)))
  (bind (_returnvalue_x_4 _returnvalue_y_4 _returnvalue_z_4) (`KismetMathLibrary.BreakVector` (`SceneComponent.K2_GetComponentLocation` (`self.Goods`))))
  (bind _returnvalue_8 (`KismetMathLibrary.NearlyEqual_FloatFloat` _returnvalue_z_4 _returnvalue_z _objspeed))
  (bind _returnvalue_9 (`KismetMathLibrary.NearlyEqual_FloatFloat` _returnvalue_x_4 _returnvalue_x _objspeed))
  (bind _returnvalue_10 (`KismetMathLibrary.NearlyEqual_FloatFloat` _returnvalue_y_4 _returnvalue_y _objspeed))
  (bind _returnvalue_11 (and _returnvalue_9 _returnvalue_10 _returnvalue_8))
  ;[1 1 1] 移動
  (`|ExecutionSequence`
    (:`then_0`
      (if (`KismetSystemLibrary.IsValid` (`self.Target`))
        (`SceneComponent.K2_SetWorldLocationAndRotation` :`self` (`self.Goods`) :`NewLocation` (`SceneComponent.K2_GetComponentLocation` (`self.Target`)))))
    (:`then_1`
      (if (`KismetSystemLibrary.IsValid` (`self.NextTarget`))
        (`|ExecutionSequence`
          (:`then_0`
            (set `self.Target` null)
            (if (`KismetSystemLibrary.IsValid` _nexttarget)
              (`|ExecutionSequence`
                (:`then_0`
                  (if (`KismetSystemLibrary.IsValid` _nexttarget)
                    (if _returnvalue_9
                      (`self.SetMyGoodsLocation` _returnvalue_11 _returnvalue_7)
                      (elif (>= (- _returnvalue_x_3 _returnvalue_x_2) 0.0)
                        (if (<= 0.9 _returnvalue_2)
                          (`SceneComponent.K2_AddWorldOffset` (`self.Goods`) (`KismetMathLibrary.MakeVector` (* (`self.ObjSpeed`) _returnvalue_2)) false false)
                          (else
                            (`SceneComponent.K2_SetWorldLocation` _goods (`SceneComponent.K2_GetComponentLocation` _goods) false false :!label _label)))
                        (elif (<= 0.9 _returnvalue_3)
                          (`SceneComponent.K2_AddWorldOffset` (`self.Goods`) (`KismetMathLibrary.MakeVector` (* (`self.ObjSpeed`) _returnvalue_3 -1.0)) false false)
                          (else
                            (goto _label)))))))
                (:`then_1`
                  (if (`KismetSystemLibrary.IsValid` _nexttarget)
                    (if _returnvalue_10
                      (`self.SetMyGoodsLocation` _returnvalue_11 _returnvalue_7)
                      (elif (>= (- _returnvalue_y_3 _returnvalue_y_2) 0.0)
                        (if (<= 0.9 _returnvalue_6)
                          (`SceneComponent.K2_AddWorldOffset` (`self.Goods`) (`KismetMathLibrary.MakeVector` 0.0 (* (`self.ObjSpeed`) _returnvalue_6)) false false)
                          (else
                            (goto _label)))
                        (elif (<= 0.9 _returnvalue_4)
                          (`SceneComponent.K2_AddWorldOffset` (`self.Goods`) (`KismetMathLibrary.MakeVector` 0.0 (* (`self.ObjSpeed`) _returnvalue_4 -1.0)) false false)
                          (else
                            (goto _label)))))))
                (:`then_2`
                  (if (`KismetSystemLibrary.IsValid` _nexttarget)
                    (if _returnvalue_8
                      (`self.SetMyGoodsLocation` _returnvalue_11 _returnvalue_7)
                      (elif (>= (- _returnvalue_z_3 _returnvalue_z_2) 0.0)
                        (if (<= 0.9 _returnvalue_5)
                          (`SceneComponent.K2_AddWorldOffset` (`self.Goods`) (`KismetMathLibrary.MakeVector` 0.0 0.0 (* (`self.ObjSpeed`) _returnvalue_5)) false false)
                          (else
                            (goto _label)))
                        (elif (<= 0.9 _returnvalue)
                          (`SceneComponent.K2_AddWorldOffset` (`self.Goods`) (`KismetMathLibrary.MakeVector` 0.0 0.0 (* (`self.ObjSpeed`) _returnvalue -1.0)) false false)
                          (else
                            (goto _label))))))))))
          (:`then_1`
            (if (`self.NextBranchTarget`)
              (if (`KismetSystemLibrary.IsValid` (`self.ReversTarget`))
                (set `self.NextTarget` (`self.ReversTarget`))
                (set `self.Return` true)
                (set `self.NextBranchTarget` false)))))))))

(event `self.Box.OnComponentBeginOverlap`
  (params (OverlappedComponent :type "PrimitiveComponent Object Reference") (OtherActor :type "Actor Object Reference") (OtherComp :type "PrimitiveComponent Object Reference") (OtherBodyIndex :type Integer) (bFromSweep :type Boolean) (SweepResult :type "HitResult Structure (by ref)"))
  ;[1 1 1] クレーンのオブジェクトをゲットし変数に格納
  (if (`KismetSystemLibrary.IsValid` (`self.As Super Clane`))
    (cast `/Game/MyContents/BluePrints/MachineObject/BP_Oven` OtherActor)
    (`/Game/MyContents/BluePrints/MachineObject/BP_Clane.NextEria` (`self.As Super Clane`))
    (set `self.As Super Clane` null)
    (else
      (bind _asbp_clane (cast `/Game/MyContents/BluePrints/MachineObject/BP_Clane` OtherActor))
      (set `self.As Super Clane` _asbp_clane))))

(fn `SetMyGoodsLocation`
  (params (Condition :type Boolean) (InputPin :type "Vector Structure"))
  (if Condition
    (`SceneComponent.K2_SetWorldLocationAndRotation` :`self` (`self.Goods`) :`NewLocation` InputPin)
    (set `self.NextBranchTarget` true)))

(fn `UserConstructionScript`)