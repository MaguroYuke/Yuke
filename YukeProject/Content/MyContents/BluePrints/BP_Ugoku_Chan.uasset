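; BP_Ugoku_Chan is a moving actor that travels to a press point, waits for pressing, moves to a fixed exit point, then destroys itself.
; While Kkey is set, Tick lerps it to the first target, flags a widget and starts the CompletePressing timer.
; A looping timer drives the second lerp, then schedules destruction and, if WaitingCount is positive, spawns replacements at StartLocation actors.
; The earlier spawn branch is disabled.
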(event `self.ReceiveTick`
  (params (DeltaSeconds :type "Float (single-precision)"))
  (if (`self.Kkey`)
    (set `self.Elapsed` (- (`GameplayStatics.GetTimeSeconds`) (`self.Start Time`)))
    (set `self.Alpha` (/ (`self.Elapsed`) (`self.Move Duration`)))
    (if (>= (`self.Alpha`) 1.0)
      (set `self.Alpha` 1.0)
      (`self.K2_SetActorLocation` (`self.Target Location`))
      (set `self.IsActorActive` false)
      (set `self.Kkey` false)
      (set `/Game/MyContents/BluePrints/BP_UgokuUI.NewVar` true (`self.Widget`))
      (if (not (`self.PressingComplete`))
        (`KismetSystemLibrary.K2_SetTimer` null "CompletePressing" 3.0)
        (`KismetSystemLibrary.Delay` 5.0))
      (else
        (set `self.Current Location` (`KismetMathLibrary.VLerp` (`self.Initia Location`) (`self.Target Location`) (`self.Alpha`)))
        (`self.K2_SetActorLocation` (`self.Current Location`))))))

(event `Key|K`
  (params (Key :type "Key Structure"))
  (:`Released`
    (set `self.Kkey` false)))

(fn `CompletePressing`
  (if (not (`self.PressingComplete`))
    (set `self.PressingComplete` true)
    (set `self.NewTargetlocation` (630.0 1140.0 60.0))
    (set `self.ElapsedTime` 5.0)
    (`self.MoveToNewTarget`)))

(fn `MoveActorToNewtarget`
  (set `self.CurrentTime` (`GameplayStatics.GetTimeSeconds`))
  (set `self.ElapsedTime` (- (`self.CurrentTime`) (`self.Start Time`)))
  (if (> (`self.movementDuration`) 0.0)
    (set `self.Alpha` (/ (`self.ElapsedTime`) (`self.movementDuration`)))
    (set `self.Alpha` (`KismetMathLibrary.FClamp` (`self.Alpha`)))
    (if (< (`self.Alpha`) 1.0)
      (bind _output_get (set `self.NewLocation` (`KismetMathLibrary.VLerp` (`self.StartLocation`) (`self.Target Location`) (`self.Alpha`))))
      (`self.K2_SetActorLocation` _output_get)
      (else
        (`KismetSystemLibrary.K2_ClearTimer` null "MoveActorToNewtarget")
        (`self.K2_SetActorLocation` (`self.Target Location`))
        (`KismetSystemLibrary.K2_SetTimer` null "Visible" 3.0)
        (if (> (`self.WaitingCount`) 0)
          (bind _outactors (`GameplayStatics.GetAllActorsOfClass` "/Game/MyContents/BluePrints/StartLocation.StartLocation_C"))
          (for _array_element _outactors
            (`|SpawnActorFromClass` "BP_Ugoku_Chan_C" (`self.GetTransform` _array_element) "Undefined" "MultiplyWithRoot" null null)
            (set `self.Kkey` true)))))))

(fn `MoveToNewTarget`
  (`KismetSystemLibrary.PrintString` "NEW呼ばれた")
  (if (`self.PressingComplete`)
    (set `self.StartLocation` (`self.K2_GetActorLocation`))
    (set `self.Target Location` (`self.NewTargetlocation`))
    (set `self.Start Time` (`GameplayStatics.GetTimeSeconds`))
    (`KismetSystemLibrary.K2_SetTimer` null "MoveActorToNewtarget" 0.01 true)
    (set `self.IsActorActive` false)
    (if (and (>= (`self.WaitingCount`) 1) (== (`self.IsActorActive`) false) false)
      (`|SpawnActorFromClass` "BP_Ugoku_Chan_C" (`self.GetTransform`) "Undefined" "MultiplyWithRoot" null null)
      (set `self.WaitingCount` (- (`self.WaitingCount`) 1))
      (`KismetSystemLibrary.PrintString` "Hello"))))

(fn `UserConstructionScript`)

(fn `Visible`
  (`self.K2_DestroyActor`))