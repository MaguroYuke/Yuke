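; Automated crane actor that picks up the nearest BP_ParamGoods and carries it toward a Nanikore's NanikoreT point.
; A looping Crane level sequence drives it and pauses when yaw lines up, while Tick nudges boom and arm offsets.
; Overlap triggers set grab, lift and retract flags, and SuperKonbea's Toreruyo gates pickup.
; Work in progress: debug prints, disconnected logic, an empty ArmTargetLocation, and Mokutekichi is never set true in live logic.
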(event `self.ReceiveBeginPlay`
  (bind _outactors (`GameplayStatics.GetAllActorsOfClass` "/Game/MyContents/BluePrints/gomi/nanikore.nanikore_C"))
  (for _array_element _outactors
    (bind _outactors_2 (`GameplayStatics.GetAllActorsOfClass` "/Game/MyContents/BluePrints/gomi/SuperKonbea.SuperKonbea_C"))
    (for _array_element_2 _outactors_2
      (bind (_outactor _returnvalue) (`LevelSequencePlayer.CreateLevelSequencePlayer` "/Game/MyContents/LevelSequences/Crane.Crane" (make `MovieSceneSequencePlaybackSettings` false (struct) (`self.Settings Play Rate`))))
      (`LevelSequenceActor.SetBinding` _outactor (`|GetSequenceBinding` null) (`|MakeArray` self :!type "Actor Object Reference") false)
      (bind _output_get (set `self.Clane` _returnvalue))
      (bind _outactors_3 (`GameplayStatics.GetAllActorsOfClass` "/Game/MyContents/BluePrints/Buttons/BP_ParamGoods.BP_ParamGoods_C"))
      (set `self.Target` (`|GetArrayItem` _outactors_3))
      (set `self.StartPosision` (`SceneComponent.K2_GetComponentLocation` (`self.1stanp`)))
      (`PrimitiveComponent.SetSimulatePhysics` (`self.1dodai`) false))))

(event `self.ReceiveTick`
  (params (DeltaSeconds :type "Float (single-precision)"))
  (bind _1stanp (`self.1stanp`))
  (bind _distance (`self.Distance`))
  (bind _1arm (`self.1arm`))
  (bind _clane (`self.Clane`))
  (bind _clane_2 (`self.Clane`))
  (bind _1stanp_2 (`self.1stanp`))
  (bind _target (`self.Target`))
  (bind (_returnvalue_roll _returnvalue_pitch _returnvalue_yaw) (`KismetMathLibrary.BreakRotator` (`SceneComponent.K2_GetComponentRotation` (`self.1kaiten`))))
  (bind (_returnvalue_x _returnvalue_y _returnvalue_z) (`KismetMathLibrary.BreakVector` (`SceneComponent.K2_GetComponentLocation` _1arm)))
  (bind (_returnvalue_x_2 _returnvalue_y_2 _returnvalue_z_2) (`KismetMathLibrary.BreakVector` (`SceneComponent.K2_GetComponentLocation` _1stanp_2)))
  (bind (_returnvalue_roll_2 _returnvalue_pitch_2 _returnvalue_yaw_2) (`KismetMathLibrary.BreakRotator` (`SceneComponent.K2_GetComponentRotation` (`self.1kaiten`))))
  (bind (_returnvalue_x_3 _returnvalue_y_3 _returnvalue_z_3) (`KismetMathLibrary.BreakVector` (`SceneComponent.K2_GetComponentLocation` (`self.1stanp`))))
  (bind (_returnvalue_x_4 _returnvalue_y_4 _returnvalue_z_4) (`KismetMathLibrary.BreakVector` (`SceneComponent.K2_GetComponentLocation` _1stanp)))
  (bind (_returnvalue_roll_3 _returnvalue_pitch_3 _returnvalue_yaw_3) (`KismetMathLibrary.BreakRotator` (`SceneComponent.K2_GetComponentRotation` (`self.1kaiten`))))
  (bind (_returnvalue_x_5 _returnvalue_y_5 _returnvalue_z_5) (`KismetMathLibrary.BreakVector` (`SceneComponent.K2_GetComponentLocation` (`/Game/MyContents/BluePrints/Buttons/BP_ParamGoods.Goods` (`self.Target`)))))
  (bind (_returnvalue_x_6 _returnvalue_y_6) (`KismetMathLibrary.BreakVector` (`SceneComponent.K2_GetComponentLocation` (`/Game/MyContents/BluePrints/Buttons/BP_ParamGoods.Goods` _target))))
  (bind (_returnvalue_roll_4 _returnvalue_pitch_4 _returnvalue_yaw_4) (`KismetMathLibrary.BreakRotator` (`KismetMathLibrary.FindLookAtRotation` (`SceneComponent.K2_GetComponentLocation` (`self.1kaiten`)) (`SceneComponent.K2_GetComponentLocation` (`/Game/MyContents/BluePrints/Buttons/BP_ParamGoods.Goods` (`self.Target`))))))
  (`|ExecutionSequence`
    (:`then_0`
      (if (`self.mokutekichi`)
        (`|ExecutionSequence`
          (:`then_0`
            (if (not (`self.hikkomi`))
              (`SceneComponent.K2_AddLocalOffset` (`self.1stanp`) (-10.0 0.0 0.0) false false)))
          (:`then_1`
            (if (`self.joushou`)
              (if (`self.hikkomi`)
                (`MovieSceneSequencePlayer.Pause` _clane_2)
                (set `/Game/MyContents/BluePrints/gomi/SuperKonbea.toreruyo` false (stale `self.ReceiveBeginPlay` _array_element_2))
                (set `self.mokutekichi` false))
              (else
                (`MovieSceneSequencePlayer.Pause` _clane_2)
                (`SceneComponent.K2_AddWorldOffset` (`self.1arm`) (0.0 0.0 20.0) false false)
                (`KismetSystemLibrary.Delay` 0.2)
                (if (`self.hikkomi`)
                  (set `self.mokutekichi` false))))))
        (else
          (`KismetArrayLibrary.Array_Clear` (`self.Distance`))
          (bind _outactors (`GameplayStatics.GetAllActorsOfClass` "/Game/MyContents/BluePrints/Buttons/BP_ParamGoods.BP_ParamGoods_C"))
          (bind _output_get (set `self.Out Actors` _outactors))
          (for _array_element _output_get
            (`KismetArrayLibrary.Array_Add` (`self.Distance`) (`KismetMathLibrary.Vector_Distance` (`SceneComponent.K2_GetComponentLocation` (`/Game/MyContents/BluePrints/Buttons/BP_ParamGoods.Goods` _array_element)) (`SceneComponent.K2_GetComponentLocation` (`self.Target1`)))))
          (set `self.MinDistance` (`|GetArrayItem` _distance))
          (for _array_element_2 _distance
            (if (> (`self.MinDistance`) _array_element_2)
              (set `self.MinDistance` _array_element_2)))
          (for (_array_element_3 _array_index) _distance
            (if (`KismetMathLibrary.NearlyEqual_FloatFloat` _array_element_3 (`self.MinDistance`))
              (bind _output (`|GetArrayItem` (`self.Out Actors`) _array_index))
              (if (`KismetSystemLibrary.IsValid` _output)
                (set `self.Target` _output)
                (else
                  (set `self.Target` null)))))
          (if (`KismetSystemLibrary.IsValid` (`self.Target`))
            (set `self.Return Value Z (Yaw)` _returnvalue_yaw_4)
            (if (`self.Catch`)
              (`SceneComponent.K2_SetWorldLocation` (`/Game/MyContents/BluePrints/Buttons/BP_ParamGoods.Goods` (`self.Target`)) (`SceneComponent.K2_GetComponentLocation` (`self.Target1`)) false false)
              (if (`self.joushou`)
                (bind _nanikoret (`/Game/MyContents/BluePrints/gomi/nanikore.nanikoreT` (stale `self.ReceiveBeginPlay` _array_element)))
                (if (`KismetSystemLibrary.IsValid` _nanikoret)
                  (bind (_returnvalue_roll_5 _returnvalue_pitch_5 _returnvalue_yaw_5) (`KismetMathLibrary.BreakRotator` (`KismetMathLibrary.FindLookAtRotation` (`SceneComponent.K2_GetComponentLocation` (`self.1kaiten`)) (`SceneComponent.K2_GetComponentLocation` _nanikoret))))
                  (set `self.Return Value Z (Yaw)` _returnvalue_yaw_5)
                  (if (`self.Catch`)
                    (if (`KismetMathLibrary.NearlyEqual_FloatFloat` _returnvalue_yaw (`self.Return Value Z (Yaw)`) (+ (/ (`KismetMathLibrary.Abs` (- (`self.NowKaiten`) _returnvalue_yaw)) (`MovieSceneSequencePlayer.GetFrameDuration` (`self.Clane`))) (`self.Settings Play Rate`)))
                      (`MovieSceneSequencePlayer.Pause` (`self.Clane`))
                      (`SceneComponent.K2_SetWorldRotation` (`self.1kaiten`) (`KismetMathLibrary.MakeRotator` 0.0 0.0 (`self.Return Value Z (Yaw)`)) false false)
                      (if (`self.Catch`)
                        (if (`self.mokutekichi`)
                          (`SceneComponent.K2_SetWorldLocation` (`/Game/MyContents/BluePrints/Buttons/BP_ParamGoods.Goods` (`self.Target`)) (`SceneComponent.K2_GetComponentLocation` (`/Game/MyContents/BluePrints/gomi/nanikore.nanikoreT` (stale `self.ReceiveBeginPlay` _array_element))) false false)
                          (`MovieSceneSequencePlayer.Pause` _clane)
                          (`KismetSystemLibrary.Delay` 1.0)
                          (`MovieSceneSequencePlayer.PlayLooping` _clane -1)
                          (set `self.joushou` false)
                          (set `self.Catch` false)
                          (set `self.hit` false)
                          (else
                            (`SceneComponent.K2_AddWorldOffset` (`self.1arm`) (0.0 0.0 -20.0) false false)
                            (bind (_returnvalue_x_7 _returnvalue_y_7) (`KismetMathLibrary.BreakVector` (`SceneComponent.K2_GetComponentLocation` (`/Game/MyContents/BluePrints/gomi/nanikore.nanikoreT` (stale `self.ReceiveBeginPlay` _array_element)))))
                            (if (`KismetMathLibrary.NearlyEqual_FloatFloat` _returnvalue_x_4 _returnvalue_x_7 20.0)
                              (`SceneComponent.K2_SetWorldLocation` _1stanp (`KismetMathLibrary.MakeVector` _returnvalue_x_7 _returnvalue_y_7 _returnvalue_z_4) false false)
                              (else
                                (`SceneComponent.K2_AddLocalOffset` _1stanp (20.0 0.0 0.0) false false)))))))))
                (else
                  (`SceneComponent.K2_AddWorldOffset` (`self.1arm`) (0.0 0.0 20.0) false false)))
              (elif (and (`KismetMathLibrary.NearlyEqual_FloatFloat` _returnvalue_yaw_3 (`self.Return Value Z (Yaw)`) (+ (/ (`KismetMathLibrary.Abs` _returnvalue_yaw_3) (`MovieSceneSequencePlayer.GetFrameDuration` (`self.Clane`))) (`self.Settings Play Rate`))) (`/Game/MyContents/BluePrints/gomi/SuperKonbea.toreruyo` (stale `self.ReceiveBeginPlay` _array_element_2)))
                (`MovieSceneSequencePlayer.Pause` (`self.Clane`))
                (`SceneComponent.K2_SetWorldRotation` (`self.1kaiten`) (`KismetMathLibrary.MakeRotator` 0.0 0.0 (`self.Return Value Z (Yaw)`)) false false)
                (if (`self.hit`)
                  (set `self.Catch` true)
                  (elif (`KismetSystemLibrary.IsValid` _target)
                    (if (`KismetMathLibrary.NearlyEqual_FloatFloat` _returnvalue_y_2 _returnvalue_x_6 100.0)
                      (`SceneComponent.K2_SetWorldLocation` _1stanp_2 (`KismetMathLibrary.MakeVector` _returnvalue_x_6 _returnvalue_y_6 _returnvalue_z_2) true false)
                      (else
                        (`SceneComponent.K2_AddLocalOffset` _1stanp_2 (5.0 0.0 0.0) false false)))
                    (if (`KismetMathLibrary.NearlyEqual_FloatFloat` _returnvalue_z_5 _returnvalue_z 20.0)
                      (`SceneComponent.K2_SetWorldLocationAndRotation` :`self` _1arm :`NewLocation` (`KismetMathLibrary.MakeVector` _returnvalue_x_3 _returnvalue_y_3 _returnvalue_z_3))
                      (else
                        (`SceneComponent.K2_AddWorldOffset` _1arm (0.0 0.0 -20.0) false false)
                        (`KismetSystemLibrary.PrintString` "sagaruyo")))))
                (else
                  (set `self.StartPosision` (`SceneComponent.K2_GetComponentLocation` (`self.1stanp`)))
                  (set `self.NowKaiten` _returnvalue_yaw_2))))))))
    (:`then_1`
      (if (`self.saisei`)
        (`MovieSceneSequencePlayer.PlayLooping` (`self.Clane`) -1)
        (set `self.saisei` false)))
    (:`then_2`
      (`KismetSystemLibrary.PrintString` (`KismetStringLibrary.Conv_BoolToString` (`/Game/MyContents/BluePrints/gomi/SuperKonbea.toreruyo` (stale `self.ReceiveBeginPlay` _array_element_2)))))))

(event `self.StaticMesh.OnComponentBeginOverlap`
  (params (OverlappedComponent :type "PrimitiveComponent Object Reference") (OtherActor :type "Actor Object Reference") (OtherComp :type "PrimitiveComponent Object Reference") (OtherBodyIndex :type Integer) (bFromSweep :type Boolean) (SweepResult :type "HitResult Structure (by ref)")))

(event `self.armbox.OnComponentBeginOverlap`
  (params (OverlappedComponent :type "PrimitiveComponent Object Reference") (OtherActor :type "Actor Object Reference") (OtherComp :type "PrimitiveComponent Object Reference") (OtherBodyIndex :type Integer) (bFromSweep :type Boolean) (SweepResult :type "HitResult Structure (by ref)"))
  (if (== OtherComp (`self.dodaibox`))
    (set `self.joushou` true)
    (`KismetSystemLibrary.PrintString` "判定ある？")))

(event `self.Target1.OnComponentBeginOverlap`
  (params (OverlappedComponent :type "PrimitiveComponent Object Reference") (OtherActor :type "Actor Object Reference") (OtherComp :type "PrimitiveComponent Object Reference") (OtherBodyIndex :type Integer) (bFromSweep :type Boolean) (SweepResult :type "HitResult Structure (by ref)"))
  (if (not (`self.hit`))
    (bind _asbp_param_goods (cast `/Game/MyContents/BluePrints/Buttons/BP_ParamGoods` OtherActor))
    (set `self.joushou` false)
    (set `self.hit` true)
    (`PrimitiveComponent.SetSimulatePhysics` (`/Game/MyContents/BluePrints/Buttons/BP_ParamGoods.Goods` _asbp_param_goods) false)
    (`KismetSystemLibrary.PrintString` "Hello")
    (`KismetSystemLibrary.Delay` 1.0)
    (`MovieSceneSequencePlayer.PlayLooping` (`self.Clane`) -1)))

(event `self.Yuketarget.OnComponentBeginOverlap`
  (params (OverlappedComponent :type "PrimitiveComponent Object Reference") (OtherActor :type "Actor Object Reference") (OtherComp :type "PrimitiveComponent Object Reference") (OtherBodyIndex :type Integer) (bFromSweep :type Boolean) (SweepResult :type "HitResult Structure (by ref)")))

(event `self.hikkomu.OnComponentBeginOverlap`
  (params (OverlappedComponent :type "PrimitiveComponent Object Reference") (OtherActor :type "Actor Object Reference") (OtherComp :type "PrimitiveComponent Object Reference") (OtherBodyIndex :type Integer) (bFromSweep :type Boolean) (SweepResult :type "HitResult Structure (by ref)"))
  (if (== OtherComp (`self.hikkomuhou`))
    (set `self.hikkomi` true)
    (`KismetSystemLibrary.PrintString` "hikkomi")
    (else
      (`KismetSystemLibrary.PrintString` "chigau"))))

(fn `ArmTargetLocation`
  (params (Target :type "SceneComponent Object Reference")))

(fn `UserConstructionScript`)