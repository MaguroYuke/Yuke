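; Conveyor sorting machine actor that spawns a random red, white or blue Yuke item whenever its spawn flag is set.
; Color-specific triggers play push-out Level Sequences bound to this actor at runtime when a matching item overlaps.
; Other overlap volumes hand items to physics, clear their on-conveyor flag, or destroy them after a short delay.
; BluePush hits also apply force along the item's forward vector.
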(event `self.ReceiveTick`
  (params (DeltaSeconds :type "Float (single-precision)"))
  (if (`self.NewVar`)
    (`|SpawnActorFromClass` (`KismetArrayLibrary.Array_Random` (`|MakeArray` "/Game/MyContents/BluePrints/Objects/YukeRed.YukeRed_C" "/Game/MyContents/BluePrints/Objects/YukeWhite.YukeWhite_C" "/Game/MyContents/BluePrints/Objects/YukeBlue.YukeBlue_C" :!type "Actor Class Reference")) (`KismetMathLibrary.MakeTransform` (`SceneComponent.K2_GetComponentLocation` (`self.StaticMesh`))) "Undefined" "MultiplyWithRoot" null null)
    (set `self.NewVar` false)))

(event `self.ReceiveBeginPlay`
  (`PrimitiveComponent.SetSimulatePhysics` (`self.3dodai`) false))

(event `self.BlueTrigger.OnComponentBeginOverlap`
  (params (OverlappedComponent :type "PrimitiveComponent Object Reference") (OtherActor :type "Actor Object Reference") (OtherComp :type "PrimitiveComponent Object Reference") (OtherBodyIndex :type Integer) (bFromSweep :type Boolean) (SweepResult :type "HitResult Structure (by ref)"))
  (cast `/Game/MyContents/BluePrints/Objects/YukeBlue` OtherActor)
  (bind (_outactor _returnvalue) (`LevelSequencePlayer.CreateLevelSequencePlayer` "/Game/MyContents/LevelSequences/3oshidashi1.3oshidashi1"))
  (`LevelSequenceActor.SetBinding` _outactor (`|GetSequenceBinding` null) (`|MakeArray` self :!type "Actor Object Reference") false)
  (`MovieSceneSequencePlayer.Play` _returnvalue))

(event `self.RedTrigger.OnComponentBeginOverlap`
  (params (OverlappedComponent :type "PrimitiveComponent Object Reference") (OtherActor :type "Actor Object Reference") (OtherComp :type "PrimitiveComponent Object Reference") (OtherBodyIndex :type Integer) (bFromSweep :type Boolean) (SweepResult :type "HitResult Structure (by ref)"))
  (cast `/Game/MyContents/BluePrints/Objects/YukeRed` OtherActor)
  (bind (_outactor _returnvalue) (`LevelSequencePlayer.CreateLevelSequencePlayer` "/Game/MyContents/LevelSequences/3oshidashi2.3oshidashi2"))
  (`LevelSequenceActor.SetBinding` _outactor (`|GetSequenceBinding` null) (`|MakeArray` self :!type "Actor Object Reference") false)
  (`MovieSceneSequencePlayer.Play` _returnvalue))

(event `self.WhiteTrigger.OnComponentBeginOverlap`
  (params (OverlappedComponent :type "PrimitiveComponent Object Reference") (OtherActor :type "Actor Object Reference") (OtherComp :type "PrimitiveComponent Object Reference") (OtherBodyIndex :type Integer) (bFromSweep :type Boolean) (SweepResult :type "HitResult Structure (by ref)"))
  (cast `/Game/MyContents/BluePrints/Objects/YukeWhite` OtherActor)
  (bind (_outactor _returnvalue) (`LevelSequencePlayer.CreateLevelSequencePlayer` "/Game/MyContents/LevelSequences/3oshidashi3.3oshidashi3"))
  (`LevelSequenceActor.SetBinding` _outactor (`|GetSequenceBinding` null) (`|MakeArray` self :!type "Actor Object Reference") false)
  (`MovieSceneSequencePlayer.Play` _returnvalue))

(event `self.BluePush.OnComponentHit`
  (params (HitComponent :type "PrimitiveComponent Object Reference") (OtherActor :type "Actor Object Reference") (OtherComp :type "PrimitiveComponent Object Reference") (NormalImpulse :type "Vector Structure") (Hit :type "HitResult Structure (by ref)"))
  (bind _asbp_param_goods (cast `/Game/MyContents/BluePrints/Buttons/BP_ParamGoods` OtherActor))
  (`PrimitiveComponent.AddForce` (`/Game/MyContents/BluePrints/Buttons/BP_ParamGoods.Goods` _asbp_param_goods) (* (`KismetMathLibrary.GetForwardVector` (`self.K2_GetActorRotation` _asbp_param_goods)) (`self.power`)) "None" false))

(event `self.Box.OnComponentBeginOverlap`
  (params (OverlappedComponent :type "PrimitiveComponent Object Reference") (OtherActor :type "Actor Object Reference") (OtherComp :type "PrimitiveComponent Object Reference") (OtherBodyIndex :type Integer) (bFromSweep :type Boolean) (SweepResult :type "HitResult Structure (by ref)"))
  (bind _asbp_param_goods (cast `/Game/MyContents/BluePrints/Buttons/BP_ParamGoods` OtherActor))
  (`/Game/MyContents/BluePrints/Buttons/BP_ParamGoods.B` _asbp_param_goods (`self.Box`))
  (`KismetSystemLibrary.PrintString` "物理演算外れたよ"))

(event `self.Box.OnComponentEndOverlap`
  (params (OverlappedComponent :type "PrimitiveComponent Object Reference") (OtherActor :type "Actor Object Reference") (OtherComp :type "PrimitiveComponent Object Reference") (OtherBodyIndex :type Integer))
  (bind _asbp_param_goods (cast `/Game/MyContents/BluePrints/Buttons/BP_ParamGoods` OtherActor)))

(event `self.BluePush.OnComponentBeginOverlap`
  (params (OverlappedComponent :type "PrimitiveComponent Object Reference") (OtherActor :type "Actor Object Reference") (OtherComp :type "PrimitiveComponent Object Reference") (OtherBodyIndex :type Integer) (bFromSweep :type Boolean) (SweepResult :type "HitResult Structure (by ref)"))
  (bind _asyuke_blue (cast `/Game/MyContents/BluePrints/Objects/YukeBlue` OtherActor))
  (`PrimitiveComponent.SetSimulatePhysics` (`/Game/MyContents/BluePrints/Buttons/BP_ParamGoods.Goods` _asyuke_blue) true))

(event `self.Box1.OnComponentBeginOverlap`
  (params (OverlappedComponent :type "PrimitiveComponent Object Reference") (OtherActor :type "Actor Object Reference") (OtherComp :type "PrimitiveComponent Object Reference") (OtherBodyIndex :type Integer) (bFromSweep :type Boolean) (SweepResult :type "HitResult Structure (by ref)"))
  (bind _asyuke_red (cast `/Game/MyContents/BluePrints/Objects/YukeRed` OtherActor))
  (`PrimitiveComponent.SetSimulatePhysics` (`/Game/MyContents/BluePrints/Buttons/BP_ParamGoods.Goods` _asyuke_red) true))

(event `self.Box2.OnComponentBeginOverlap`
  (params (OverlappedComponent :type "PrimitiveComponent Object Reference") (OtherActor :type "Actor Object Reference") (OtherComp :type "PrimitiveComponent Object Reference") (OtherBodyIndex :type Integer) (bFromSweep :type Boolean) (SweepResult :type "HitResult Structure (by ref)"))
  (bind _asyuke_white (cast `/Game/MyContents/BluePrints/Objects/YukeWhite` OtherActor))
  (`PrimitiveComponent.SetSimulatePhysics` (`/Game/MyContents/BluePrints/Buttons/BP_ParamGoods.Goods` _asyuke_white) true))

(event `self.Box5.OnComponentBeginOverlap`
  (params (OverlappedComponent :type "PrimitiveComponent Object Reference") (OtherActor :type "Actor Object Reference") (OtherComp :type "PrimitiveComponent Object Reference") (OtherBodyIndex :type Integer) (bFromSweep :type Boolean) (SweepResult :type "HitResult Structure (by ref)"))
  (bind _asbp_param_goods (cast `/Game/MyContents/BluePrints/Buttons/BP_ParamGoods` OtherActor))
  (`KismetSystemLibrary.Delay` 1.0)
  (`self.K2_DestroyActor` _asbp_param_goods))

(event `self.Box4.OnComponentBeginOverlap`
  (params (OverlappedComponent :type "PrimitiveComponent Object Reference") (OtherActor :type "Actor Object Reference") (OtherComp :type "PrimitiveComponent Object Reference") (OtherBodyIndex :type Integer) (bFromSweep :type Boolean) (SweepResult :type "HitResult Structure (by ref)"))
  (bind _asbp_param_goods (cast `/Game/MyContents/BluePrints/Buttons/BP_ParamGoods` OtherActor))
  (`KismetSystemLibrary.Delay` 1.0)
  (`self.K2_DestroyActor` _asbp_param_goods))

(event `self.Box3.OnComponentBeginOverlap`
  (params (OverlappedComponent :type "PrimitiveComponent Object Reference") (OtherActor :type "Actor Object Reference") (OtherComp :type "PrimitiveComponent Object Reference") (OtherBodyIndex :type Integer) (bFromSweep :type Boolean) (SweepResult :type "HitResult Structure (by ref)"))
  (bind _asbp_param_goods (cast `/Game/MyContents/BluePrints/Buttons/BP_ParamGoods` OtherActor))
  (`KismetSystemLibrary.Delay` 1.0)
  (`self.K2_DestroyActor` _asbp_param_goods))

(event `self.boo.OnComponentBeginOverlap`
  (params (OverlappedComponent :type "PrimitiveComponent Object Reference") (OtherActor :type "Actor Object Reference") (OtherComp :type "PrimitiveComponent Object Reference") (OtherBodyIndex :type Integer) (bFromSweep :type Boolean) (SweepResult :type "HitResult Structure (by ref)"))
  (bind _asbp_param_goods (cast `/Game/MyContents/BluePrints/Buttons/BP_ParamGoods` OtherActor))
  (`PrimitiveComponent.SetSimulatePhysics` (`/Game/MyContents/BluePrints/Buttons/BP_ParamGoods.Goods` _asbp_param_goods) true)
  (set `/Game/MyContents/BluePrints/Buttons/BP_ParamGoods.boo` true _asbp_param_goods))

(event `self.yukeBlueyuke.OnComponentBeginOverlap`
  (params (OverlappedComponent :type "PrimitiveComponent Object Reference") (OtherActor :type "Actor Object Reference") (OtherComp :type "PrimitiveComponent Object Reference") (OtherBodyIndex :type Integer) (bFromSweep :type Boolean) (SweepResult :type "HitResult Structure (by ref)"))
  (bind _asyuke_blue (cast `/Game/MyContents/BluePrints/Objects/YukeBlue` OtherActor))
  (set `/Game/MyContents/BluePrints/Buttons/BP_ParamGoods.bOnConveyor` false _asyuke_blue)
  (`KismetSystemLibrary.PrintString` "押されたよ" :!label _label))

(event `self.yukeRedyuke.OnComponentBeginOverlap`
  (params (OverlappedComponent :type "PrimitiveComponent Object Reference") (OtherActor :type "Actor Object Reference") (OtherComp :type "PrimitiveComponent Object Reference") (OtherBodyIndex :type Integer) (bFromSweep :type Boolean) (SweepResult :type "HitResult Structure (by ref)"))
  (bind _asyuke_red (cast `/Game/MyContents/BluePrints/Objects/YukeRed` OtherActor))
  (set `/Game/MyContents/BluePrints/Buttons/BP_ParamGoods.bOnConveyor` false _asyuke_red)
  (goto _label))

(event `self.yukeWhiteyuke.OnComponentBeginOverlap`
  (params (OverlappedComponent :type "PrimitiveComponent Object Reference") (OtherActor :type "Actor Object Reference") (OtherComp :type "PrimitiveComponent Object Reference") (OtherBodyIndex :type Integer) (bFromSweep :type Boolean) (SweepResult :type "HitResult Structure (by ref)"))
  (bind _asyuke_white (cast `/Game/MyContents/BluePrints/Objects/YukeWhite` OtherActor))
  (set `/Game/MyContents/BluePrints/Buttons/BP_ParamGoods.bOnConveyor` false _asyuke_white)
  (goto _label))

(fn `UserConstructionScript`)