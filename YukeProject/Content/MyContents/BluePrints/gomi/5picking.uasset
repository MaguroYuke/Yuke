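; Picking machine actor that moves BP_ParamGoods from nine white, blue and red pickup slots to a transport point.
; Slot overlaps update an occupancy map, which Tick polls to play that slot's Level Sequence, bound to this actor at BeginPlay, one at a time.
; Goods touching Box follow it until HakobuLocation, then get targeted at HakobuLocation1 through their state enum.
; Actors reaching HakobuLocation1 are destroyed after a delay.
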(event `self.ReceiveBeginPlay`
  (bind _output_get (set `self.Binding` (`|MakeMap` "/Game/MyContents/LevelSequences/Picking/Picking_White1.Picking_White1" (`|GetSequenceBinding` null) "/Game/MyContents/LevelSequences/Picking/Picking_Blue1.Picking_Blue1" (`|GetSequenceBinding` null) "/Game/MyContents/LevelSequences/Picking/Picking_Red1.Picking_Red1" (`|GetSequenceBinding` null) "/Game/MyContents/LevelSequences/Picking/Picking_White2.Picking_White2" (`|GetSequenceBinding` null) "/Game/MyContents/LevelSequences/Picking/Picking_Blue2.Picking_Blue2" (`|GetSequenceBinding` null) "/Game/MyContents/LevelSequences/Picking/Picking_Red2.Picking_Red2" (`|GetSequenceBinding` null) "/Game/MyContents/LevelSequences/Picking/Picking_White3.Picking_White3" (`|GetSequenceBinding` null) "/Game/MyContents/LevelSequences/Picking/Picking_Blue3.Picking_Blue3" (`|GetSequenceBinding` null) "/Game/MyContents/LevelSequences/Picking/PickingRed3.PickingRed3" (`|GetSequenceBinding` null) :!type "LevelSequence Object Reference")))
  (bind _keys (`BlueprintMapLibrary.Map_Keys` _output_get))
  (for _array_element _keys
    (bind (_outactor _returnvalue) (`LevelSequencePlayer.CreateLevelSequencePlayer` _array_element))
    (`LevelSequenceActor.SetBinding` _outactor (`BlueprintMapLibrary.Map_Find` (`self.Binding`) _array_element) (`|MakeArray` self :!type "Actor Object Reference") false)
    (`BlueprintMapLibrary.Map_Add` (`self.PickingLevelSequence`) _array_element _returnvalue))
  (`self.InputCollitionName`))

(event `self.ReceiveTick`
  (params (DeltaSeconds :type "Float (single-precision)"))
  (bind _bp_pramamgoods (`self.BP_PramamGoods`))
  (bind (_value _returnvalue) (`BlueprintMapLibrary.Map_Find` (`self.BPE_Picking Or LevelSequence_0`) (`self.PlayString`)))
  (`|ExecutionSequence`
    (:`then_0`
      (bind _keys (`BlueprintMapLibrary.Map_Keys` (`self.spawnallay`)))
      (for _array_element _keys
        (if (`BlueprintMapLibrary.Map_Find` (`self.spawnallay`) _array_element)
          (if (`self.PlaySequence`)
            (if (not (`self.HitHakobuLocation`))
              (bind _output_get (set `self.PlayString` _array_element))
              (`MovieSceneSequencePlayer.Play` (`BlueprintMapLibrary.Map_Find` (`self.PickingLevelSequence`) (`BlueprintMapLibrary.Map_Find` (`self.BPE_Picking Or LevelSequence_0`) _output_get)))
              (set `self.PlaySequence` false))
            (else
              (break)))))
      (if _returnvalue
        (add `MovieSceneSequencePlayer.OnFinished` (`BlueprintMapLibrary.Map_Find` (`self.PickingLevelSequence`) _value) (delegate `NextAnimetion`))))
    (:`then_1`
      (if (`self.HitHakobuLocation`)
        (set `self.Other Comp` null)
        (elif (`KismetSystemLibrary.IsValid` (`self.Other Comp`))
          (`SceneComponent.K2_SetWorldLocation` (`self.Other Comp`) (`SceneComponent.K2_GetComponentLocation` (`self.Box`)) false false))))
    (:`then_2`
      (if (`KismetSystemLibrary.IsValid` (`self.BP_PramamGoods`))
        (switch `/Game/MyContents/BluePrints/Objects/BPE_Artifact` (`/Game/MyContents/BluePrints/Buttons/BP_ParamGoods.BPE_Artifact` (`self.BP_PramamGoods`))
          (:`NewEnumerator0`
            (if (not (`self.HitHakobuLocation1`))
              (set `/Game/MyContents/BluePrints/Buttons/BP_ParamGoods.Target` (`SceneComponent.K2_GetComponentLocation` (`self.HakobuLocation1`)) _bp_pramamgoods)
              (set `/Game/MyContents/BluePrints/Buttons/BP_ParamGoods.BPE_Artifact` "NewEnumerator1" _bp_pramamgoods)))
          (:`NewEnumerator3`
            (set `/Game/MyContents/BluePrints/Buttons/BP_ParamGoods.BPE_Artifact` "NewEnumerator0" (`self.BP_PramamGoods`))
            (set `self.BP_PramamGoods` null)))))))

(event `NextAnimetion`
  (set `self.PlayString` "")
  (set `self.PlaySequence` true))

(event `self.HakobuLocation.OnComponentBeginOverlap`
  (params (OverlappedComponent :type "PrimitiveComponent Object Reference") (OtherActor :type "Actor Object Reference") (OtherComp :type "PrimitiveComponent Object Reference") (OtherBodyIndex :type Integer) (bFromSweep :type Boolean) (SweepResult :type "HitResult Structure (by ref)"))
  (bind _asbp_param_goods (cast `/Game/MyContents/BluePrints/Buttons/BP_ParamGoods` OtherActor))
  (bind _output_get (set `self.BP_PramamGoods` _asbp_param_goods))
  (`SceneComponent.K2_SetWorldLocation` (`/Game/MyContents/BluePrints/Buttons/BP_ParamGoods.Goods` _output_get) (`SceneComponent.K2_GetComponentLocation` (`self.HakobuLocation`)) false false)
  (set `self.HitHakobuLocation` true))

(event `self.HakobuLocation.OnComponentEndOverlap`
  (params (OverlappedComponent :type "PrimitiveComponent Object Reference") (OtherActor :type "Actor Object Reference") (OtherComp :type "PrimitiveComponent Object Reference") (OtherBodyIndex :type Integer))
  (cast `/Game/MyContents/BluePrints/Buttons/BP_ParamGoods` OtherActor)
  (set `self.HitHakobuLocation` false))

(event `self.Box.OnComponentBeginOverlap`
  (params (OverlappedComponent :type "PrimitiveComponent Object Reference") (OtherActor :type "Actor Object Reference") (OtherComp :type "PrimitiveComponent Object Reference") (OtherBodyIndex :type Integer) (bFromSweep :type Boolean) (SweepResult :type "HitResult Structure (by ref)"))
  (bind _asbp_param_goods (cast `/Game/MyContents/BluePrints/Buttons/BP_ParamGoods` OtherActor))
  (set `self.Other Comp` (`/Game/MyContents/BluePrints/Buttons/BP_ParamGoods.Goods` _asbp_param_goods))
  (`ActorComponent.K2_DestroyComponent` (`/Game/MyContents/BluePrints/Buttons/BP_ParamGoods.Dodai` _asbp_param_goods))
  (set `self.Catch` true))

(event `self.Box.OnComponentEndOverlap`
  (params (OverlappedComponent :type "PrimitiveComponent Object Reference") (OtherActor :type "Actor Object Reference") (OtherComp :type "PrimitiveComponent Object Reference") (OtherBodyIndex :type Integer))
  (cast `/Game/MyContents/BluePrints/Buttons/BP_ParamGoods` OtherActor)
  (set `self.Catch` false))

(event `self.HakobuLocation1.OnComponentBeginOverlap`
  (params (OverlappedComponent :type "PrimitiveComponent Object Reference") (OtherActor :type "Actor Object Reference") (OtherComp :type "PrimitiveComponent Object Reference") (OtherBodyIndex :type Integer) (bFromSweep :type Boolean) (SweepResult :type "HitResult Structure (by ref)"))
  (set `self.HitHakobuLocation1` true)
  (`KismetSystemLibrary.Delay` 10.0)
  (`self.K2_DestroyActor` OtherActor))

(event `self.HakobuLocation1.OnComponentEndOverlap`
  (params (OverlappedComponent :type "PrimitiveComponent Object Reference") (OtherActor :type "Actor Object Reference") (OtherComp :type "PrimitiveComponent Object Reference") (OtherBodyIndex :type Integer))
  (set `self.HitHakobuLocation1` false))

(event `self.SpawnLocationWhite1.OnComponentBeginOverlap`
  (params (OverlappedComponent :type "PrimitiveComponent Object Reference") (OtherActor :type "Actor Object Reference") (OtherComp :type "PrimitiveComponent Object Reference") (OtherBodyIndex :type Integer) (bFromSweep :type Boolean) (SweepResult :type "HitResult Structure (by ref)"))
  (bind _asbp_param_goods (cast `/Game/MyContents/BluePrints/Buttons/BP_ParamGoods` OtherActor))
  (`self.HitGoodsObject` (`/Game/MyContents/BluePrints/Buttons/BP_ParamGoods.Goods` _asbp_param_goods) OtherComp (`self.SpawnLocationWhite1`)))

(event `self.SpawnLocationWhite1.OnComponentEndOverlap`
  (params (OverlappedComponent :type "PrimitiveComponent Object Reference") (OtherActor :type "Actor Object Reference") (OtherComp :type "PrimitiveComponent Object Reference") (OtherBodyIndex :type Integer))
  (cast `/Game/MyContents/BluePrints/Buttons/BP_ParamGoods` OtherActor)
  (`self.Hit End Goods Object` (`self.SpawnLocationWhite1`) OtherComp))

(event `self.SpawnLocationWhite2.OnComponentBeginOverlap`
  (params (OverlappedComponent :type "PrimitiveComponent Object Reference") (OtherActor :type "Actor Object Reference") (OtherComp :type "PrimitiveComponent Object Reference") (OtherBodyIndex :type Integer) (bFromSweep :type Boolean) (SweepResult :type "HitResult Structure (by ref)"))
  (bind _asbp_param_goods (cast `/Game/MyContents/BluePrints/Buttons/BP_ParamGoods` OtherActor))
  (`self.HitGoodsObject` (`/Game/MyContents/BluePrints/Buttons/BP_ParamGoods.Goods` _asbp_param_goods) OtherComp (`self.SpawnLocationWhite2`)))

(event `self.SpawnLocationWhite2.OnComponentEndOverlap`
  (params (OverlappedComponent :type "PrimitiveComponent Object Reference") (OtherActor :type "Actor Object Reference") (OtherComp :type "PrimitiveComponent Object Reference") (OtherBodyIndex :type Integer))
  (cast `/Game/MyContents/BluePrints/Buttons/BP_ParamGoods` OtherActor)
  (`self.Hit End Goods Object` (`self.SpawnLocationWhite2`) OtherComp))

(event `self.SpawnLocationWhite3.OnComponentBeginOverlap`
  (params (OverlappedComponent :type "PrimitiveComponent Object Reference") (OtherActor :type "Actor Object Reference") (OtherComp :type "PrimitiveComponent Object Reference") (OtherBodyIndex :type Integer) (bFromSweep :type Boolean) (SweepResult :type "HitResult Structure (by ref)"))
  (bind _asbp_param_goods (cast `/Game/MyContents/BluePrints/Buttons/BP_ParamGoods` OtherActor))
  (`self.HitGoodsObject` (`/Game/MyContents/BluePrints/Buttons/BP_ParamGoods.Goods` _asbp_param_goods) OtherComp (`self.SpawnLocationWhite3`)))

(event `self.SpawnLocationWhite3.OnComponentEndOverlap`
  (params (OverlappedComponent :type "PrimitiveComponent Object Reference") (OtherActor :type "Actor Object Reference") (OtherComp :type "PrimitiveComponent Object Reference") (OtherBodyIndex :type Integer))
  (cast `/Game/MyContents/BluePrints/Buttons/BP_ParamGoods` OtherActor)
  (`self.Hit End Goods Object` (`self.SpawnLocationWhite3`) OtherComp))

(event `self.SpawnLocationBlue1.OnComponentBeginOverlap`
  (params (OverlappedComponent :type "PrimitiveComponent Object Reference") (OtherActor :type "Actor Object Reference") (OtherComp :type "PrimitiveComponent Object Reference") (OtherBodyIndex :type Integer) (bFromSweep :type Boolean) (SweepResult :type "HitResult Structure (by ref)"))
  (bind _asbp_param_goods (cast `/Game/MyContents/BluePrints/Buttons/BP_ParamGoods` OtherActor))
  (`self.HitGoodsObject` (`/Game/MyContents/BluePrints/Buttons/BP_ParamGoods.Goods` _asbp_param_goods) OtherComp (`self.SpawnLocationBlue1`)))

(event `self.SpawnLocationBlue1.OnComponentEndOverlap`
  (params (OverlappedComponent :type "PrimitiveComponent Object Reference") (OtherActor :type "Actor Object Reference") (OtherComp :type "PrimitiveComponent Object Reference") (OtherBodyIndex :type Integer))
  (cast `/Game/MyContents/BluePrints/Buttons/BP_ParamGoods` OtherActor)
  (`self.Hit End Goods Object` (`self.SpawnLocationBlue1`) OtherComp))

(event `self.SpawnLocationBlue2.OnComponentBeginOverlap`
  (params (OverlappedComponent :type "PrimitiveComponent Object Reference") (OtherActor :type "Actor Object Reference") (OtherComp :type "PrimitiveComponent Object Reference") (OtherBodyIndex :type Integer) (bFromSweep :type Boolean) (SweepResult :type "HitResult Structure (by ref)"))
  (bind _asbp_param_goods (cast `/Game/MyContents/BluePrints/Buttons/BP_ParamGoods` OtherActor))
  (`self.HitGoodsObject` (`/Game/MyContents/BluePrints/Buttons/BP_ParamGoods.Goods` _asbp_param_goods) OtherComp (`self.SpawnLocationBlue2`)))

(event `self.SpawnLocationBlue2.OnComponentEndOverlap`
  (params (OverlappedComponent :type "PrimitiveComponent Object Reference") (OtherActor :type "Actor Object Reference") (OtherComp :type "PrimitiveComponent Object Reference") (OtherBodyIndex :type Integer))
  (cast `/Game/MyContents/BluePrints/Buttons/BP_ParamGoods` OtherActor)
  (`self.Hit End Goods Object` (`self.SpawnLocationBlue2`) OtherComp))

(event `self.SpawnLocationBlue3.OnComponentBeginOverlap`
  (params (OverlappedComponent :type "PrimitiveComponent Object Reference") (OtherActor :type "Actor Object Reference") (OtherComp :type "PrimitiveComponent Object Reference") (OtherBodyIndex :type Integer) (bFromSweep :type Boolean) (SweepResult :type "HitResult Structure (by ref)"))
  (bind _asbp_param_goods (cast `/Game/MyContents/BluePrints/Buttons/BP_ParamGoods` OtherActor))
  (`self.HitGoodsObject` (`/Game/MyContents/BluePrints/Buttons/BP_ParamGoods.Goods` _asbp_param_goods) OtherComp (`self.SpawnLocationBlue3`)))

(event `self.SpawnLocationBlue3.OnComponentEndOverlap`
  (params (OverlappedComponent :type "PrimitiveComponent Object Reference") (OtherActor :type "Actor Object Reference") (OtherComp :type "PrimitiveComponent Object Reference") (OtherBodyIndex :type Integer))
  (cast `/Game/MyContents/BluePrints/Buttons/BP_ParamGoods` OtherActor)
  (`self.Hit End Goods Object` (`self.SpawnLocationBlue3`) OtherComp))

(event `self.SpawnLocationRed1.OnComponentBeginOverlap`
  (params (OverlappedComponent :type "PrimitiveComponent Object Reference") (OtherActor :type "Actor Object Reference") (OtherComp :type "PrimitiveComponent Object Reference") (OtherBodyIndex :type Integer) (bFromSweep :type Boolean) (SweepResult :type "HitResult Structure (by ref)"))
  (bind _asbp_param_goods (cast `/Game/MyContents/BluePrints/Buttons/BP_ParamGoods` OtherActor))
  (`self.HitGoodsObject` (`/Game/MyContents/BluePrints/Buttons/BP_ParamGoods.Goods` _asbp_param_goods) OtherComp (`self.SpawnLocationRed1`)))

(event `self.SpawnLocationRed1.OnComponentEndOverlap`
  (params (OverlappedComponent :type "PrimitiveComponent Object Reference") (OtherActor :type "Actor Object Reference") (OtherComp :type "PrimitiveComponent Object Reference") (OtherBodyIndex :type Integer))
  (cast `/Game/MyContents/BluePrints/Buttons/BP_ParamGoods` OtherActor)
  (`self.Hit End Goods Object` (`self.SpawnLocationRed1`) OtherComp))

(event `self.SpawnLocationRed2.OnComponentBeginOverlap`
  (params (OverlappedComponent :type "PrimitiveComponent Object Reference") (OtherActor :type "Actor Object Reference") (OtherComp :type "PrimitiveComponent Object Reference") (OtherBodyIndex :type Integer) (bFromSweep :type Boolean) (SweepResult :type "HitResult Structure (by ref)"))
  (bind _asbp_param_goods (cast `/Game/MyContents/BluePrints/Buttons/BP_ParamGoods` OtherActor))
  (`self.HitGoodsObject` (`/Game/MyContents/BluePrints/Buttons/BP_ParamGoods.Goods` _asbp_param_goods) OtherComp (`self.SpawnLocationRed2`)))

(event `self.SpawnLocationRed2.OnComponentEndOverlap`
  (params (OverlappedComponent :type "PrimitiveComponent Object Reference") (OtherActor :type "Actor Object Reference") (OtherComp :type "PrimitiveComponent Object Reference") (OtherBodyIndex :type Integer))
  (cast `/Game/MyContents/BluePrints/Buttons/BP_ParamGoods` OtherActor)
  (`self.Hit End Goods Object` (`self.SpawnLocationRed2`) OtherComp))

(event `self.SpawnLocationRed3.OnComponentBeginOverlap`
  (params (OverlappedComponent :type "PrimitiveComponent Object Reference") (OtherActor :type "Actor Object Reference") (OtherComp :type "PrimitiveComponent Object Reference") (OtherBodyIndex :type Integer) (bFromSweep :type Boolean) (SweepResult :type "HitResult Structure (by ref)"))
  (bind _asbp_param_goods (cast `/Game/MyContents/BluePrints/Buttons/BP_ParamGoods` OtherActor))
  (`self.HitGoodsObject` (`/Game/MyContents/BluePrints/Buttons/BP_ParamGoods.Goods` _asbp_param_goods) OtherComp (`self.SpawnLocationRed3`)))

(event `self.SpawnLocationRed3.OnComponentEndOverlap`
  (params (OverlappedComponent :type "PrimitiveComponent Object Reference") (OtherActor :type "Actor Object Reference") (OtherComp :type "PrimitiveComponent Object Reference") (OtherBodyIndex :type Integer))
  (cast `/Game/MyContents/BluePrints/Buttons/BP_ParamGoods` OtherActor)
  (`self.Hit End Goods Object` (`self.SpawnLocationRed3`) OtherComp))

(fn `Hit End Goods Object`
  (params (SpawnLocation :type "Object Object Reference") (OtherComp :type "PrimitiveComponent Object Reference"))
  (`BlueprintMapLibrary.Map_Add` (`self.spawnallay`) (`KismetSystemLibrary.GetObjectName` SpawnLocation))
  (`PrimitiveComponent.SetSimulatePhysics` OtherComp false))

(fn `HitGoodsObject`
  (params (Goods :type "SceneComponent Object Reference") (OtherComp :type "PrimitiveComponent Object Reference") (SpawnLocation :type "BoxComponent Object Reference"))
  (`PrimitiveComponent.SetSimulatePhysics` OtherComp false)
  (if (not (`KismetSystemLibrary.IsValid` (`self.Other Comp`)))
    (`BlueprintMapLibrary.Map_Add` (`self.spawnallay`) (`KismetSystemLibrary.GetObjectName` SpawnLocation) true)
    (`SceneComponent.K2_SetWorldLocationAndRotation` :`self` Goods :`NewLocation` (`SceneComponent.K2_GetComponentLocation` SpawnLocation))
    (`KismetSystemLibrary.PrintString` "位置が変わります")))

(fn `InputCollitionName`
  (bind _spawnlocationwhite1 (`self.SpawnLocationWhite1`))
  (bind _spawnlocationwhite2 (`self.SpawnLocationWhite2`))
  (bind _spawnlocationwhite3 (`self.SpawnLocationWhite3`))
  (bind _spawnlocationred1 (`self.SpawnLocationRed1`))
  (bind _spawnlocationred2 (`self.SpawnLocationRed2`))
  (bind _spawnlocationred3 (`self.SpawnLocationRed3`))
  (bind _spawnlocationblue3 (`self.SpawnLocationBlue3`))
  (bind _spawnlocationblue1 (`self.SpawnLocationBlue1`))
  (bind _spawnlocationblue2 (`self.SpawnLocationBlue2`))
  (bind _returnvalue (`KismetSystemLibrary.GetObjectName` _spawnlocationblue3))
  (bind _returnvalue_2 (`KismetSystemLibrary.GetObjectName` _spawnlocationblue1))
  (bind _returnvalue_3 (`KismetSystemLibrary.GetObjectName` _spawnlocationblue2))
  (bind _returnvalue_4 (`KismetSystemLibrary.GetObjectName` _spawnlocationwhite1))
  (bind _returnvalue_5 (`KismetSystemLibrary.GetObjectName` _spawnlocationwhite2))
  (bind _returnvalue_6 (`KismetSystemLibrary.GetObjectName` _spawnlocationwhite3))
  (bind _returnvalue_7 (`KismetSystemLibrary.GetObjectName` _spawnlocationred1))
  (bind _returnvalue_8 (`KismetSystemLibrary.GetObjectName` _spawnlocationred2))
  (bind _returnvalue_9 (`KismetSystemLibrary.GetObjectName` _spawnlocationred3))
  (`BlueprintMapLibrary.Map_Add` (`self.spawnallay`) _returnvalue_4)
  (`BlueprintMapLibrary.Map_Add` (`self.Spawn Location`) _returnvalue_4 _spawnlocationwhite1)
  (`BlueprintMapLibrary.Map_Add` (`self.BPE_Picking Or LevelSequence_0`) _returnvalue_4 "/Game/MyContents/LevelSequences/Picking/Picking_White1.Picking_White1")
  (`BlueprintMapLibrary.Map_Add` (`self.spawnallay`) _returnvalue_5)
  (`BlueprintMapLibrary.Map_Add` (`self.Spawn Location`) _returnvalue_5 _spawnlocationwhite2)
  (`BlueprintMapLibrary.Map_Add` (`self.BPE_Picking Or LevelSequence_0`) _returnvalue_5 "/Game/MyContents/LevelSequences/Picking/Picking_White2.Picking_White2")
  (`BlueprintMapLibrary.Map_Add` (`self.spawnallay`) _returnvalue_6)
  (`BlueprintMapLibrary.Map_Add` (`self.Spawn Location`) _returnvalue_6 _spawnlocationwhite3)
  (`BlueprintMapLibrary.Map_Add` (`self.BPE_Picking Or LevelSequence_0`) _returnvalue_6 "/Game/MyContents/LevelSequences/Picking/Picking_White3.Picking_White3")
  (`BlueprintMapLibrary.Map_Add` (`self.spawnallay`) _returnvalue_7)
  (`BlueprintMapLibrary.Map_Add` (`self.Spawn Location`) _returnvalue_7 _spawnlocationred1)
  (`BlueprintMapLibrary.Map_Add` (`self.BPE_Picking Or LevelSequence_0`) _returnvalue_7 "/Game/MyContents/LevelSequences/Picking/Picking_Red1.Picking_Red1")
  (`BlueprintMapLibrary.Map_Add` (`self.spawnallay`) _returnvalue_8)
  (`BlueprintMapLibrary.Map_Add` (`self.Spawn Location`) _returnvalue_8 _spawnlocationred2)
  (`BlueprintMapLibrary.Map_Add` (`self.BPE_Picking Or LevelSequence_0`) _returnvalue_8 "/Game/MyContents/LevelSequences/Picking/Picking_Red2.Picking_Red2")
  (`BlueprintMapLibrary.Map_Add` (`self.spawnallay`) _returnvalue_9)
  (`BlueprintMapLibrary.Map_Add` (`self.Spawn Location`) _returnvalue_9 _spawnlocationred3)
  (`BlueprintMapLibrary.Map_Add` (`self.BPE_Picking Or LevelSequence_0`) _returnvalue_9 "/Game/MyContents/LevelSequences/Picking/PickingRed3.PickingRed3")
  (`BlueprintMapLibrary.Map_Add` (`self.spawnallay`) _returnvalue_2)
  (`BlueprintMapLibrary.Map_Add` (`self.Spawn Location`) _returnvalue_2 _spawnlocationblue1)
  (`BlueprintMapLibrary.Map_Add` (`self.BPE_Picking Or LevelSequence_0`) _returnvalue_2 "/Game/MyContents/LevelSequences/Picking/Picking_Blue1.Picking_Blue1")
  (`BlueprintMapLibrary.Map_Add` (`self.spawnallay`) _returnvalue_3)
  (`BlueprintMapLibrary.Map_Add` (`self.Spawn Location`) _returnvalue_3 _spawnlocationblue2)
  (`BlueprintMapLibrary.Map_Add` (`self.BPE_Picking Or LevelSequence_0`) _returnvalue_3 "/Game/MyContents/LevelSequences/Picking/Picking_Blue2.Picking_Blue2")
  (`BlueprintMapLibrary.Map_Add` (`self.spawnallay`) _returnvalue)
  (`BlueprintMapLibrary.Map_Add` (`self.Spawn Location`) _returnvalue _spawnlocationblue3)
  (`BlueprintMapLibrary.Map_Add` (`self.BPE_Picking Or LevelSequence_0`) _returnvalue "/Game/MyContents/LevelSequences/Picking/Picking_Blue3.Picking_Blue3"))

(fn `UserConstructionScript`)