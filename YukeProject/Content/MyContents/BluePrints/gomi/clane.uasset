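; Crane actor that lowers to pick up a BP_Goods item and carries it back to its starting position.
; Tick runs an enum state machine, stepping the Clane component via StartMove and MoveActor.
; A StopCollision overlap records the goods and starts movement toward zero Z; Box touching that item triggers the return.
; During later movement, the goods snap to Box while Pillar's yaw interpolates toward Targetcube.
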(event `self.ReceiveBeginPlay`
  (bind _clane (`self.clane`))
  (bind (_returnvalue_x _returnvalue_y) (`KismetMathLibrary.BreakVector` (`SceneComponent.K2_GetComponentLocation` _clane)))
  (set `self.start` (`SceneComponent.K2_GetComponentLocation` _clane))
  (set `self.Next` (`KismetMathLibrary.MakeVector` _returnvalue_x _returnvalue_y))
  (`self.InitLocation`)
  (set `self.Speed` 10.0)
  (`KismetSystemLibrary.PrintString` "初期設定")
  (set `self.BPE_Artifact` "NewEnumerator0")
  (`PrimitiveComponent.SetSimulatePhysics` (`self.StopEria`) false))

(event `self.ReceiveTick`
  (params (DeltaSeconds :type "Float (single-precision)"))
  (bind _bp_goods (`self.BP_Goods`))
  (bind _returnvalue (`SceneComponent.K2_GetComponentLocation` (`self.Box`)))
  (bind _returnvalue_2 (`SceneComponent.K2_GetComponentLocation` (`self.Pillar`)))
  (bind (_returnvalue_roll _returnvalue_pitch _returnvalue_yaw) (`KismetMathLibrary.BreakRotator` (`KismetMathLibrary.RInterpTo` (`KismetMathLibrary.Conv_VectorToRotator` _returnvalue_2) (`KismetMathLibrary.FindLookAtRotation` _returnvalue_2 (`self.Targetcube`)) (`GameplayStatics.GetWorldDeltaSeconds`) (`self.RSpeed`))))
  (switch `/Game/MyContents/BluePrints/Objects/BPE_Artifact` (`self.BPE_Artifact`)
    (:`NewEnumerator1`
      (`self.StartMove` (`SceneComponent.K2_GetComponentLocation` (`self.clane`)) (`self.Next`))
      (set `self.BPE_Artifact` "NewEnumerator2"))
    (:`NewEnumerator2`
      (bind (_location _onmove) (`self.MoveActor` (`SceneComponent.K2_GetComponentLocation` (`self.clane`))))
      (`SceneComponent.K2_SetWorldLocation` (`self.clane`) _location false false)
      (if _onmove
        (if (`self.NewVar`)
          (if (`KismetSystemLibrary.IsValid` _bp_goods)
            (`KismetSystemLibrary.PrintString` (`KismetStringLibrary.Conv_VectorToString` (`self.K2_GetActorLocation` _bp_goods)))
            (`SceneComponent.K2_SetWorldLocation` (`/Game/MyContents/BluePrints/Objects/BP_Goods.Goods` _bp_goods) _returnvalue false false)
            (`self.K2_SetActorLocation` _bp_goods _returnvalue false false)
            (`SceneComponent.K2_SetWorldRotation` (`self.Pillar`) (`KismetMathLibrary.MakeRotator` 0.0 0.0 _returnvalue_yaw) false false)))
        (else
          (set `self.BPE_Artifact` "NewEnumerator0"))))
    (:`NewEnumerator3`
      (`self.StartMove` (`SceneComponent.K2_GetComponentLocation` (`self.clane`)) (`self.start`))
      (set `self.BPE_Artifact` "NewEnumerator2"))))

(event `self.Box.OnComponentBeginOverlap`
  (params (OverlappedComponent :type "PrimitiveComponent Object Reference") (OtherActor :type "Actor Object Reference") (OtherComp :type "PrimitiveComponent Object Reference") (OtherBodyIndex :type Integer) (bFromSweep :type Boolean) (SweepResult :type "HitResult Structure (by ref)"))
  (bind _asbp_goods (cast `/Game/MyContents/BluePrints/Objects/BP_Goods` OtherActor))
  (`PrimitiveComponent.SetSimulatePhysics` (`/Game/MyContents/BluePrints/Objects/BP_Goods.Goods` _asbp_goods) false)
  (if (== _asbp_goods (`self.BP_Goods`))
    (`KismetSystemLibrary.PrintString` "降れた")
    (set `self.BPE_Artifact` "NewEnumerator3")
    (set `self.NewVar` true)
    (else
      (`KismetSystemLibrary.PrintString` "違う"))))

(event `self.Box.OnComponentEndOverlap`
  (params (OverlappedComponent :type "PrimitiveComponent Object Reference") (OtherActor :type "Actor Object Reference") (OtherComp :type "PrimitiveComponent Object Reference") (OtherBodyIndex :type Integer)))

(event `self.StopCollision.OnComponentBeginOverlap`
  (params (OverlappedComponent :type "PrimitiveComponent Object Reference") (OtherActor :type "Actor Object Reference") (OtherComp :type "PrimitiveComponent Object Reference") (OtherBodyIndex :type Integer) (bFromSweep :type Boolean) (SweepResult :type "HitResult Structure (by ref)"))
  (bind _asbp_goods (cast `/Game/MyContents/BluePrints/Objects/BP_Goods` OtherActor))
  (set `self.BP_Goods` _asbp_goods)
  (`KismetSystemLibrary.PrintString` "actor")
  (set `self.BPE_Artifact` "NewEnumerator1"))

(fn `UserConstructionScript`)