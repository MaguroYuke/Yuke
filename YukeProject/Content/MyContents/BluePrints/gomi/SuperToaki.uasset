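; SuperToaki is a machine actor that carries BP_ParamGoods through overlap-box stations, animated by the 4Move level sequence bound to itself at BeginPlay.
; Tablebox grabs goods, disables their physics and plays the sequence, while Tick snaps them to the current target or to the Bakyumu and Kaiten stations.
; Box3 and Oshidashibox restore physics, the latter adding spin or push force; KonbeaBox notifies goods.
; Flag H spawns YukeBlue and replays the sequence.
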(event `self.ReceiveBeginPlay`
  (bind (_outactor _returnvalue) (`LevelSequencePlayer.CreateLevelSequencePlayer` "/Game/MyContents/LevelSequences/4Move.4Move" (make `MovieSceneSequencePlaybackSettings` false)))
  (`LevelSequenceActor.SetBinding` _outactor (`|GetSequenceBinding` null) (`|MakeArray` self :!type "Actor Object Reference") false)
  (`KismetSystemLibrary.PrintString` (`KismetSystemLibrary.GetObjectName` _outactor))
  (set `self.LevelSequence` _returnvalue)
  (`MovieSceneSequencePlayer.SetPlayRate` (`self.LevelSequence`) 1.0)
  (set `self.BPE_WorldObject` "NewEnumerator2")
  (`PrimitiveComponent.SetSimulatePhysics` (`self.4dodai`) false))

(event `self.ReceiveTick`
  (params (DeltaSeconds :type "Float (single-precision)"))
  (bind _target (`self.Target`))
  (bind _other_comp (`self.Other Comp`))
  (`|ExecutionSequence`
    (:`then_0`
      (if true
        (if (and (`KismetSystemLibrary.IsValid` _other_comp) (`KismetSystemLibrary.IsValid` _target))
          (`SceneComponent.K2_SetWorldLocation` _other_comp (`SceneComponent.K2_GetComponentLocation` _target) false false)
          (if (`self.bakyu--mu`)
            (bind _goods (`/Game/MyContents/BluePrints/Buttons/BP_ParamGoods.Goods` (stale `self.tablebox.OnComponentBeginOverlap` _asbp_param_goods)))
            (`SceneComponent.K2_SetWorldLocationAndRotation` :`self` _goods :`NewLocation` (`SceneComponent.K2_GetComponentLocation` (`self.bakyu--------------mu`)))
            (if (`self.kaiten`)
              (`SceneComponent.K2_SetWorldLocationAndRotation` :`self` _goods :`NewLocation` (`SceneComponent.K2_GetComponentLocation` (`self.kaitenbox`)))
              (set `self.bakyu--mu` false))))))
    (:`then_1`
      (if (`self.H`)
        (if true
          (`|SpawnActorFromClass` "/Game/MyContents/BluePrints/Objects/YukeBlue.YukeBlue_C" (`KismetMathLibrary.MakeTransform` (`SceneComponent.K2_GetComponentLocation` (`self.Box`))) "Undefined" "MultiplyWithRoot" null null)
          (set `self.H` false)
          (`MovieSceneSequencePlayer.Play` (`self.LevelSequence`)))))
    (:`then_2`
      (if true
        _))))

(event `self.tablebox.OnComponentBeginOverlap`
  (params (OverlappedComponent :type "PrimitiveComponent Object Reference") (OtherActor :type "Actor Object Reference") (OtherComp :type "PrimitiveComponent Object Reference") (OtherBodyIndex :type Integer) (bFromSweep :type Boolean) (SweepResult :type "HitResult Structure (by ref)"))
  (if (!= (`self.Target`) (`self.tablebox`))
    (bind _asbp_param_goods (cast `/Game/MyContents/BluePrints/Buttons/BP_ParamGoods` OtherActor))
    (set `self.Other Comp` OtherComp)
    (set `self.Target` (`self.tablebox`))
    (`PrimitiveComponent.SetSimulatePhysics` OtherComp false)
    (`MovieSceneSequencePlayer.Play` (`self.LevelSequence`))))

(event `self.Box1.OnComponentBeginOverlap`
  (params (OverlappedComponent :type "PrimitiveComponent Object Reference") (OtherActor :type "Actor Object Reference") (OtherComp :type "PrimitiveComponent Object Reference") (OtherBodyIndex :type Integer) (bFromSweep :type Boolean) (SweepResult :type "HitResult Structure (by ref)"))
  (if (!= (`self.Target`) (`self.Box1`))
    (cast `/Game/MyContents/BluePrints/Buttons/BP_ParamGoods` OtherActor)
    (set `self.Target` (`self.Box1`))
    (`KismetSystemLibrary.PrintString` "呼ばれちゃったよ第二")))

(event `Key|H`
  (params (Key :type "Key Structure")))

(event `self.kaitenbox.OnComponentBeginOverlap`
  (params (OverlappedComponent :type "PrimitiveComponent Object Reference") (OtherActor :type "Actor Object Reference") (OtherComp :type "PrimitiveComponent Object Reference") (OtherBodyIndex :type Integer) (bFromSweep :type Boolean) (SweepResult :type "HitResult Structure (by ref)"))
  (if (!= (`self.Target`) (`self.kaitenbox`))
    (cast `/Game/MyContents/BluePrints/Buttons/BP_ParamGoods` OtherActor)
    (set `self.Target` (`self.kaitenbox`))
    (set `self.bakyu--mu` false)
    (set `self.kaiten` true)
    (`KismetSystemLibrary.PrintString` "呼ばれちゃったよ第三")))

(event `self.Box3.OnComponentBeginOverlap`
  (params (OverlappedComponent :type "PrimitiveComponent Object Reference") (OtherActor :type "Actor Object Reference") (OtherComp :type "PrimitiveComponent Object Reference") (OtherBodyIndex :type Integer) (bFromSweep :type Boolean) (SweepResult :type "HitResult Structure (by ref)"))
  (cast `/Game/MyContents/BluePrints/Buttons/BP_ParamGoods` OtherActor)
  (`PrimitiveComponent.SetSimulatePhysics` OtherComp true)
  (set `self.Other Comp` null))

(event `self.konbeaBox.OnComponentBeginOverlap`
  (params (OverlappedComponent :type "PrimitiveComponent Object Reference") (OtherActor :type "Actor Object Reference") (OtherComp :type "PrimitiveComponent Object Reference") (OtherBodyIndex :type Integer) (bFromSweep :type Boolean) (SweepResult :type "HitResult Structure (by ref)"))
  (bind _konbeabox (`self.konbeaBox`))
  (bind _asbp_param_goods (cast `/Game/MyContents/BluePrints/Buttons/BP_ParamGoods` OtherActor))
  (`/Game/MyContents/BluePrints/Buttons/BP_ParamGoods.B` _asbp_param_goods _konbeabox)
  (`PrimitiveComponent.SetSimulatePhysics` _konbeabox false))

(event `self.konbeaBox.OnComponentEndOverlap`
  (params (OverlappedComponent :type "PrimitiveComponent Object Reference") (OtherActor :type "Actor Object Reference") (OtherComp :type "PrimitiveComponent Object Reference") (OtherBodyIndex :type Integer))
  (bind _asbp_param_goods (cast `/Game/MyContents/BluePrints/Buttons/BP_ParamGoods` OtherActor)))

(event `self.bakyu--------------mu.OnComponentBeginOverlap`
  (params (OverlappedComponent :type "PrimitiveComponent Object Reference") (OtherActor :type "Actor Object Reference") (OtherComp :type "PrimitiveComponent Object Reference") (OtherBodyIndex :type Integer) (bFromSweep :type Boolean) (SweepResult :type "HitResult Structure (by ref)"))
  (cast `/Game/MyContents/BluePrints/Buttons/BP_ParamGoods` OtherActor)
  (set `self.bakyu--mu` true))

(event `self.oshidashibox.OnComponentBeginOverlap`
  (params (OverlappedComponent :type "PrimitiveComponent Object Reference") (OtherActor :type "Actor Object Reference") (OtherComp :type "PrimitiveComponent Object Reference") (OtherBodyIndex :type Integer) (bFromSweep :type Boolean) (SweepResult :type "HitResult Structure (by ref)"))
  (bind _asbp_param_goods (cast `/Game/MyContents/BluePrints/Buttons/BP_ParamGoods` OtherActor))
  (set `self.kaiten` false)
  (bind _goods (`/Game/MyContents/BluePrints/Buttons/BP_ParamGoods.Goods` _asbp_param_goods))
  (`PrimitiveComponent.SetSimulatePhysics` _goods true)
  (`PrimitiveComponent.SetPhysicsAngularVelocityInRadians` _goods (6000.0 0.0 0.0) true "None"))

(event `self.oshidashibox.OnComponentHit`
  (params (HitComponent :type "PrimitiveComponent Object Reference") (OtherActor :type "Actor Object Reference") (OtherComp :type "PrimitiveComponent Object Reference") (NormalImpulse :type "Vector Structure") (Hit :type "HitResult Structure (by ref)"))
  (bind _asbp_param_goods (cast `/Game/MyContents/BluePrints/Buttons/BP_ParamGoods` OtherActor))
  (`PrimitiveComponent.AddForce` (`/Game/MyContents/BluePrints/Buttons/BP_ParamGoods.Goods` _asbp_param_goods) (* (`KismetMathLibrary.GetForwardVector` (`self.K2_GetActorRotation` _asbp_param_goods)) (`self.Power1`)) "None" false))

(fn `UserConstructionScript`)