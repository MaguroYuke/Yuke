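; BP_Goods is a goods actor that travels through a queue of BP_StopEria stop areas and destroys itself when none remain.
; Tick runs an enum state machine (stop, start, moving, end, delete) with delays, showing state and progress in a text widget.
; It departs only when checks on other goods and target occupancy find no conflict.
; After arrival, NextEria removes the reached area and restarts the cycle; deletion updates an actor-count widget.
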(event `self.ReceiveBeginPlay`
  (`self.InitLocation`) ; 移動する変数の初期化
  (`self.InitActorWidget` (make `SlateColor` (struct :`R` 0.870817 :`B` 1.0 :`A` 1.0))) ; ウィジットの初期化
  (set `self.NoStart` false)
  (set `self.Remove` false)
  (set `self.Delete` false)
  (`PrimitiveComponent.SetSimulatePhysics` (`self.Goods`) false))

(event `self.ReceiveTick`
  (params (DeltaSeconds :type "Float (single-precision)"))
  (if (`self.ActorStart`)
    (bind _outactors (`GameplayStatics.GetAllActorsOfClass` "/Game/MyContents/BluePrints/Objects/BP_StopEria.BP_StopEria_C"))
    (set `self.ClearObj` (`KismetStringLibrary.Concat_StrStr` "｜" "完了数" "｜" (`KismetStringLibrary.Conv_IntToString` (`KismetArrayLibrary.Array_Length` (`self.ALLTarget`))) "/" (`KismetStringLibrary.Conv_IntToString` (`KismetArrayLibrary.Array_Length` _outactors))))
    (switch `/Game/MyContents/BluePrints/Objects/BPE_Artifact` (`self.BPE_Artifact`)
      (:`NewEnumerator0`
        (`self.Stop`) ; 止まっているとき
      )
      (:`NewEnumerator1`
        (`self.Start`) ; 移動開始するとき
        (`KismetSystemLibrary.Delay` (`self.Delay`))
        (set `self.BPE_Artifact` "NewEnumerator2"))
      (:`NewEnumerator2`
        (bind _onmove (`self.UpData`)) ; 移動中のとき
        (if (not _onmove)
          (set `self.BPE_Artifact` "NewEnumerator3")))
      (:`NewEnumerator3`
        (bind _remove (`self.End`)) ; 移動終了のとき
        (if (not _remove)
          (`KismetSystemLibrary.Delay` (`self.Delay`))
          (set `self.Remove` true)))
      (:`NewEnumerator4`
        (bind _delete (`self.Destroy`)) ; 削除したいとき
        (if (not _delete)
          (`KismetSystemLibrary.Delay` (`self.Delay`))
          (set `self.Delete` true))))))

(event `NextEria`
  (params (StopEria :type "/Game/MyContents/BluePrints/Objects/BP_StopEria Object Reference"))
  (bind _target (`self.TargetPos`))
  (if _target
    (set `self.Remove` false)
    (`KismetArrayLibrary.Array_RemoveItem` (`self.ALLTarget`) StopEria)
    (set `self.BPE_Artifact` "NewEnumerator0")))

(fn `Destroy`
  (returns (Delete :type Boolean))
  (`self.SetText` (`KismetStringLibrary.Concat_StrStr` "削除" (`self.ClearObj`)))
  (if (`self.Delete`)
    (`/Game/MyContents/BluePrints/Objects/BPW_ActorCount.ClearActor` (`self.BPW_ActorCount`))
    (`self.K2_DestroyActor`)
    (return true)
    (else
      (return false))))

(fn `End`
  (returns (Remove :type Boolean))
  (if (`self.Remove`)
    (`self.SetText` (`KismetStringLibrary.Concat_StrStr` "停止中" (`self.ClearObj`)))
    (return true)
    (else
      (`self.SetText` (`KismetStringLibrary.Concat_StrStr` "到着" (`self.ClearObj`)))
      (return false))))

(fn `Start`
  (`self.SetText` (`KismetStringLibrary.Concat_StrStr` "開始" (`self.ClearObj`)))
  (`self.StartMove` (`self.K2_GetActorLocation`) (`self.K2_GetActorLocation` (`|GetArrayItem` (`self.ALLTarget`)))) ; 移動先を登録
)

(fn `Stop`
  (if (> (`KismetArrayLibrary.Array_Length` (`self.ALLTarget`)) 0)
    (set `self.NoStart` false)
    (bind _outactors (`GameplayStatics.GetAllActorsOfClass` "BP_Goods_C"))
    (for _array_element _outactors
      (if (and (or (`self.Target_Artifact` _array_element) (`self.Target_HitAllActors`)) (`self.ALLTarget_Object` _array_element))
        (set `self.NoStart` true)))
    (if (not (`self.NoStart`))
      (set `self.BPE_Artifact` "NewEnumerator1"))
    (else
      (set `self.BPE_Artifact` "NewEnumerator4"))))

(fn `TargetPos`
  (returns (Target :type Boolean))
  (return (and (`|EnumEquality` (`self.BPE_Artifact`) "NewEnumerator3") (`self.Remove`))))

(fn `UpData`
  (returns (OnMove :type Boolean))
  (`self.SetText` (`KismetStringLibrary.Concat_StrStr` "移動中" (`self.ClearObj`)))
  (bind (_location _onmove) (`self.MoveActor` (`self.K2_GetActorLocation`))) ; 移動中
  (`self.K2_SetActorLocation` _location)
  (return _onmove))

(fn `UserConstructionScript`)