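; BP_Element is a world object actor that displays named progress items on a production-quantity widget, which starts hidden.
; InitProgress creates an item, and UpDataProgress caps its value at the maximum, stores both in maps keyed by text and refreshes the bar, setting the color flag when full or requested.
; Tick scales the widget inversely with player pawn distance, within clamped limits.
; Init stores the world-object value and an override material.
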(event `self.ReceiveBeginPlay`
  (`|ExecutionSequence`
    (:`then_0`
      ;[1 1 1] オブジェクトのウィジットを格納
      (bind _asbpw_element (cast `/Game/MyContents/Widget/ObjectWidget/BPW_ProductionQuantity` (`WidgetComponent.GetWidget` (`self.Widget`))))
      (bind _output_get (set `self.As BPW Element` _asbpw_element))
      (`Widget.SetVisibility` _output_get "Hidden"))))

(event `self.ReceiveTick`
  (params (DeltaSeconds :type "Float (single-precision)"))
  (bind _returnvalue (/ 5000.0 (`KismetMathLibrary.Vector_Distance` (`self.K2_GetActorLocation` (`Controller.K2_GetPawn` (`GameplayStatics.GetPlayerController` 0))) (`SceneComponent.K2_GetComponentLocation` (`self.Widget`)))))
  (bind (_returnvalue_x _returnvalue_y) (`KismetMathLibrary.BreakVector` (`KismetMathLibrary.ClampVectorSize` (`KismetMathLibrary.MakeVector` _returnvalue _returnvalue) 0.5 2.0)))
  ;[1 1 1] ウィジットの配置の調整
  (`Widget.SetRenderScale` (`WidgetComponent.GetWidget` (`self.Widget`)) (`KismetMathLibrary.MakeVector2D` _returnvalue_x _returnvalue_y)))

(event `InitProgress`
  (params (Progress :type "Float (double-precision)") (MaxProgress :type "Float (double-precision)") (TextString :type String) (MaximumFractionalDigits :type Integer) (ProgressVisibility :type "ESlateVisibility Enum" :default "Visible"))
  ;[1 1 1] Itemを作成
  (`BlueprintMapLibrary.Map_Add` (`self.Progress`) TextString Progress)
  (`BlueprintMapLibrary.Map_Add` (`self.MaxProgress`) TextString MaxProgress)
  (`/Game/MyContents/Widget/ObjectWidget/BPW_ProductionQuantity.InstanceItem` (`self.As BPW Element`) TextString (`BlueprintMapLibrary.Map_Find` (`self.Progress`) TextString) (`BlueprintMapLibrary.Map_Find` (`self.MaxProgress`) TextString) MaximumFractionalDigits ProgressVisibility))

(event `UpDataProgress`
  (params (TextString :type String) (MaxProgress :type "Float (double-precision)") (Progress :type "Float (double-precision)") (SetColorProgress :type Boolean))
  (bind _progress (`self.Progress`))
  (bind _value (`BlueprintMapLibrary.Map_Find` (`self.Progress`) TextString))
  (bind _value_2 (`BlueprintMapLibrary.Map_Find` (`self.MaxProgress`) TextString))
  (bind _value_3 (`BlueprintMapLibrary.Map_Find` (`self.MaxProgress`) TextString))
  ;[1 1 1] ウィジットのアイテムを更新させる
  (`|ExecutionSequence`
    (:`then_0`
      ;;[0.4299 1 0.9622] ProgressBarの表示に表示する数値の更新
      (`BlueprintMapLibrary.Map_Add` (`self.MaxProgress`) TextString MaxProgress)
      (if (<= _value_3 Progress)
        (`BlueprintMapLibrary.Map_Add` _progress TextString _value_3)
        (else
          (`BlueprintMapLibrary.Map_Add` _progress TextString Progress))))
    (:`then_1`
      ;;[0.4299 1 0.9622] ProgressBarの更新
      (`/Game/MyContents/Widget/ObjectWidget/BPW_ProductionQuantity.SetBPW_ElementTextItem` (`self.As BPW Element`) TextString (or (>= _value _value_2) SetColorProgress) _value _value_2))))

(fn `Init`
  (params (BPE_WorldObject :type "/Game/MyContents/BluePrints/SaveGames/SaveGames/BPE_WorldObjects Enum" :default "NewEnumerator1") (OverYukeMaterial :type "Array of StaticMeshComponent Object Reference"))
  (set `self.BPE_WorldObject` BPE_WorldObject)
  (set `self.OverYukeMaterial` OverYukeMaterial))

(fn `UserConstructionScript`)