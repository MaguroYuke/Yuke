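; BP_Spawn is a spawn area object that tracks whether anything overlaps its Box component.
; On BeginPlay it sets its world object type enum and turns off physics simulation on SpawnEria.
; Box begin and end overlap events raise and lower HitCount, keeping the HitObj flag true while the count is above zero.
; The file itself contains no spawning logic.
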(event `self.ReceiveBeginPlay`
  (set `self.BPE_WorldObject` "NewEnumerator6")
  (`PrimitiveComponent.SetSimulatePhysics` (`self.SpawnEria`) false))

(event `self.Box.OnComponentBeginOverlap`
  (params (OverlappedComponent :type "PrimitiveComponent Object Reference") (OtherActor :type "Actor Object Reference") (OtherComp :type "PrimitiveComponent Object Reference") (OtherBodyIndex :type Integer) (bFromSweep :type Boolean) (SweepResult :type "HitResult Structure (by ref)"))
  (`/Engine/EditorBlueprintResources/StandardMacros.IncrementInt` (`self.HitCount`)
    (:`  `
      (if (not (`self.HitObj`))
        (set `self.HitObj` true)))))

(event `self.Box.OnComponentEndOverlap`
  (params (OverlappedComponent :type "PrimitiveComponent Object Reference") (OtherActor :type "Actor Object Reference") (OtherComp :type "PrimitiveComponent Object Reference") (OtherBodyIndex :type Integer))
  (bind _result (`/Engine/EditorBlueprintResources/StandardMacros.DecrementInt` (`self.HitCount`))
    (:`  `
      (if (not (> _result 0))
        (set `self.HitObj` false)))))

(fn `UserConstructionScript`)