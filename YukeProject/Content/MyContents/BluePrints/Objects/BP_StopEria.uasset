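; BP_StopEria is a stop-area actor that tracks BP_Goods objects inside its StopCollision volume.
; Begin and end overlap events add and remove goods from the ALLActors array.
; Every Tick, ALLNextEria calls NextEria on each tracked good, passing itself as the argument.
; BeginPlay clears the array, calls InitActorWidget and disables physics simulation on the StopEria component.
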(event `self.ReceiveBeginPlay`
  (`KismetArrayLibrary.Array_Clear` (`self.ALL_Actors`))
  (`self.InitActorWidget` (struct))
  (`PrimitiveComponent.SetSimulatePhysics` (`self.StopEria`) false))

(event `self.ReceiveTick`
  (params (DeltaSeconds :type "Float (single-precision)"))
  (`self.ALL_NextEria`))

(event `self.StopCollision.OnComponentBeginOverlap`
  (params (OverlappedComponent :type "PrimitiveComponent Object Reference") (OtherActor :type "Actor Object Reference") (OtherComp :type "PrimitiveComponent Object Reference") (OtherBodyIndex :type Integer) (bFromSweep :type Boolean) (SweepResult :type "HitResult Structure (by ref)"))
  (bind _asbp_goods (cast `/Game/MyContents/BluePrints/Objects/BP_Goods` OtherActor))
  (`KismetArrayLibrary.Array_Add` (`self.ALL_Actors`) _asbp_goods))

(event `self.StopCollision.OnComponentEndOverlap`
  (params (OverlappedComponent :type "PrimitiveComponent Object Reference") (OtherActor :type "Actor Object Reference") (OtherComp :type "PrimitiveComponent Object Reference") (OtherBodyIndex :type Integer))
  (bind _asbp_goods (cast `/Game/MyContents/BluePrints/Objects/BP_Goods` OtherActor))
  (`KismetArrayLibrary.Array_RemoveItem` (`self.ALL_Actors`) _asbp_goods))

(fn `ALL_NextEria`
  (for _array_element (`self.ALL_Actors`)
    (`/Game/MyContents/BluePrints/Objects/BP_Goods.NextEria` _array_element self)))

(fn `UserConstructionScript`)