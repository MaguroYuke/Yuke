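; BP_Sample is an actor that moves to the first target in its ALLTarget array and displays its state on a floating widget.
; Tick runs an enum state machine: wait, start, move, arrive, and end with self-destruction and a cleared-count increment.
; Before starting, it scans all BP_Sample actors and waits if that target is occupied or contested.
; Movement precomputes one distance-normalized lerp step, repeats it, then snaps to the target.
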(event `self.ReceiveBeginPlay`
  ;[1 1 1] Actorの初期設定
  (`self.InitWidget`)
  (set `self.DeltaTime` 0.01)
  (set `self.BPE_Artifact` "NewEnumerator5") ; 最初の行動
  (`self.InitPosition`))

(event `self.ReceiveActorBeginOverlap`
  (params (OtherActor :type "Actor Object Reference")))

(event `self.ReceiveTick`
  (params (DeltaSeconds :type "Float (single-precision)"))
  ;[1 1 1] 自身の行動の制御
  (switch `/Game/MyContents/BluePrints/Objects/BPE_Artifact` (`self.BPE_Artifact`)
    (:`NewEnumerator5`
      (`self.SetText` "待機中")
      (`self.Prosesing` "NewEnumerator0") ; 移動先に移動中のアクターや移動先に物があるとき移動しない
    )
    (:`NewEnumerator0`
      (`self.SetText` "開始")
      (`KismetSystemLibrary.Delay` (`self.DelayTime`))
      (`self.NextActorLocation`) ; 移動先の座標を入力し開始
    )
    (:`NewEnumerator1`
      (`self.SetText` "移動中")
      (`self.SetMyActorLocation`) ; 指定した場所まで移動
    )
    (:`NewEnumerator2`
      (`self.SetText` "到着")
      (`KismetSystemLibrary.Delay` (`self.DelayTime`))
      (set `self.BPE_Artifact` "NewEnumerator5"))
    (:`NewEnumerator3`
      (`self.SetText` "終了")
      (`KismetSystemLibrary.Delay` (`self.DelayTime`))
      (`self.MyDestroyActor`) ; 自分のアクターを削除し配列から取り除く
      (`/Engine/EditorBlueprintResources/StandardMacros.IncrementInt` (`/Game/MyContents/BluePrints/Objects/BPW_ActorCount.ClearObj` (`self.BPW_ActorCount`))))))

(event `カスタムイベント`)

(fn `InitWidget`
  (bind _asbpw_actor_widget (cast `/Game/MyContents/BluePrints/Objects/BPW_ActorWidget` (`WidgetComponent.GetUserWidgetObject` (`self.Widget`))))
  (bind _output_get (set `self.BPW_ActorWidget` _asbpw_actor_widget))
  (set `/Game/MyContents/BluePrints/Objects/BPW_ActorWidget.ActorText` "" _output_get)
  (set `/Game/MyContents/BluePrints/Objects/BPW_ActorWidget.E_Visibility` "Hidden" _output_get))

(fn `MyDestroyActor`
  (`self.K2_DestroyActor`))

(fn `NextActorLocation`
  (bind _output (`|GetArrayItem` (`self.ALLTarget`)))
  (bind _returnvalue (`self.K2_GetActorLocation` _output))
  (if (`KismetSystemLibrary.IsValid` _output)
    (bind _uplocation (`self.SetLerp` _returnvalue)) ; 移動する場所と自分の場所を分割する
    (set `self.UpLocation` _uplocation)
    (set `self.TargetLocation` _returnvalue)
    (set `self.BPE_Artifact` "NewEnumerator1")
    (else
      (set `self.BPE_Artifact` "NewEnumerator3")
      (`KismetSystemLibrary.PrintString` "予期せぬエラーで終了します。"))))

(fn `Prosesing`
  (params (Artifact :type "/Game/MyContents/BluePrints/Objects/BPE_Artifact Enum" :default "NewEnumerator5"))
  (bind _nostart (`self.NoStart`))
  (if (> (`KismetArrayLibrary.Array_Length` (`self.ALLTarget`)) 0)
    (bind _outactors (`GameplayStatics.GetAllActorsOfClass` "BP_Sample_C"))
    (for _array_element _outactors
      (bind _bpe_artifact (`/Game/MyContents/BluePrints/Objects/BP_Sample.BPE_Artifact` _array_element))
      (if (and (or (`|EnumEquality` _bpe_artifact "NewEnumerator0") (`|EnumEquality` _bpe_artifact "NewEnumerator1") (`|EnumEquality` _bpe_artifact "NewEnumerator2") (> (`KismetArrayLibrary.Array_Length` (`/Game/MyContents/BluePrints/Objects/BP_StopEria.AllActor` (`|GetArrayItem` (`self.ALLTarget`)))) 0)) (== (`|GetArrayItem` (`/Game/MyContents/BluePrints/Objects/BP_Sample.ALLTarget` _array_element)) (`|GetArrayItem` (`self.ALLTarget`))))
        (`KismetArrayLibrary.Array_Add` (`self.NoStart`) true)))
    (if (>= (`KismetArrayLibrary.Array_Length` _nostart) 1)
      (for _array_element_2 _nostart
        (if _array_element_2
          (break)
          (else
            (set `self.Start` true))))
      (else
        (set `self.Start` true)
        (set `self.End` true)))
    (`KismetArrayLibrary.Array_Clear` _nostart)
    (if (`self.Start`)
      (switch `/Game/MyContents/BluePrints/Objects/BPE_Artifact` Artifact
        (:`NewEnumerator0`
          (if (`self.End`)
            (set `self.BPE_Artifact` "NewEnumerator0")
            (set `self.Start` false)
            (set `self.End` false)))
        (:`NewEnumerator1`
          (set `self.BPE_Artifact` "NewEnumerator1"))
        (:`NewEnumerator2`
          (set `self.BPE_Artifact` "NewEnumerator2")))
      (else
        (set `self.BPE_Artifact` "NewEnumerator5")))
    (else
      (set `self.BPE_Artifact` "NewEnumerator3"))))

(fn `SetLerp`
  (params (NextActorLocation :type "Vector Structure"))
  (returns (UpLocation :type "Vector Structure"))
  (bind _output_get (set `self.LerpAlpha` (`KismetMathLibrary.FClamp` (* (`self.DeltaTime`) (* (`KismetMathLibrary.FClamp` (`self.Speed`) 0.01 100.0) (/ 100.0 (`KismetMathLibrary.Vector_Distance` (`self.K2_GetActorLocation`) NextActorLocation)))))))
  (return (- (`KismetMathLibrary.VLerp` (`self.K2_GetActorLocation`) NextActorLocation _output_get) (`self.K2_GetActorLocation`))))

(fn `SetMyActorLocation`
  (if (<= (`self.LocationPartition`) 1.0)
    (set `self.LocationPartition` (+ (`self.LocationPartition`) (`self.LerpAlpha`)))
    (`self.K2_SetActorLocation` (+ (`self.K2_GetActorLocation`) (`self.UpLocation`)))
    (else
      (set `self.LocationPartition` 0.0)
      (`self.K2_SetActorLocation` (`self.TargetLocation`))
      (set `self.BPE_Artifact` "NewEnumerator2"))))

(fn `SetText`
  (params (SetText :type String))
  (bind _bpw_actorwidget (`self.BPW_ActorWidget`))
  (set `/Game/MyContents/BluePrints/Objects/BPW_ActorWidget.ActorText` SetText _bpw_actorwidget)
  (set `/Game/MyContents/BluePrints/Objects/BPW_ActorWidget.E_Visibility` "Visible" _bpw_actorwidget))

(fn `UserConstructionScript`)