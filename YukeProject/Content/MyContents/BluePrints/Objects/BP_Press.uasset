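; BP_Press is a press machine that moves its mesh to a target point and back when work items are in position.
; Tick runs a Stop, Start, UpData, End state machine, using StartMove and MoveActor to drive the stroke.
; Box1 overlaps force a return and count hits, calling ALLNextEria from the second onward.
; Leaving StopCollision resets the count, and a widget shows Japanese work-status text.
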(event `self.ReceiveBeginPlay`
  (`self.InitActorWidget` (make `SlateColor` (struct :`G` 0.170037 :`B` 1.0 :`A` 1.0)))
  (`self.InitLocation`)
  (set `self.Speed` 1.0)
  (set `self.StartLocation` (`SceneComponent.K2_GetComponentLocation` (`self.StaticMesh1`)))
  (set `self.BPE_Artifact` "NewEnumerator0"))

(event `self.StopCollision.OnComponentBeginOverlap`
  (params (OverlappedComponent :type "PrimitiveComponent Object Reference") (OtherActor :type "Actor Object Reference") (OtherComp :type "PrimitiveComponent Object Reference") (OtherBodyIndex :type Integer) (bFromSweep :type Boolean) (SweepResult :type "HitResult Structure (by ref)")))

(event `self.ReceiveTick`
  (params (DeltaSeconds :type "Float (single-precision)"))
  (if (`self.ActorStart`)
    (switch `/Game/MyContents/BluePrints/Objects/BPE_Artifact` (`self.BPE_Artifact`)
      (:`NewEnumerator0`
        (for _array_element (`self.ALL_Actors`)
          (bind _target (`/Game/MyContents/BluePrints/Objects/BP_Goods.TargetPos` _array_element))
          (if _target
            (if (not (>= (`self.Count`) 5))
              (`self.SetText` "作業開始")
              (`KismetSystemLibrary.Delay` (`self.Delay`))
              (set `self.BPE_Artifact` "NewEnumerator1")))))
      (:`NewEnumerator1`
        (`self.StartMove` (`SceneComponent.K2_GetComponentLocation` (`self.StaticMesh1`)) (`SceneComponent.K2_GetComponentLocation` (`self.NextEria`)))
        (set `self.BPE_Artifact` "NewEnumerator2")
        (`self.SetText` "作業中"))
      (:`NewEnumerator2`
        (bind (_location _onmove) (`self.MoveActor` (`SceneComponent.K2_GetComponentLocation` (`self.StaticMesh1`))))
        (`SceneComponent.K2_SetWorldLocation` (`self.StaticMesh1`) _location false false)
        (if _onmove
          _
          (elif (`self.Return`)
            (set `self.BPE_Artifact` "NewEnumerator0")
            (set `self.Return` false)
            (else
              (set `self.BPE_Artifact` "NewEnumerator3")
              (set `self.Return` true)))))
      (:`NewEnumerator3`
        (`self.StartMove` (`SceneComponent.K2_GetComponentLocation` (`self.StaticMesh1`)) (`self.StartLocation`))
        (set `self.BPE_Artifact` "NewEnumerator2")))))

(event `self.StopCollision.OnComponentEndOverlap`
  (params (OverlappedComponent :type "PrimitiveComponent Object Reference") (OtherActor :type "Actor Object Reference") (OtherComp :type "PrimitiveComponent Object Reference") (OtherBodyIndex :type Integer))
  (set `self.Count` 0)
  (`self.SetText` "待機中")
  (`KismetSystemLibrary.Delay` (`self.Delay`))
  (`self.NoText`))

(event `self.Box1.OnComponentBeginOverlap`
  (params (OverlappedComponent :type "PrimitiveComponent Object Reference") (OtherActor :type "Actor Object Reference") (OtherComp :type "PrimitiveComponent Object Reference") (OtherBodyIndex :type Integer) (bFromSweep :type Boolean) (SweepResult :type "HitResult Structure (by ref)"))
  (set `self.BPE_Artifact` "NewEnumerator3")
  (set `self.Return` true)
  (bind _result (`/Engine/EditorBlueprintResources/StandardMacros.IncrementInt` (`self.Count`))
    (:`  `
      (if (>= _result 2)
        (`self.ALL_NextEria`)
        (`self.SetText` "作業終了")))))

(event `self.Box1.OnComponentEndOverlap`
  (params (OverlappedComponent :type "PrimitiveComponent Object Reference") (OtherActor :type "Actor Object Reference") (OtherComp :type "PrimitiveComponent Object Reference") (OtherBodyIndex :type Integer)))

(fn `UserConstructionScript`)