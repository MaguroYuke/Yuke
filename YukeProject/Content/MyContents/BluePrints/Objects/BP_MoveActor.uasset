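; BP_MoveActor is an actor that supplies point-to-point movement and a text widget label.
; StartMove turns clamped Speed, distance and DeltaTime (set to 0.01 by InitLocation) into a constant per-step offset.
; Each MoveActor call returns the next location, then the exact target with OnMove false once accumulated alpha exceeds one; it never moves the actor itself.
; Helper functions initialize BPW_ActorWidget's color and show or hide its text.
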(event `self.ReceiveBeginPlay`)

(event `EndActor`
  (set `self.ActorStart` false))

(fn `InitActorWidget`
  (params (TextColor :type "SlateColor Structure"))
  (bind _asbpw_actor_widget (cast `/Game/MyContents/BluePrints/Objects/BPW_ActorWidget` (`WidgetComponent.GetUserWidgetObject` (`self.Widget`))))
  (bind _output_get (set `self.BPW_ActorWidget` _asbpw_actor_widget))
  (`/Game/MyContents/BluePrints/Objects/BPW_ActorWidget.InitActorWidget` _output_get TextColor))

(fn `InitLocation`
  (`|ExecutionSequence`
    (:`then_0`
      (set `self.UpLocation` (0.0 0.0 0.0)))
    (:`then_1`
      (set `self.TargetLocation` (0.0 0.0 0.0)))
    (:`then_2`
      (set `self.LerpAlpha` 0.0))
    (:`then_3`
      (set `self.LocationPartition` 0.0))
    (:`then_4`
      (set `self.DeltaTime` 0.01))
    (:`then_5`
      (set `self.ActorStart` true))))

(fn `MoveActor`
  (params (MyLocation :type "Vector Structure"))
  (returns (Location :type "Vector Structure") (OnMove :type Boolean))
  (if (<= (`self.LocationPartition`) 1.0)
    (set `self.LocationPartition` (+ (`self.LocationPartition`) (`self.LerpAlpha`)))
    (return (+ MyLocation (`self.UpLocation`)) true)
    (else
      (set `self.LocationPartition` 0.0)
      (return (`self.TargetLocation`) false))))

(fn `NoText`
  (bind _bpw_actorwidget (`self.BPW_ActorWidget`))
  (set `/Game/MyContents/BluePrints/Objects/BPW_ActorWidget.ActorText` "" _bpw_actorwidget)
  (set `/Game/MyContents/BluePrints/Objects/BPW_ActorWidget.E_Visibility` "Hidden" _bpw_actorwidget))

(fn `SetText`
  (params (Text :type String))
  (bind _bpw_actorwidget (`self.BPW_ActorWidget`))
  (set `/Game/MyContents/BluePrints/Objects/BPW_ActorWidget.ActorText` Text _bpw_actorwidget)
  (set `/Game/MyContents/BluePrints/Objects/BPW_ActorWidget.E_Visibility` "Visible" _bpw_actorwidget))

(fn `StartMove`
  (params (MyLocation :type "Vector Structure") (TargetLocation :type "Vector Structure"))
  (set `self.TargetLocation` TargetLocation)
  (bind _output_get (set `self.LerpAlpha` (`KismetMathLibrary.FClamp` (* (`self.DeltaTime`) (* (`KismetMathLibrary.FClamp` (`self.Speed`) 0.01 100.0) (/ 100.0 (`KismetMathLibrary.Vector_Distance` MyLocation TargetLocation)))))))
  (set `self.UpLocation` (- (`KismetMathLibrary.VLerp` MyLocation TargetLocation _output_get) MyLocation))
  (set `self.LocationPartition` 0.0))

(fn `UserConstructionScript`)