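; BuleTest is a test Blueprint that moves its Blue component as if it were carried by a conveyor.
; While OnConveyor is true, Tick offsets Blue along negative Y with sweep, by a fixed per-frame step that ignores DeltaSeconds.
; Nothing in these graphs sets OnConveyor, and the disconnected impulse, physics, actor-offset and direction-times-speed nodes never run.
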(event `self.ReceiveTick`
  (params (DeltaSeconds :type "Float (single-precision)"))
  (`|ExecutionSequence`
    (:`then_0`
      (if (`self.bOnConveyor`)
        (`SceneComponent.K2_AddWorldOffset` (`self.blue`) (0.0 -10.0 0.0) true false)))))

(fn `UserConstructionScript`)