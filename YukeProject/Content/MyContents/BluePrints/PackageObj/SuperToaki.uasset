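; SuperToaki is a factory-simulation machine actor that animates processing of BP_ParamGoods via a Level Sequence and reports production count and cycle times.
; Station overlap boxes advance an enum state machine, retargeting each item's movement along the line.
; Overlaps also record cycle times and update the count and average for progress displays refreshed on Tick.
; Tick also starts the delayed animation and, in the simulation tutorial map, debug-spawns goods while idle.
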(event `self.ReceiveBeginPlay`
  (bind _timearray (`self.TimeArray`))
  (bind _average (`self.Average`))
  (bind _maximum_fractional_digits (`self.Maximum Fractional Digits`))
  (bind _returnvalue (`KismetMathLibrary.Conv_IntToDouble` (`self.count`)))
  (`|ExecutionSequence`
    (:`then_0`
      ;[1 1 1] 初期設定
      (`parent.ReceiveBeginPlay`)
      (bind (_outactor _returnvalue_2) (`LevelSequencePlayer.CreateLevelSequencePlayer` "/Game/MyContents/LevelSequences/4Move.4Move"))
      (`LevelSequenceActor.SetBinding` _outactor (`|GetSequenceBinding` null) (`|MakeArray` self :!type "Actor Object Reference") false)
      (set `self.LevelSequence` _returnvalue_2)
      (`MovieSceneSequencePlayer.SetPlayRate` (`self.LevelSequence`) (`self.Speed`))
      (`self.Init` "NewEnumerator3" (`|MakeArray` (`self.4dodai`) (`self.4kanban`) (`self.4idou`) (`self.4stanp`) (`self.4kaiten`) (`self.4oshidashi`) (`self.4table`) (`self.4kaitenneji`))) ; 親の変数の初期化
      (`PrimitiveComponent.SetSimulatePhysics` (`self.4dodai`) false)
      (bind _asbpi_my_content (cast `/Game/MyContents/BluePrints/Objects/BPI_MyContent` (`GameplayStatics.GetGameInstance`)))
      (set `self.As BPI My Content` _asbpi_my_content))
    (:`then_1`
      (`self.InitProgress` _average (* _average 2.0) (`self.AverageTimeString`) _maximum_fractional_digits)
      (`self.InitProgress` (`|GetArrayItem` _timearray (`KismetArrayLibrary.Array_LastIndex` _timearray)) (* (`self.Average`) 2.0) (`self.OneTimeGoods`) _maximum_fractional_digits)
      (`self.InitProgress` _returnvalue _returnvalue (`self.CountString`) 0 "Hidden"))
    (:`then_2`
      (bind _returnvalue_3 (`GameplayStatics.GetCurrentLevelName` true))
      (if (not (or (!= _returnvalue_3 "Map_Edit") (!= _returnvalue_3 "Map_EditTurorial")))
        (`PrimitiveComponent.SetSimulatePhysics` (`self.4dodai`) false)))))

(event `self.ReceiveTick`
  (params (DeltaSeconds :type "Float (single-precision)"))
  (bind _average (`self.Average`))
  (bind _timearray (`self.TimeArray`))
  (bind _returnvalue (`KismetMathLibrary.Conv_IntToDouble` (`self.count`)))
  (bind _output (`|GetArrayItem` _timearray (`KismetArrayLibrary.Array_LastIndex` _timearray)))
  (`parent.ReceiveTick` DeltaSeconds)
  (`|ExecutionSequence`
    (:`then_0`
      ;[1 1 1] オブジェクトがヒットしたときにアニメーションの再生
      (add `MovieSceneSequencePlayer.OnFinished` (`self.LevelSequence`) (delegate `TeisiOFF`)))
    (:`then_1`
      (if (`self.H`)
        (if (not (`self.teisi`))
          (bind _returnvalue_2 (`GameplayStatics.GetCurrentLevelName` true))
          (if (!= _returnvalue_2 "Map_Edit")
            (`KismetSystemLibrary.Delay` 3.0)
            (`MovieSceneSequencePlayer.Play` (`self.LevelSequence`))
            (set `self.teisi` true)))))
    (:`then_2`
      (bind _returnvalue_3 (`GameplayStatics.GetCurrentLevelName` true))
      (if (`KismetStringLibrary.EqualEqual_StrStr` _returnvalue_3 "Map_SimulationTutorial")
        (if (== (`/Game/MyContents/Widget/Tutorial/BPW_Tutorial.CurrentMessageIndex` (`/Game/MyContents/BluePrints/Objects/BPI_MyContent.BPW_TutorialWidget` (`self.As BPI My Content`))) 46)
          ;[1 1 1] あとで消すヤツ（ランダムにアクターをスポーンさせるデバック用）
          (if (`self.H`)
            _
            (elif (not (`self.teisi`))
              (bind _returnvalue_4 (`|SpawnActorFromClass` "/Game/MyContents/BluePrints/Objects/YukeBlue.YukeBlue_C" (`KismetMathLibrary.MakeTransform` (`SceneComponent.K2_GetComponentLocation` (`self.tablebox`))) "Undefined" "MultiplyWithRoot" null null))
              (`/Game/MyContents/BluePrints/Buttons/BP_ParamGoods.DodaiDestroy` _returnvalue_4)))
          (elif (`self.H`)
            _
            (elif (not (`self.teisi`))
              (bind _returnvalue_5 (`|SpawnActorFromClass` (`KismetArrayLibrary.Array_Random` (`|MakeArray` "/Game/MyContents/BluePrints/Objects/YukeRed.YukeRed_C" "/Game/MyContents/BluePrints/Objects/YukeWhite.YukeWhite_C" "/Game/MyContents/BluePrints/Objects/YukeBlue.YukeBlue_C" :!type "Actor Class Reference")) (`KismetMathLibrary.MakeTransform` (`SceneComponent.K2_GetComponentLocation` (`self.tablebox`))) "Undefined" "MultiplyWithRoot" null null))
              (bind _asbp_param_goods (cast `/Game/MyContents/BluePrints/Buttons/BP_ParamGoods` _returnvalue_5))
              (`/Game/MyContents/BluePrints/Buttons/BP_ParamGoods.DodaiDestroy` _asbp_param_goods))))))
    (:`then_3`
      ;[1 1 1] カウントが5以上になったときに平均タイムを求める
      (if (>= (`self.count`) 1)
        _))
    (:`then_5`
      (`self.UpDataProgress` (`self.AverageTimeString`) (* _average 2.0) _average true)
      (`self.UpDataProgress` (`self.OneTimeGoods`) (* (`self.Average`) 2.0) _output (>= (`self.Average`) _output))
      (`self.UpDataProgress` (`self.CountString`) _returnvalue _returnvalue))))

(event `TeisiOFF`
  ;[1 1 1] オブジェクトがヒットしたときにアニメーションの再生
  (set `self.teisi` false))

(event `self.CountBox.OnComponentBeginOverlap`
  (params (OverlappedComponent :type "PrimitiveComponent Object Reference") (OtherActor :type "Actor Object Reference") (OtherComp :type "PrimitiveComponent Object Reference") (OtherBodyIndex :type Integer) (bFromSweep :type Boolean) (SweepResult :type "HitResult Structure (by ref)"))
  ;[1 1 1] コリジョンに当たったらCount++;
  (`/Engine/EditorBlueprintResources/StandardMacros.DoOnce` false :!label _label
    (:`Completed`
      (cast `/Game/MyContents/BluePrints/Buttons/BP_ParamGoods` OtherActor)
      (`/Engine/EditorBlueprintResources/StandardMacros.IncrementInt` (`self.count`)
        (:`  `
          (`/Engine/EditorBlueprintResources/StandardMacros.IncrementInt` (`self.seisan`)
            (:`  `
              ;[1 1 1] 平均タイムの計算　（5個作られたときの平均タイム）
              (set `self.Average` 0.0)
              (for _array_element (`self.TimeArray`)
                (set `self.Average` (+ _array_element (`self.Average`))))
              (set `self.Average` (/ (`self.Average`) (`KismetArrayLibrary.Array_Length` (`self.TimeArray`)))))))))))

(event `self.tablebox.OnComponentBeginOverlap`
  (params (OverlappedComponent :type "PrimitiveComponent Object Reference") (OtherActor :type "Actor Object Reference") (OtherComp :type "PrimitiveComponent Object Reference") (OtherBodyIndex :type Integer) (bFromSweep :type Boolean) (SweepResult :type "HitResult Structure (by ref)"))
  ;[1 1 1] 加工品を手順通りに移動できるための制御（加工品の移動先変更や速度の変更
  ;[1 1 1] コリジョンに当たったらCount++;
  (`|ExecutionSequence`
    (:`then_0`
      (goto _label :!via `Reset`))
    (:`then_1`
      ;;[0.4206 0.9502 1] NowTime=現在の時刻をセット
      (set `self.nowTime` (`KismetSystemLibrary.GetGameTimeInSeconds`))
      (if (`|EnumEquality` (`self.BPE_SuperToaki`) "NewEnumerator4")
        (bind _asbp_param_goods (cast `/Game/MyContents/BluePrints/Buttons/BP_ParamGoods` OtherActor)
          (:`then`
            (set `/Game/MyContents/BluePrints/Buttons/BP_ParamGoods.Target` (`self.tablebox`) _asbp_param_goods)
            (`PrimitiveComponent.SetSimulatePhysics` (`/Game/MyContents/BluePrints/Buttons/BP_ParamGoods.Goods` _asbp_param_goods) false)
            (set `self.BPE_SuperToaki` "NewEnumerator0")
            (set `self.H` true)
            (set `/Game/MyContents/BluePrints/Buttons/BP_ParamGoods.Catch` true _asbp_param_goods)
            (set `/Game/MyContents/BluePrints/Buttons/BP_ParamGoods.NextTarget` null _asbp_param_goods)
            (`KismetSystemLibrary.Delay` 3.0)
            (set `/Game/MyContents/BluePrints/Buttons/BP_ParamGoods.Catch` false _asbp_param_goods))
          (:`CastFailed`
            (bind _assuper_clane (cast `/Game/MyContents/BluePrints/PackageObj/SuperClane` OtherActor))
            (`/Game/MyContents/BluePrints/PackageObj/SuperClane.NextEria` _assuper_clane)))))))

(event `self.bakyu--------------mu.OnComponentBeginOverlap`
  (params (OverlappedComponent :type "PrimitiveComponent Object Reference") (OtherActor :type "Actor Object Reference") (OtherComp :type "PrimitiveComponent Object Reference") (OtherBodyIndex :type Integer) (bFromSweep :type Boolean) (SweepResult :type "HitResult Structure (by ref)"))
  ;[1 1 1] 加工品を手順通りに移動できるための制御（加工品の移動先変更や速度の変更
  (if (`|EnumEquality` (`self.BPE_SuperToaki`) "NewEnumerator0")
    (bind _asbp_param_goods (cast `/Game/MyContents/BluePrints/Buttons/BP_ParamGoods` OtherActor))
    (set `/Game/MyContents/BluePrints/Buttons/BP_ParamGoods.Target` (`self.bakyu--------------mu`) _asbp_param_goods)
    (set `self.BPE_SuperToaki` "NewEnumerator1")
    (set `self.H` false)))

(event `self.kaitenbox.OnComponentBeginOverlap`
  (params (OverlappedComponent :type "PrimitiveComponent Object Reference") (OtherActor :type "Actor Object Reference") (OtherComp :type "PrimitiveComponent Object Reference") (OtherBodyIndex :type Integer) (bFromSweep :type Boolean) (SweepResult :type "HitResult Structure (by ref)"))
  ;[1 1 1] 加工品を手順通りに移動できるための制御（加工品の移動先変更や速度の変更
  (if (`|EnumEquality` (`self.BPE_SuperToaki`) "NewEnumerator1")
    (bind _asbp_param_goods (cast `/Game/MyContents/BluePrints/Buttons/BP_ParamGoods` OtherActor))
    (set `/Game/MyContents/BluePrints/Buttons/BP_ParamGoods.Target` (`self.kaitenbox`) _asbp_param_goods)
    (set `self.BPE_SuperToaki` "NewEnumerator2")))

(event `self.Box3.OnComponentBeginOverlap`
  (params (OverlappedComponent :type "PrimitiveComponent Object Reference") (OtherActor :type "Actor Object Reference") (OtherComp :type "PrimitiveComponent Object Reference") (OtherBodyIndex :type Integer) (bFromSweep :type Boolean) (SweepResult :type "HitResult Structure (by ref)"))
  ;[1 1 1] 加工品を手順通りに移動できるための制御（加工品の移動先変更や速度の変更
  (if (`|EnumEquality` (`self.BPE_SuperToaki`) "NewEnumerator2")
    (bind _asbp_param_goods (cast `/Game/MyContents/BluePrints/Buttons/BP_ParamGoods` OtherActor))
    (set `/Game/MyContents/BluePrints/Buttons/BP_ParamGoods.Target` null _asbp_param_goods)
    (set `/Game/MyContents/BluePrints/Buttons/BP_ParamGoods.NextTarget` (`self.Box`) _asbp_param_goods)
    (set `/Game/MyContents/BluePrints/Buttons/BP_ParamGoods.ReversTarget` (`self.Box2`) _asbp_param_goods)
    (set `self.BPE_SuperToaki` "NewEnumerator4")
    (set `/Game/MyContents/BluePrints/Buttons/BP_ParamGoods.ObjSpeed` 20.0 _asbp_param_goods)
    (set `/Game/MyContents/BluePrints/Buttons/BP_ParamGoods.Catch` false _asbp_param_goods)
    (`KismetArrayLibrary.Array_Add` (`self.TimeArray`) (- (`KismetSystemLibrary.GetGameTimeInSeconds`) (`self.nowTime`)))))

(event `self.Box.OnComponentBeginOverlap`
  (params (OverlappedComponent :type "PrimitiveComponent Object Reference") (OtherActor :type "Actor Object Reference") (OtherComp :type "PrimitiveComponent Object Reference") (OtherBodyIndex :type Integer) (bFromSweep :type Boolean) (SweepResult :type "HitResult Structure (by ref)"))
  ;[1 1 1] 加工品を手順通りに移動できるための制御（加工品の移動先変更や速度の変更
  (bind _asbp_param_goods (cast `/Game/MyContents/BluePrints/Buttons/BP_ParamGoods` OtherActor))
  (bind _goods (`/Game/MyContents/BluePrints/Buttons/BP_ParamGoods.Goods` _asbp_param_goods))
  (`PrimitiveComponent.SetSimulatePhysics` _goods false)
  (`SceneComponent.K2_SetWorldRotation` :`self` _goods)
  (set `/Game/MyContents/BluePrints/Buttons/BP_ParamGoods.ObjSpeed` 20.0 _asbp_param_goods))

(fn `UserConstructionScript`)