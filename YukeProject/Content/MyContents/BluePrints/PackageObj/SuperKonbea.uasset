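; Sorting conveyor machine that separates blue, red and white goods and tallies production and error counts.
; Colour triggers enable physics on matching goods and play Level Sequence pushers bound to this actor.
; Get triggers queue goods for the SuperClane crane, while goods reaching Box4 count as errors, get launched and are later destroyed.
; Tick refreshes inherited progress displays, taking targets from the BPW_SpeedSetting widget when present.
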(event `self.ReceiveTick`
  (params (DeltaSeconds :type "Float (single-precision)"))
  (bind _as_bp_param_goods (`self.As BP Param Goods`))
  (bind _returnvalue (`KismetMathLibrary.Conv_IntToDouble` (`self.ErrorCount`)))
  (bind _output (`|GetArrayItem` _as_bp_param_goods))
  (`parent.ReceiveTick` DeltaSeconds)
  (`|ExecutionSequence`
    (:`then_0`
      (bind _foundwidgets (`WidgetBlueprintLibrary.GetAllWidgetsOfClass` "/Game/MyContents/Widget/SpeedSetting/BPW_SpeedSetting.BPW_SpeedSetting_C"))
      (if (`KismetSystemLibrary.IsValid` (`|GetArrayItem` _foundwidgets))
        (for _array_element _foundwidgets
          (`|ExecutionSequence`
            (:`then_0`
              (set `self.MaxBlueSeisan` (`/Game/MyContents/Widget/SpeedSetting/BPW_SpeedSettingItem.Data` (`/Game/MyContents/Widget/SpeedSetting/BPW_SpeedSetting.BlueMokuhyousuu` _array_element))))
            (:`then_1`
              (set `self.MaxRedSeisan` (`/Game/MyContents/Widget/SpeedSetting/BPW_SpeedSettingItem.Data` (`/Game/MyContents/Widget/SpeedSetting/BPW_SpeedSetting.RedMokuhyousuu` _array_element))))
            (:`then_2`
              (set `self.MaxWhiteSeisan` (`/Game/MyContents/Widget/SpeedSetting/BPW_SpeedSettingItem.Data` (`/Game/MyContents/Widget/SpeedSetting/BPW_SpeedSetting.WhiteMokuhyousuu` _array_element))))))
        (else
          (`|ExecutionSequence`
            (:`then_0`
              (set `self.MaxBlueSeisan` (`KismetMathLibrary.Conv_IntToDouble` (`self.BlueSeisan`))))
            (:`then_1`
              (set `self.MaxRedSeisan` (`KismetMathLibrary.Conv_IntToDouble` (`self.RedSeisan`))))
            (:`then_2`
              (set `self.MaxWhiteSeisan` (`KismetMathLibrary.Conv_IntToDouble` (`self.WhiteSeisan`))))))))
    (:`then_1`
      ;[1 1 1] ウィジットの初期化
      (`self.UpDataProgress` (`self.BlueCount`) (`self.MaxBlueSeisan`) (`KismetMathLibrary.Conv_IntToDouble` (`self.BlueSeisan`)) true)
      (`self.UpDataProgress` (`self.RedCount`) (`self.MaxRedSeisan`) (`KismetMathLibrary.Conv_IntToDouble` (`self.RedSeisan`)) true)
      (`self.UpDataProgress` (`self.WhiteCount`) (`self.MaxWhiteSeisan`) (`KismetMathLibrary.Conv_IntToDouble` (`self.WhiteSeisan`)) true)
      (`self.UpDataProgress` (`self.Error`) _returnvalue _returnvalue true)
      (if (> (`KismetArrayLibrary.Array_Length` (`self.As BP Param Goods`)) 0)
        (`KismetSystemLibrary.Delay` 1.0)
        (`self.K2_DestroyActor` _output)
        (`KismetArrayLibrary.Array_RemoveItem` _as_bp_param_goods _output)))))

(event `self.ReceiveBeginPlay`
  (bind _returnvalue (`KismetMathLibrary.Conv_IntToDouble` (`self.ErrorCount`)))
  (bind _returnvalue_2 (`KismetMathLibrary.Conv_IntToDouble` (`self.WhiteSeisan`)))
  (bind _returnvalue_3 (`KismetMathLibrary.Conv_IntToDouble` (`self.RedSeisan`)))
  (bind _returnvalue_4 (`KismetMathLibrary.Conv_IntToDouble` (`self.BlueSeisan`)))
  (`parent.ReceiveBeginPlay`)
  ;[1 1 1] データの初期設定
  (`PrimitiveComponent.SetSimulatePhysics` (`self.3dodai`) false)
  (`self.Init` "NewEnumerator4" (`|MakeArray` (`self.3dodai`) (`self.3oshidashi2`) (`self.3oshidashi`) (`self.3oshidashi1`))) ; 親の変数の初期化
  ;[1 1 1] ウィジットの初期化
  (`self.InitProgress` _returnvalue_4 _returnvalue_4 (`self.BlueCount`) 0 "Hidden")
  (`self.InitProgress` _returnvalue_3 _returnvalue_3 (`self.RedCount`) 0 "Hidden")
  (`self.InitProgress` _returnvalue_2 _returnvalue_2 (`self.WhiteCount`) 0 "Hidden")
  (`self.InitProgress` _returnvalue _returnvalue (`self.Error`) 0 "Hidden")
  ;[1 1 1] シーケンスの初期設定
  (`|ExecutionSequence`
    (:`then_0`
      (bind (_outactor _returnvalue_5) (`LevelSequencePlayer.CreateLevelSequencePlayer` "/Game/MyContents/LevelSequences/3oshidashi3.3oshidashi3"))
      (set `self.BlueOsidashiAnim` _returnvalue_5)
      (`LevelSequenceActor.SetBinding` _outactor (`|GetSequenceBinding` null) (`|MakeArray` self :!type "Actor Object Reference") false)
      (`MovieSceneSequencePlayer.SetPlayRate` (`self.BlueOsidashiAnim`) (`self.Speed`)))
    (:`then_1`
      (bind (_outactor_2 _returnvalue_6) (`LevelSequencePlayer.CreateLevelSequencePlayer` "/Game/MyContents/LevelSequences/3oshidashi2.3oshidashi2"))
      (set `self.RedOsidashiAnim` _returnvalue_6)
      (`LevelSequenceActor.SetBinding` _outactor_2 (`|GetSequenceBinding` null) (`|MakeArray` self :!type "Actor Object Reference") false)
      (`MovieSceneSequencePlayer.SetPlayRate` (`self.RedOsidashiAnim`) (`self.Speed`)))
    (:`then_2`
      (bind (_outactor_3 _returnvalue_7) (`LevelSequencePlayer.CreateLevelSequencePlayer` "/Game/MyContents/LevelSequences/3oshidashi1.3oshidashi1"))
      (set `self.WhiteOsidashiAnim` _returnvalue_7)
      (`LevelSequenceActor.SetBinding` _outactor_3 (`|GetSequenceBinding` null) (`|MakeArray` self :!type "Actor Object Reference") false)
      (`MovieSceneSequencePlayer.SetPlayRate` (`self.WhiteOsidashiAnim`) (`self.Speed`)))
    (:`then_3`
      (`PrimitiveComponent.SetCollisionEnabled` (`self.3dodai`) "QueryAndPhysics"))))

(event `self.BlueTrigger.OnComponentBeginOverlap`
  (params (OverlappedComponent :type "PrimitiveComponent Object Reference") (OtherActor :type "Actor Object Reference") (OtherComp :type "PrimitiveComponent Object Reference") (OtherBodyIndex :type Integer) (bFromSweep :type Boolean) (SweepResult :type "HitResult Structure (by ref)"))
  ;[1 1 1] 仕分け機のアニメーションの再生
  (bind _asyuke_blue (cast `/Game/MyContents/BluePrints/Objects/YukeBlue` OtherActor))
  (`PrimitiveComponent.SetSimulatePhysics` (`/Game/MyContents/BluePrints/Buttons/BP_ParamGoods.Goods` _asyuke_blue) true)
  (`MovieSceneSequencePlayer.Play` (`self.BlueOsidashiAnim`))
  (`self.ResetDoOnceBlue`))

(event `self.RedTrigger.OnComponentBeginOverlap`
  (params (OverlappedComponent :type "PrimitiveComponent Object Reference") (OtherActor :type "Actor Object Reference") (OtherComp :type "PrimitiveComponent Object Reference") (OtherBodyIndex :type Integer) (bFromSweep :type Boolean) (SweepResult :type "HitResult Structure (by ref)"))
  ;[1 1 1] 仕分け機のアニメーションの再生
  (bind _asyuke_red (cast `/Game/MyContents/BluePrints/Objects/YukeRed` OtherActor))
  (`PrimitiveComponent.SetSimulatePhysics` (`/Game/MyContents/BluePrints/Buttons/BP_ParamGoods.Goods` _asyuke_red) true)
  (`MovieSceneSequencePlayer.Play` (`self.RedOsidashiAnim`))
  (`self.ResetDoOnceBlue`))

(event `self.WhiteTrigger.OnComponentBeginOverlap`
  (params (OverlappedComponent :type "PrimitiveComponent Object Reference") (OtherActor :type "Actor Object Reference") (OtherComp :type "PrimitiveComponent Object Reference") (OtherBodyIndex :type Integer) (bFromSweep :type Boolean) (SweepResult :type "HitResult Structure (by ref)"))
  ;[1 1 1] 仕分け機のアニメーションの再生
  (bind _asyuke_white (cast `/Game/MyContents/BluePrints/Objects/YukeWhite` OtherActor))
  (`PrimitiveComponent.SetSimulatePhysics` (`/Game/MyContents/BluePrints/Buttons/BP_ParamGoods.Goods` _asyuke_white) true)
  (`MovieSceneSequencePlayer.Play` (`self.WhiteOsidashiAnim`))
  (`self.ResetDoOnceBlue`))

(event `self.WhiteGet.OnComponentBeginOverlap`
  (params (OverlappedComponent :type "PrimitiveComponent Object Reference") (OtherActor :type "Actor Object Reference") (OtherComp :type "PrimitiveComponent Object Reference") (OtherBodyIndex :type Integer) (bFromSweep :type Boolean) (SweepResult :type "HitResult Structure (by ref)"))
  ;[1 1 1] 加工品の仕分けが完了しオブジェクトをクレーンに運んでもらうための初期値をセット
  (`self.SetNextEria` OtherActor :!label _label))

(event `self.RedGet.OnComponentBeginOverlap`
  (params (OverlappedComponent :type "PrimitiveComponent Object Reference") (OtherActor :type "Actor Object Reference") (OtherComp :type "PrimitiveComponent Object Reference") (OtherBodyIndex :type Integer) (bFromSweep :type Boolean) (SweepResult :type "HitResult Structure (by ref)"))
  ;[1 1 1] 加工品の仕分けが完了しオブジェクトをクレーンに運んでもらうための初期値をセット
  (`self.SetNextEria` OtherActor :!label _label_2))

(event `self.BlueGet.OnComponentBeginOverlap`
  (params (OverlappedComponent :type "PrimitiveComponent Object Reference") (OtherActor :type "Actor Object Reference") (OtherComp :type "PrimitiveComponent Object Reference") (OtherBodyIndex :type Integer) (bFromSweep :type Boolean) (SweepResult :type "HitResult Structure (by ref)"))
  ;[1 1 1] 加工品の仕分けが完了しオブジェクトをクレーンに運んでもらうための初期値をセット
  (`self.SetNextEria` OtherActor :!label _label_3))

(event `resetDoonce`
  (`|ExecutionSequence`
    (:`then_0`
      ;[1 1 1] 加工品の仕分けが完了しオブジェクトをクレーンに運んでもらうための初期値をセット
      (`/Engine/EditorBlueprintResources/StandardMacros.DoOnce` false :!via `Reset`
        (:`Completed`
          (goto _label))))
    (:`then_1`
      (`/Engine/EditorBlueprintResources/StandardMacros.DoOnce` false :!via `Reset`
        (:`Completed`
          (goto _label_2))))
    (:`then_2`
      (`/Engine/EditorBlueprintResources/StandardMacros.DoOnce` false :!via `Reset`
        (:`Completed`
          (goto _label_3))))))

(event `self.yukeBlueyuke.OnComponentBeginOverlap`
  (params (OverlappedComponent :type "PrimitiveComponent Object Reference") (OtherActor :type "Actor Object Reference") (OtherComp :type "PrimitiveComponent Object Reference") (OtherBodyIndex :type Integer) (bFromSweep :type Boolean) (SweepResult :type "HitResult Structure (by ref)"))
  ;[1 1 1] 移動の停止
  (bind _asyuke_blue (cast `/Game/MyContents/BluePrints/Objects/YukeBlue` OtherActor))
  (set `/Game/MyContents/BluePrints/Buttons/BP_ParamGoods.NextTarget` null _asyuke_blue))

(event `self.yukeRedyuke.OnComponentBeginOverlap`
  (params (OverlappedComponent :type "PrimitiveComponent Object Reference") (OtherActor :type "Actor Object Reference") (OtherComp :type "PrimitiveComponent Object Reference") (OtherBodyIndex :type Integer) (bFromSweep :type Boolean) (SweepResult :type "HitResult Structure (by ref)"))
  ;[1 1 1] 移動の停止
  (bind _asyuke_red (cast `/Game/MyContents/BluePrints/Objects/YukeRed` OtherActor))
  (set `/Game/MyContents/BluePrints/Buttons/BP_ParamGoods.NextTarget` null _asyuke_red))

(event `self.yukeWhiteyuke.OnComponentBeginOverlap`
  (params (OverlappedComponent :type "PrimitiveComponent Object Reference") (OtherActor :type "Actor Object Reference") (OtherComp :type "PrimitiveComponent Object Reference") (OtherBodyIndex :type Integer) (bFromSweep :type Boolean) (SweepResult :type "HitResult Structure (by ref)"))
  ;[1 1 1] 移動の停止
  (bind _asyuke_white (cast `/Game/MyContents/BluePrints/Objects/YukeWhite` OtherActor))
  (set `/Game/MyContents/BluePrints/Buttons/BP_ParamGoods.NextTarget` null _asyuke_white))

(event `self.Box3.OnComponentBeginOverlap`
  (params (OverlappedComponent :type "PrimitiveComponent Object Reference") (OtherActor :type "Actor Object Reference") (OtherComp :type "PrimitiveComponent Object Reference") (OtherBodyIndex :type Integer) (bFromSweep :type Boolean) (SweepResult :type "HitResult Structure (by ref)"))
  ;[1 1 1] 加工品の移動先を更新
  (bind _asbp_param_goods (cast `/Game/MyContents/BluePrints/Buttons/BP_ParamGoods` OtherActor))
  (set `/Game/MyContents/BluePrints/Buttons/BP_ParamGoods.NextTarget` (`self.Box4`) _asbp_param_goods)
  (`PrimitiveComponent.SetSimulatePhysics` (`/Game/MyContents/BluePrints/Buttons/BP_ParamGoods.Goods` _asbp_param_goods) false))

(event `self.Box4.OnComponentBeginOverlap`
  (params (OverlappedComponent :type "PrimitiveComponent Object Reference") (OtherActor :type "Actor Object Reference") (OtherComp :type "PrimitiveComponent Object Reference") (OtherBodyIndex :type Integer) (bFromSweep :type Boolean) (SweepResult :type "HitResult Structure (by ref)"))
  ;[1 1 1] 青、赤、白、エラーの数をカウントする
  (bind _asbp_param_goods (cast `/Game/MyContents/BluePrints/Buttons/BP_ParamGoods` OtherActor))
  (`KismetArrayLibrary.Array_Add` (`self.As BP Param Goods`) _asbp_param_goods)
  (set `/Game/MyContents/BluePrints/Buttons/BP_ParamGoods.NextTarget` null _asbp_param_goods)
  (bind _goods (`/Game/MyContents/BluePrints/Buttons/BP_ParamGoods.Goods` _asbp_param_goods))
  (`PrimitiveComponent.SetSimulatePhysics` _goods true)
  (`PrimitiveComponent.AddImpulse` _goods (`KismetMathLibrary.MakeVector` 0.0 (* -270.0 (`self.Speed`))) "None" true)
  (`/Engine/EditorBlueprintResources/StandardMacros.IncrementInt` (`self.ErrorCount`)))

(event `ResetDoOnceBlue`
  ;[1 1 1] 青、赤、白、エラーの数をカウントする
  (goto _label_4 :!via `Reset`))

(event `self.Box5.OnComponentBeginOverlap`
  (params (OverlappedComponent :type "PrimitiveComponent Object Reference") (OtherActor :type "Actor Object Reference") (OtherComp :type "PrimitiveComponent Object Reference") (OtherBodyIndex :type Integer) (bFromSweep :type Boolean) (SweepResult :type "HitResult Structure (by ref)"))
  ;[1 1 1] 青、赤、白、エラーの数をカウントする
  (`self.resetDoonce`)
  (`|ExecutionSequence`
    (:`then_0`
      (cast `/Game/MyContents/BluePrints/Objects/YukeBlue` OtherActor)
      (`/Engine/EditorBlueprintResources/StandardMacros.DoOnce` false :!label _label_4
        (:`Completed`
          (`/Engine/EditorBlueprintResources/StandardMacros.IncrementInt` (`self.BlueSeisan`)))))
    (:`then_1`
      (cast `/Game/MyContents/BluePrints/Objects/YukeRed` OtherActor)
      (`/Engine/EditorBlueprintResources/StandardMacros.DoOnce` false :!label _label_5
        (:`Completed`
          (`/Engine/EditorBlueprintResources/StandardMacros.IncrementInt` (`self.RedSeisan`)))))
    (:`then_2`
      (cast `/Game/MyContents/BluePrints/Objects/YukeWhite` OtherActor)
      (`/Engine/EditorBlueprintResources/StandardMacros.DoOnce` false :!label _label_6
        (:`Completed`
          (`/Engine/EditorBlueprintResources/StandardMacros.IncrementInt` (`self.WhiteSeisan`)))))))

(event `ResetDoOnceRed`
  ;[1 1 1] 青、赤、白、エラーの数をカウントする
  (goto _label_5 :!via `Reset`))

(event `ResetDoOnceWhite`
  ;[1 1 1] 青、赤、白、エラーの数をカウントする
  (goto _label_6 :!via `Reset`))

(fn `SetNextEria`
  (params (Object :type "Object Object Reference"))
  (bind _asbp_param_goods (cast `/Game/MyContents/BluePrints/Buttons/BP_ParamGoods` Object))
  (bind _outactors (`GameplayStatics.GetAllActorsOfClass` "/Game/MyContents/BluePrints/PackageObj/nanikore.nanikore_C"))
  (bind _output (`|GetArrayItem` _outactors))
  (if (`KismetSystemLibrary.IsValid` _output)
    (set `/Game/MyContents/BluePrints/Buttons/BP_ParamGoods.NextEria` (`/Game/MyContents/BluePrints/PackageObj/nanikore.nanikoreT` _output) _asbp_param_goods)
    (bind _outactors_2 (`GameplayStatics.GetAllActorsOfClass` "/Game/MyContents/BluePrints/PackageObj/SuperClane.SuperClane_C"))
    (for _array_element _outactors_2
      (`/Game/MyContents/BluePrints/PackageObj/SuperClane.AddTargetArray` _array_element _asbp_param_goods)
      (break))))

(fn `UserConstructionScript`)