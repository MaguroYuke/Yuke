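; Free-fly camera pawn for the edit, simulation and tutorial maps, branching on level name for view setup and look behavior.
; Input axes offset the actor directly, with forward flattened from control rotation; Shift or Space boosts speed.
; Right-click enables mouse look; Tick applies yaw only and lets the camera follow control rotation only in Map_Simulation.
; In Map_EditTurorial, movement is blocked while the tutorial widget's message is visible.
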(event `InputAxis|XMove`
  (params (AxisValue :type "Float (single-precision)"))
  (bind (_returnvalue_x _returnvalue_y) (`KismetMathLibrary.BreakVector` (`KismetMathLibrary.GetForwardVector` (`Controller.GetControlRotation` (`GameplayStatics.GetPlayerController` 0)))))
  (bind (_returnvalue_x_2 _returnvalue_y_2) (`KismetMathLibrary.BreakVector` (* (`KismetMathLibrary.Normal` (`KismetMathLibrary.MakeVector` _returnvalue_x _returnvalue_y (`self.zZero`))) AxisValue (`self.Speed`))))
  (if (`KismetStringLibrary.EqualEqual_StrStr` (stale `InputAxis|ZMove` _returnvalue) "Map_EditTurorial")
    (if (not (`Widget.IsVisible` (`/Game/MyContents/BluePrints/Widget/BPW_Tutorial.Text_Message` (stale `self.ReceiveBeginPlay` _array_element))))
      (`self.K2_AddActorWorldOffset` (`KismetMathLibrary.MakeVector` _returnvalue_x_2 _returnvalue_y_2) :!label _label))
    (else
      (goto _label))))

(event `InputAxis|YMove`
  (params (AxisValue :type "Float (single-precision)"))
  (if (`KismetStringLibrary.EqualEqual_StrStr` (stale `InputAxis|ZMove` _returnvalue) "Map_EditTurorial")
    (if (not (`Widget.IsVisible` (`/Game/MyContents/BluePrints/Widget/BPW_Tutorial.Text_Message` (stale `self.ReceiveBeginPlay` _array_element))))
      (`self.K2_AddActorLocalOffset` (`KismetMathLibrary.MakeVector` 0.0 (* AxisValue (`self.Speed`)) (`self.zZero`)) :!label _label_2))
    (else
      (goto _label_2))))

(event `InputAxis|ZMove`
  (params (AxisValue :type "Float (single-precision)"))
  (bind _returnvalue (`GameplayStatics.GetCurrentLevelName` true))
  (if (`KismetStringLibrary.EqualEqual_StrStr` _returnvalue "Map_EditTurorial")
    (if (not (`Widget.IsVisible` (`/Game/MyContents/BluePrints/Widget/BPW_Tutorial.Text_Message` (stale `self.ReceiveBeginPlay` _array_element))))
      (`self.K2_AddActorWorldOffset` (`KismetMathLibrary.MakeVector` 0.0 0.0 (* AxisValue (`self.Speed`))) :!label _label_3))
    (else
      (goto _label_3))))

(event `self.ReceiveBeginPlay`
  (bind _returnvalue (`GameplayStatics.GetPlayerController` 0))
  (`|ExecutionSequence`
    (:`then_0`
      (bind _returnvalue_2 (`GameplayStatics.GetCurrentLevelName` true))
      (if (or (`KismetStringLibrary.EqualEqual_StrStr` _returnvalue_2 "Map_Edit") (`KismetStringLibrary.EqualEqual_StrStr` _returnvalue_2 "YuukiMap") (`KismetStringLibrary.EqualEqual_StrStr` _returnvalue_2 "Map_EditTurorial"))
        (`Controller.SetIgnoreLookInput` _returnvalue true)
        (`InputDeviceLibrary.GetPlayerControllerFromInputDevice` (struct))
        (`PlayerController.SetViewTargetWithBlend` _returnvalue self 0.0 "VTBlend_Linear" 0.0 false)
        (bind _foundwidgets (`WidgetBlueprintLibrary.GetAllWidgetsOfClass` "/Game/MyContents/BluePrints/Widget/BPW_Tutorial.BPW_Tutorial_C" false))
        (for _array_element _foundwidgets
          _)
        (else
          (bind _returnvalue_3 (`GameplayStatics.GetCurrentLevelName` true))
          (set `self.bIsMouseLookEnabled` (or (`KismetStringLibrary.EqualEqual_StrStr` _returnvalue_3 "Map_SimulationTutorial") (`KismetStringLibrary.EqualEqual_StrStr` _returnvalue_3 "Map_Simulation")))
          (`WidgetBlueprintLibrary.SetInputMode_GameAndUIEx` (`GameplayStatics.GetPlayerController` 0) null))))
    (:`then_1`
      (bind _returnvalue_4 (`GameplayStatics.GetCurrentLevelName` true))
      (if (or (== _returnvalue_4 "Map_Edit") (== _returnvalue_4 "Map_EditTurorial"))
        (if (not (`self.IsCamera_Rotation`))
          (`Controller.SetControlRotation` (`GameplayStatics.GetPlayerController` 0) (`self.Camera_Rotation`))
          (set `self.IsCamera_Rotation` true))))))

(event `InputAction|Shift_Dush`
  (params (Key :type "Key Structure"))
  (bind _speed (`self.Speed`))
  (:`Pressed`
    (set `self.Speed` (+ _speed 200.0) :!label _label_4))
  (:`Released`
    (set `self.Speed` (- _speed 200.0) :!label _label_5)))

(event `InputAction|Space_Dush`
  (params (Key :type "Key Structure"))
  (:`Pressed`
    (goto _label_4))
  (:`Released`
    (goto _label_5)))

(event `InputAction|RightClick`
  (params (Key :type "Key Structure"))
  (bind _returnvalue (`GameplayStatics.GetPlayerController` 0))
  (bind (_deltax _deltay) (`PlayerController.GetInputMouseDelta` _returnvalue))
  (:`Pressed`
    (set `PlayerController.bShowMouseCursor` false _returnvalue)
    (set `self.bIsMouseLookEnabled` true)
    (`self.AddControllerYawInput` _deltax)
    (`self.AddControllerPitchInput` (* _deltay -1.0)))
  (:`Released`
    (set `PlayerController.bShowMouseCursor` true _returnvalue)
    (set `self.bIsMouseLookEnabled` false)))

(event `self.ReceiveTick`
  (params (DeltaSeconds :type "Float (single-precision)"))
  (bind _returnvalue (`GameplayStatics.GetPlayerPawn` 0))
  (bind _camera (`self.Camera`))
  (`|ExecutionSequence`
    (:`then_0`
      (if (`self.bIsMouseLookEnabled`)
        (`self.AddControllerYawInput` _returnvalue (`self.GetInputAxisKeyValue`))
        (`self.AddControllerPitchInput` _returnvalue 0.0)))
    (:`then_1`
      (bind _returnvalue_2 (`GameplayStatics.GetCurrentLevelName` true))
      (if (== _returnvalue_2 "Map_Simulation")
        (set `CameraComponent.bUsePawnControlRotation` true _camera)
        (else
          (set `CameraComponent.bUsePawnControlRotation` false _camera))))))

(fn `UserConstructionScript`)