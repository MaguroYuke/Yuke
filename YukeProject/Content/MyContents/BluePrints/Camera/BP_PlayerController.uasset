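; Player controller Blueprint that sets up the view at level start and flags the game as simulation mode.
; On BeginPlay it adds a child actor component, calls SetViewTargetWithBlend on the first player controller and sets IsSimulationMode to true unconditionally.
; A Map_Simulation level-name check and pawn pitch/yaw look input are left unconnected, and Tick does nothing.
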(event `self.ReceiveBeginPlay`
  (`AddComponent|NODE_AddChildActorComponent-0`)
  (`self.SetViewTargetWithBlend` (`GameplayStatics.GetPlayerController` 0) null 0.0 "VTBlend_Linear" 0.0 false)
  (set `self.bIsSimulationMode` true))

(event `self.ReceiveTick`
  (params (DeltaSeconds :type "Float (single-precision)")))

(fn `UserConstructionScript`)