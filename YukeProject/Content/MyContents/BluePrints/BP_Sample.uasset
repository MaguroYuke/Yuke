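; Sample actor that visits a queue of target locations, briefly shows an "到着" (arrived) widget label at each, then destroys itself.
; The externally called Artifact event runs an enum state machine: wait, pick the next target, move, show text, end; Tick is unused.
; Movement repeats a lerp-derived offset computed once per target, then snaps to it.
; Ending removes the actor from the passed array and decrements the widget's actor count.
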(event `self.ReceiveBeginPlay`
  ;[1 1 1] Actorの初期設定
  (`self.InitWidget`)
  (set `self.DeltaTime` 0.01)
  (set `self.Timer` 0.0)
  (set `self.BPE_Artifact` "NewEnumerator5")
  (`self.InitPosition`))

(event `self.ReceiveActorBeginOverlap`
  (params (OtherActor :type "Actor Object Reference")))

(event `self.ReceiveTick`
  (params (DeltaSeconds :type "Float (single-precision)")))

(event `Artifact`
  (params (WidgetTimer :type "Float (double-precision)") (MyActors :type "Array of /Game/MyContents/BluePrints/BP_Sample Object Reference") (BPW_ActorCount :type "/Game/MyContents/BluePrints/BPW_ActorCount Object Reference"))
  (switch `/Game/MyContents/BluePrints/BPE_Artifact` (`self.BPE_Artifact`)
    (:`NewEnumerator5`
      (`KismetSystemLibrary.Delay` WidgetTimer)
      (set `self.BPE_Artifact` "NewEnumerator0"))
    (:`NewEnumerator0`
      (if (>= (`KismetArrayLibrary.Array_LastIndex` (`self.ALLTargetLocations`)) 0)
        (`self.NextActorLocation` (`|GetArrayItem` (`self.ALLTargetLocations`))) ; 移動先の座標を入力し開始
        (`KismetArrayLibrary.Array_Remove` (`self.ALLTargetLocations`))
        (else
          (set `self.BPE_Artifact` "NewEnumerator3"))))
    (:`NewEnumerator1`
      (`self.SetMyActorLocation`) ; 指定した場所まで移動
    )
    (:`NewEnumerator2`
      (`self.SetMyActorText` WidgetTimer) ; 移動終了したときにTextを表示
    )
    (:`NewEnumerator3`
      (`self.MyDestroyActor` MyActors) ; 自分のアクターを削除し配列から取り除く
      (`/Engine/EditorBlueprintResources/StandardMacros.DecrementInt` (`/Game/MyContents/BluePrints/BPW_ActorCount.ActorCount` BPW_ActorCount)))))

(fn `InitWidget`
  (bind _asbpw_actor_widget (cast `/Game/MyContents/BluePrints/BPW_ActorWidget` (`WidgetComponent.GetUserWidgetObject` (`self.Widget`))))
  (bind _output_get (set `self.BPW_ActorWidget` _asbpw_actor_widget))
  (set `/Game/MyContents/BluePrints/BPW_ActorWidget.ActorText` "" _output_get)
  (set `/Game/MyContents/BluePrints/BPW_ActorWidget.E_Visibility` "Hidden" _output_get))

(fn `MyDestroyActor`
  (params (Actor :type "Array of /Game/MyContents/BluePrints/BP_Sample Object Reference (by ref)"))
  (bind _returnvalue (`KismetArrayLibrary.Array_RemoveItem` Actor self))
  (if _returnvalue
    (`KismetSystemLibrary.PrintString` (`KismetStringLibrary.Concat_StrStr` (`KismetSystemLibrary.GetObjectName` self) ":削除"))
    (`self.K2_DestroyActor`)))

(fn `NextActorLocation`
  (params (NextActorLocation :type "Vector Structure"))
  (bind _bpw_actorwidget (`self.BPW_ActorWidget`))
  (set `self.StartActorLocation` true)
  (bind _uplocation (`self.SetLerp` NextActorLocation)) ; 移動する場所と自分の場所を分割する
  (set `self.UpLocation` _uplocation)
  (set `self.TargetLocation` NextActorLocation)
  (set `/Game/MyContents/BluePrints/BPW_ActorWidget.ActorText` "" _bpw_actorwidget)
  (set `/Game/MyContents/BluePrints/BPW_ActorWidget.E_Visibility` "Hidden" _bpw_actorwidget)
  (set `self.BPE_Artifact` "NewEnumerator1"))

(fn `SetLerp`
  (params (NextActorLocation :type "Vector Structure"))
  (returns (UpLocation :type "Vector Structure"))
  (bind _output_get (set `self.LerpAlpha` (`KismetMathLibrary.FClamp` (* (`self.DeltaTime`) (`self.Speed`)))))
  (return (- (`KismetMathLibrary.VLerp` (`self.K2_GetActorLocation`) NextActorLocation _output_get) (`self.K2_GetActorLocation`))))

(fn `SetMyActorLocation`
  (if (<= (`self.LocationPartition`) 1.0)
    (set `self.LocationPartition` (+ (`self.LocationPartition`) (`self.LerpAlpha`)))
    (`self.K2_SetActorLocation` (+ (`self.K2_GetActorLocation`) (`self.UpLocation`)))
    (else
      (set `self.LocationPartition` 0.0)
      (`self.K2_SetActorLocation` (`self.TargetLocation`))
      (set `self.BPE_Artifact` "NewEnumerator2"))))

(fn `SetMyActorText`
  (params (EndTime :type "Float (double-precision)"))
  (bind _bpw_actorwidget (`self.BPW_ActorWidget`))
  (bind _bpw_actorwidget_2 (`self.BPW_ActorWidget`))
  (bind _returnvalue (+ (`self.Timer`) (`self.DeltaTime`)))
  (if (<= _returnvalue EndTime)
    (set `self.Timer` _returnvalue)
    (set `/Game/MyContents/BluePrints/BPW_ActorWidget.ActorText` "到着" _bpw_actorwidget_2)
    (set `/Game/MyContents/BluePrints/BPW_ActorWidget.E_Visibility` "Visible" _bpw_actorwidget_2)
    (else
      (set `self.Timer` 0.0)
      (set `/Game/MyContents/BluePrints/BPW_ActorWidget.ActorText` "" _bpw_actorwidget)
      (set `/Game/MyContents/BluePrints/BPW_ActorWidget.E_Visibility` "Hidden" _bpw_actorwidget)
      (set `self.BPE_Artifact` "NewEnumerator0"))))

(fn `UserConstructionScript`)