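; BP_ParamGoods is a goods item that rides a conveyor.
; On BeginPlay it initializes its location and state and destroys its Dodai component.
; Event B enables physics on Goods and snaps its X to the given component, after which Tick forces a constant -Y velocity.
; NextLocation offers state-driven movement (Stop, Start, UpData, End) via StartMove and MoveActor; a similar EventGraph copy never runs.
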(event `self.ReceiveBeginPlay`
  (`self.InitLocation`)
  (set `self.BPE_Artifact` "NewEnumerator0")
  (set `self.Speed` 10.0)
  (`ActorComponent.K2_DestroyComponent` (`self.Dodai`)))

(event `self.ReceiveTick`
  (params (DeltaSeconds :type "Float (single-precision)"))
  (if (`self.bOnConveyor`)
    (`PrimitiveComponent.SetPhysicsLinearVelocity` (`self.Goods`) (0.0 -400.0 0.0) false "None")))

(event `B`
  (params (SceneComponent :type "SceneComponent Object Reference"))
  (bind _returnvalue_x (`KismetMathLibrary.BreakVector` (`SceneComponent.K2_GetComponentLocation` SceneComponent)))
  (bind _zero (`self.zero`))
  (bind _goods (`self.Goods`))
  (bind (_returnvalue_x_2 _returnvalue_y _returnvalue_z) (`KismetMathLibrary.BreakVector` (`SceneComponent.K2_GetComponentLocation` _goods)))
  (`PrimitiveComponent.SetSimulatePhysics` _goods true)
  (set `self.bOnConveyor` true)
  (`SceneComponent.K2_SetWorldLocationAndRotation` _goods (`KismetMathLibrary.MakeVector` _returnvalue_x _returnvalue_y _returnvalue_z) (`KismetMathLibrary.MakeRotator` _zero _zero _zero) false false))

(fn `NextLocation`
  (params (MyActor :type "Actor Object Reference") (TargetLocation :type "Vector Structure") (targetItem :type "PrimitiveComponent Object Reference"))
  (bind _returnvalue (`SceneComponent.K2_GetComponentLocation` targetItem))
  (switch `/Game/MyContents/BluePrints/Objects/BPE_Artifact` (`self.BPE_Artifact`)
    (:`NewEnumerator0`
      (`self.K2_SetActorLocation` MyActor _returnvalue false false))
    (:`NewEnumerator1`
      (`self.StartMove` _returnvalue TargetLocation)
      (set `self.BPE_Artifact` "NewEnumerator2"))
    (:`NewEnumerator2`
      (bind (_location _onmove) (`self.MoveActor` _returnvalue))
      (`SceneComponent.K2_SetWorldLocation` targetItem _location false false)
      (if (not _onmove)
        (set `self.BPE_Artifact` "NewEnumerator3")))))

(fn `UserConstructionScript`)