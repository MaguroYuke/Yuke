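; Conveyor belt actor for the sorting machine that animates during play and stays still in the edit maps.
; Every Tick it checks the current level name, stopping the SaikyouBeruto component in Map_Edit and Map_EditTurorial and calling looped Play on it in any other level.
; The same Tick also re-applies query and physics collision to that component each frame.
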(event `self.ReceiveTick`
  (params (DeltaSeconds :type "Float (single-precision)"))
  (bind _saikyou_beruto (`self.Saikyou_Beruto`))
  (`|ExecutionSequence`
    (:`then_0`
      (bind _returnvalue (`GameplayStatics.GetCurrentLevelName` true))
      (if (or (== _returnvalue "Map_Edit") (== _returnvalue "Map_EditTurorial"))
        (`SkeletalMeshComponent.Stop` _saikyou_beruto)
        (else
          (`SkeletalMeshComponent.Play` _saikyou_beruto true))))
    (:`then_1`
      (`PrimitiveComponent.SetCollisionEnabled` (`self.Saikyou_Beruto`) "QueryAndPhysics"))))

(fn `UserConstructionScript`)